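; BP_Item is a world pickup item that the player can focus, inspect and add to their inventory.
; Its row in DT_Items supplies the item data, with gem rarity and icon derived from polish, which can be overridden per instance.
; Focus toggles a custom-depth highlight and a pickup widget initialized at BeginPlay.
; Interaction tries to add it to the character's InventoryComponent, then on success hides it on remote clients and unregisters it.
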(event EventBeginPlay
  (bind _item (CallFunction|GetItemData))
  (Physics|SetSimulatePhysics (Variables|Default|GetItemMesh) (Variables|Default|GetSimulatePhysics))
  (Rendering|SetVisibility (Variables|Default|GetWidget) false false)
  (bind _aswb_item_pickup (Utilities|Casting|CastToWB_ItemPickup (UserInterface|GetWidget (Variables|Default|GetWidget))))
  (Default|Init _aswb_item_pickup (CallFunction|GetItemRarity) (.itemname _item) (Math|Float|SelectFloat (Variables|Default|GetDefaultPolish) (.defaultpolish _item) (Variables|Default|GetbOverridePolish)) (.itemtype _item)))

(event EventOnStartFocus
  (Rendering|SetRenderCustomDepth (Variables|Default|GetItemMesh) true)
  (if (not (Variables|Default|GetShowedWidget))
    (Rendering|SetVisibility (Variables|Default|GetWidget) true false)
    (Variables|Default|SetShowedWidget true)))

(event EventOnInteract
  (params (Invoker :type Actor%20Object%20Reference))
  (bind _item (CallFunction|GetItemData))
  (bind _asbp_first_person_character (Utilities|Casting|CastToBP_FirstPersonCharacter Invoker))
  (bind _returnvalue (Class|InventoryComp|TryAddItembyAddItemInfo (Variables|/Script/ExtractionGame.ExtractionGameCharacter|GetInventoryComponent _asbp_first_person_character) (Utilities|Struct|MakeAddItemInfo (Math|Vector2D|MakeVector2D (Math|Conversions|ToFloat(Integer) (.sizex _item)) (Math|Conversions|ToFloat(Integer) (.sizey _item))) (select (Utilities|Enum|Equal(Enum) (.itemtype _item) "Gem") (Utilities|Array|Get(acopy) (.icon _item) (Math|Conversions|ToInteger(Byte) (CallFunction|GetGemIcon))) (Utilities|Array|Get(acopy) (.icon _item))) (.iconrotated _item) (.itemname _item) (.itemtype _item) (CallFunction|GetItemRarity) (.description _item) (.gemtype _item) (Math|Float|SelectFloat (Variables|Default|GetDefaultPolish) (.defaultpolish _item) (Variables|Default|GetbOverridePolish)) (Utilities|String|StringToName (Variables|Default|GetRowName)))))
  (if _returnvalue
    (Networking|SwitchHasAuthority
      (:Authority
        _)
      (:Remote
        (Rendering|SetVisibility (Variables|Default|GetItemMesh) false false)
        (Rendering|SetVisibility (Variables|Default|GetWidget) false false)))
    (Class|ItemActor|UnregisterItem)))

(event EventOnCancelFocus
  (Rendering|SetRenderCustomDepth (Variables|Default|GetItemMesh) false)
  (Rendering|SetVisibility (Variables|Default|GetWidget) false false)
  (Variables|Default|SetShowedWidget false))

(fn ConstructionScript)

(fn GetItemData
  (bind _returnvalue (Utilities|GetDataTableRow "/Game/DataAssets/DataTables/DT_Items.DT_Items" (Utilities|String|StringToName (Variables|Default|GetRowName)))
    (:then
      (return _returnvalue))
    (:RowNotFound
      (Development|PrintText "row not found"))))

(fn GetItemRarity
  (bind _item (CallFunction|GetItemData))
  (Utilities|FlowControl|Sequence
    (:then_0
      (LocalVariables|SetPolish (Math|Float|SelectFloat (Variables|Default|GetDefaultPolish) (.defaultpolish (CallFunction|GetItemData)) (Variables|Default|GetbOverridePolish))))
    (:then_1
      (if (Utilities|Enum|Equal(Enum) (.itemtype _item) "Gem")
        (if (<= (LocalVariables|GetPolish) 25.0)
          (return "Uncommon")
          (elif (<= (LocalVariables|GetPolish) 5e+01)
            (return "Rare")
            (elif (<= (LocalVariables|GetPolish) 75.0)
              (return "Epic")
              (else
                (return "Legendary")))))
        (else
          (return (.rarity _item)))))))

(fn GetGemIcon
  (LocalVariables|SetPurity (Math|Float|SelectFloat (Variables|Default|GetDefaultPolish) (.defaultpolish (CallFunction|GetItemData)) (Variables|Default|GetbOverridePolish)))
  (if (<= (LocalVariables|GetPurity) 25.0)
    (return 0)
    (elif (<= (LocalVariables|GetPurity) 5e+01)
      (return 0)
      (elif (<= (LocalVariables|GetPurity) 75.0)
        (return 1)
        (else
          (return 2))))))