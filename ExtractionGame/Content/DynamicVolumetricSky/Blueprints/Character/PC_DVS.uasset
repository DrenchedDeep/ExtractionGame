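; Player controller for the Dynamic Volumetric Sky asset that manages its on-screen UI widget.
; On BeginPlay it creates and shows the sky widget, enabling the mouse cursor and Game and UI input.
; V alternates between removing the widget for game-only input and restoring it with cursor and UI input.
; T toggles the widget's tutorial text through render opacity, with both keys driven by FlipFlops.
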(event EventBeginPlay
  (bind _returnvalue (UserInterface|CreateWidget "/Game/DynamicVolumetricSky/Blueprints/UI/WBP_DynamicVolumetricSky.WBP_DynamicVolumetricSky_C"))
  (bind _output_get (Variables|Default|SetWBP _returnvalue))
  (UserInterface|Viewport|AddtoViewport _output_get 0)
  (Input|SetInputModeGameandUI self 0 "DoNotLock" true false)
  (Variables|Default|SetbShowMouseCursor true))

(event Input|KeyboardEvents|T
  (params (Key :type Key%20Structure))
  (bind _wbp (Variables|Default|GetWBP))
  (bind _tutorialtext (Variables|/Game/DynamicVolumetricSky/Blueprints/UI/WBP_DynamicVolumetricSky.WBP_DynamicVolumetricSky_C|GetTutorialText _wbp))
  (:Pressed
    (Utilities|FlowControl|FlipFlop
      (:A
        (Widget|SetRenderOpacity _tutorialtext 0.0))
      (:B
        (Widget|SetRenderOpacity _tutorialtext 1.0)))))

(event Input|KeyboardEvents|V
  (params (Key :type Key%20Structure))
  (bind _wbp (Variables|Default|GetWBP))
  (:Pressed
    (Utilities|FlowControl|FlipFlop
      (:A
        (Input|SetInputModeGameOnly self false)
        (Variables|Default|SetbShowMouseCursor false)
        (if (UserInterface|Viewport|IsinViewport (Variables|Default|GetWBP))
          (Widget|RemovefromParent _wbp)))
      (:B
        (Input|SetInputModeGameandUI self 0 "DoNotLock" true false)
        (Variables|Default|SetbShowMouseCursor true)
        (if (not (UserInterface|Viewport|IsinViewport (Variables|Default|GetWBP)))
          (UserInterface|Viewport|AddtoViewport _wbp 0))))))

(fn ConstructionScript)