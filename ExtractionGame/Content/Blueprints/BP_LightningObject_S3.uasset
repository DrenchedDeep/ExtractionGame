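; Short-lived lightning effect actor that draws a bolt between an owner actor and a target actor, then destroys itself after a few seconds.
; Tick feeds both actors' current locations into the Lightning effect's start and end vectors while both are valid.
; UpdateLightingTraces, not called within this Blueprint, makes cooldown-gated random downward traces, spawns Niagara bolts at hits and applies radial damage through CheckForPlayers.
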(event EventBeginPlay
  (Utilities|FlowControl|Delay 3.0)
  (Actor|DestroyActor))

(event EventTick
  (params (DeltaSeconds :type Float%20%28single-precision%29))
  (bind _lightning (Variables|Default|GetLightning))
  (Utilities|IsValid (Variables|Default|GetOwnerActor)
    (:Is%20Valid
      (Utilities|IsValid (Variables|Default|GetTargetActor)
        (:Is%20Valid
          (Niagara|SetNiagaraVariable(Vector3) _lightning "StartLocation" (Transformation|GetActorLocation (Variables|Default|GetOwnerActor)))
          (Niagara|SetNiagaraVariable(Vector3) _lightning "EndLocation" (Transformation|GetActorLocation (Variables|Default|GetTargetActor))))))))

(fn ConstructionScript)

(fn UpdateLightingTraces
  (bind _returnvalue (Transformation|GetActorLocation))
  (bind _maxradius (Variables|Default|GetMaxRadius))
  (if (>= (- (Utilities|Time|GetTimeSeconds) (Variables|Default|GetLastTrace)) (Variables|Default|GetTraceCooldown))
    (bind _output_get (LocalVariables|SetRandomDirection (Math|Random|RandomUnitVector)))
    (LocalVariables|SetRandomDirection (Math|Vector|MakeVector (.x _output_get) (.y _output_get) 1.0))
    (bind _outhit (Collision|LineTraceByChannel (+ (Transformation|GetActorLocation) (* (LocalVariables|GetRandomDirection) (Variables|Default|GetMinRadius))) (+ (Math|Vector|MakeVector (.x _returnvalue) (.y _returnvalue) 1.0) (Math|Vector|MakeVector (* (.x (LocalVariables|GetRandomDirection)) _maxradius) (* (.y (LocalVariables|GetRandomDirection)) _maxradius) (* (.z (LocalVariables|GetRandomDirection)) -1e+03))) "TraceTypeQuery1" false 0 "None" true "(R=1.000000,G=0.000000,B=0.000000,A=1.000000)" "(R=0.000000,G=1.000000,B=0.000000,A=1.000000)" (Variables|Default|GetTraceCooldown)))
    (Variables|Default|SetLastTrace (Utilities|Time|GetTimeSeconds))
    (if (.bBlockingHit (Collision|BreakHitResult _outhit))
      (bind _returnvalue_2 (Niagara|SpawnSystemAttached "/Game/ParticleSystems/Ability/NS_Lightning.NS_Lightning" (Variables|Default|GetDefaultSceneRoot) "None" "0, 0, 0" "0, 0, 0" "KeepRelativeOffset" true))
      (Utilities|IsValid _returnvalue_2
        (:Is%20Valid
          (Niagara|SetNiagaraVariable(Vector3) _returnvalue_2 "StartLocation" (* (LocalVariables|GetRandomDirection) (Variables|Default|GetMinRadius)))
          (Niagara|SetNiagaraVariable(Vector3) _returnvalue_2 "EndLocation" (+ (.ImpactPoint (Collision|BreakHitResult _outhit)) (* (.ImpactNormal (Collision|BreakHitResult _outhit)) (LocalVariables|GetImpactOffset))))
          (Niagara|SetNiagaraVariable(Vector3) _returnvalue_2 "ImpactNormal" (.ImpactNormal (Collision|BreakHitResult _outhit)))
          (CallFunction|CheckforPlayers (+ (.ImpactPoint (Collision|BreakHitResult _outhit)) (* (.ImpactNormal (Collision|BreakHitResult _outhit)) (LocalVariables|GetImpactOffset)))))))))

(fn CheckforPlayers
  (params (InLocation :type Vector))
  (Game|Damage|ApplyRadialDamage 2e+01 InLocation 4e+02 0 0 (Components|GetOwner) (Pawn|GetController (Game|GetInstigator)) true "ECC_Visibility"))