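; Possessable ragdoll pawn that the player looks around from until it turns back into a first-person character.
; Half a second after spawning it enables its collider for queries; an overlap on the server while controlled spawns and possesses BP_FirstPersonCharacter above the mesh, then destroys the ragdoll.
; Radial and point damage push the skeletal mesh with an upward-biased impulse, scaled by damage, damage-type impulse and the CommandHandlerSubsystem knockback value.
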(event OnComponentBeginOverlap(RagdollCollider)
  (params (OverlappedComponent :type Primitive%20Component%20Object%20Reference) (OtherActor :type Actor%20Object%20Reference) (OtherComp :type Primitive%20Component%20Object%20Reference) (OtherBodyIndex :type Integer) (bFromSweep :type Boolean) (SweepResult :type Hit%20Result%20Structure%20%28by%20ref%29))
  (if (and (Class|Pawn|IsControlled) (Ability|HasAuthority))
    (CallFunction|SpawnPlayer)))

(event Custom|CustomEvent
  (Collision|SetCollisionEnabled (Variables|Default|GetRagdollCollider) "QueryOnly"))

(event Custom|OnTakePointDamage_Event
  (params (DamagedActor :type Actor%20Object%20Reference) (Damage :type Float%20%28single-precision%29) (InstigatedBy :type Controller%20Object%20Reference) (HitLocation :type Vector) (FHitComponent :type Primitive%20Component%20Object%20Reference) (BoneName :type Name) (ShotFromDirection :type Vector) (DamageType :type Damage%20Type%20Object%20Reference) (DamageCauser :type Actor%20Object%20Reference))
  (CallFunction|ApplyKnockback ShotFromDirection (* Damage (Variables|/Script/Engine.DamageType|GetDamageImpulse DamageType))))

(event Custom|OnTakeRadialDamage_Event
  (params (DamagedActor :type Actor%20Object%20Reference) (Damage :type Float%20%28single-precision%29) (DamageType :type Damage%20Type%20Object%20Reference) (Origin :type Vector) (HitInfo :type Hit%20Result%20Structure%20%28by%20ref%29) (InstigatedBy :type Controller%20Object%20Reference) (DamageCauser :type Actor%20Object%20Reference))
  (CallFunction|ApplyKnockback (- (Transformation|GetActorLocation) Origin) (* Damage (Variables|/Script/Engine.DamageType|GetDamageImpulse DamageType))))

(event Input|EnhancedActionEvents|EnhancedInputActionIACore_Look
  (params (ActionValue :type Vector%202D%20Structure) (ElapsedSeconds :type Float%20%28double-precision%29) (TriggeredSeconds :type Float%20%28double-precision%29) (InputAction :type Input%20Action%20Object%20Reference :default "/Game/Input/CoreActions/IACore_Look.IACore_Look"))
  (bind (_x _y) (Math|Vector2D|BreakVector2D ActionValue))
  (Pawn|Input|AddControllerYawInput _x)
  (Pawn|Input|AddControllerPitchInput _y))

(event EventBeginPlay
  (EventDispatchers|AssignOnTakeRadialDamage (delegate Custom|OnTakeRadialDamage_Event))
  (EventDispatchers|AssignOnTakePointDamage (delegate Custom|OnTakePointDamage_Event))
  (Utilities|Time|SetTimerbyEvent (delegate Custom|CustomEvent) 0.5)
  (bind _asplayer_controller (Utilities|Casting|CastToPlayerController (Pawn|GetController)))
  (Input|AddMappingContext (PlayerController|LocalPlayerSubsystems|GetEnhancedInputLocalPlayerSubsystem _asplayer_controller) "/Game/Input/ShipActions/IMC_Ship.IMC_Ship" 0 "(bIgnoreAllPressedKeysUntilRelease=True,bForceImmediately=False,bNotifyUserSettings=False)")
  (Game|Feedback|ClientStopCameraShake _asplayer_controller "/Game/Blueprints/Gameplay/Camera/RespawnShip/BP_RespawnShipCamShake.BP_RespawnShipCamShake_C" true))

(fn ConstructionScript)

(fn SpawnPlayer
  (bind _returnvalue (Pawn|GetController))
  (Development|PrintString "Hello" true true "(R=1.000000,G=0.038730,B=0.000000,A=1.000000)" 1e+01)
  (bind _returnvalue_2 (Game|SpawnActorfromClass "/Game/Blueprints/Gameplay/Pawns/BP_FirstPersonCharacter.BP_FirstPersonCharacter_C" (Math|Transform|MakeTransform (+ (Transformation|GetWorldLocation (Variables|Default|GetSkeletalMesh)) "0.000000,0.000000,100.000000")) "AdjustIfPossibleButAlwaysSpawn" "OverrideRootScale" _returnvalue (Game|GetInstigator)))
  (Pawn|Possess _returnvalue _returnvalue_2)
  (Actor|DestroyActor))

(fn ApplyKnockback
  (params (InDirection :type Vector) (Force :type Float%20%28double-precision%29))
  (Class|SkeletalMeshComponent|AddImpulsetoAllBodiesBelow (Variables|Default|GetSkeletalMesh) (* (+ (Math|Vector|Normalize InDirection) "0.000000,0.000000,0.400000") (* Force (Class|CommandHandlerSubsystem|GetKnockBack (Subsystems|GetCommandHandlerSubsystem)))) "None" false true))