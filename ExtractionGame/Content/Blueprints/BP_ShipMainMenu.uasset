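; BP_ShipMainMenu is a main menu spaceship actor that represents a party player, with a friend header widget attached.
; Its SetupSpaceship event waits briefly, then unhides the actor.
; It looks up the party player for its owning PlayerState through the MainMenuGameState's PartyManager and initializes the WB_FriendHeader widget with it, then prints a debug string.
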(event EventSetupSpaceship
  (Utilities|FlowControl|Delay 0.2)
  (Rendering|SetActorHiddenInGame false)
  (bind _asmain_menu_game_state (Utilities|Casting|CastToMainMenuGameState (Game|GetGameState)))
  (bind _aswb_friend_header (Utilities|Casting|CastToWB_FriendHeader (UserInterface|GetWidget (Variables|Default|GetWidget))))
  (Default|InitwithPlayer _aswb_friend_header (Class|PartyManager|GetPartyPlayer (Variables|/Script/ExtractionGame.MainMenuGameState|GetPartyManager _asmain_menu_game_state) (.AsPlayer%20State (Utilities|Casting|CastToPlayerState (Components|GetOwner)))))
  (Development|PrintText "yessir"))

(fn ConstructionScript)