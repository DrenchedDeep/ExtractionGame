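; BP_AmbientSound drives an ambient sound whose intensity drifts randomly over time.
; A looping timer started on BeginPlay periodically picks a new random target intensity in the lower half of the zero-to-one range.
; Tick eases the current intensity toward that target using delta time as the lerp alpha, then sends it to the Audio component as the "Intensity" float parameter.
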(event EventTick
  (params (DeltaSeconds :type Float%20%28single-precision%29))
  (Utilities|FlowControl|Sequence
    (:then_0
      (Variables|Default|SetIntensity (Math|Float|Lerp (Variables|Default|GetIntensity) (Variables|Default|GetTargetIntensity) DeltaSeconds)))
    (:then_1
      (Audio|Parameter|SetFloatParameter (Variables|Default|GetAudio) "Intensity" (Variables|Default|GetIntensity) :!class /Script/AudioExtensions.AudioParameterControllerInterface))))

(event EventBeginPlay
  (Utilities|Time|SetTimerbyFunctionName 0 "SwitchIntensity" 1e+01 true)
  (CallFunction|SwitchIntensity))

(fn ConstructionScript)

(fn SwitchIntensity
  (Variables|Default|SetTargetIntensity (Math|Random|RandomFloatinRange 0.0 0.5)))