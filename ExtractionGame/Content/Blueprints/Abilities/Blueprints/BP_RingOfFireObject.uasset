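; Ring of fire ability actor that grows over time and damages what lies within its radius.
; Tick increases Size up to a cap on every instance and feeds it to the Niagara effect's float parameter.
; On authority, a looping timer applies radial fireball damage at the current Size, and the actor destroys itself after a fixed lifetime.
; Sphere overlap events are empty; the local-player fire screen-parameter logic is disconnected.
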(event OnComponentBeginOverlap(Sphere)
  (params (OverlappedComponent :type Primitive%20Component%20Object%20Reference) (OtherActor :type Actor%20Object%20Reference) (OtherComp :type Primitive%20Component%20Object%20Reference) (OtherBodyIndex :type Integer) (bFromSweep :type Boolean) (SweepResult :type Hit%20Result%20Structure%20%28by%20ref%29)))

(event OnComponentEndOverlap(Sphere)
  (params (OverlappedComponent :type Primitive%20Component%20Object%20Reference) (OtherActor :type Actor%20Object%20Reference) (OtherComp :type Primitive%20Component%20Object%20Reference) (OtherBodyIndex :type Integer)))

(event Custom|DamageInsideActors
  (bind _returnvalue (Game|Damage|ApplyRadialDamage 5e+01 (+ (Transformation|GetActorLocation) "0.000000,0.000000,50.000000") (Variables|Default|GetSize) "/Game/Blueprints/Abilities/Functors/DamageTypes/DT_Fireball.DT_Fireball_C" 0 (Components|GetOwner) (Game|GetInstigatorController) false "ECC_Visibility"))
  (Development|PrintText (Utilities|Text|ToText(Boolean) _returnvalue)))

(event EventBeginPlay
  (Development|PrintText "ring of firelo")
  (Networking|SwitchHasAuthority
    (:Authority
      (Utilities|Time|SetTimerbyEvent (delegate Custom|DamageInsideActors) 1.0 true)
      (Utilities|FlowControl|Delay 11.0)
      (Actor|DestroyActor))))

(event EventTick
  (params (DeltaSeconds :type Float%20%28single-precision%29))
  (bind _output_get (Variables|Default|SetSize (Math|Float|Clamp(Float) (+ (Variables|Default|GetSize) (* DeltaSeconds (Variables|Default|GetIncreaseSpeed))) 0.0 1.5e+03)))
  (Niagara|SetNiagaraVariable(Float) (Variables|Default|GetNS_RingOfFire) "TestFloat" _output_get))

(fn ConstructionScript)