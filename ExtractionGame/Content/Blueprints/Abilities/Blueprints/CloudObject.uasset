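; CloudObject is an ability cloud actor whose size depends on its height above the surface below it.
; On BeginPlay it traces down for Hitable objects and maps the hit distance to a clamped radius for both the Capsule and the Cloud effect's FinalDist parameter.
; Without a hit, only the effect gets the maximum value, then the Cloud activates either way.
; Capsule overlap begin and end events only print the other actor's name.
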(event OnComponentBeginOverlap(Capsule)
  (params (OverlappedComponent :type Primitive%20Component%20Object%20Reference) (OtherActor :type Actor%20Object%20Reference) (OtherComp :type Primitive%20Component%20Object%20Reference) (OtherBodyIndex :type Integer) (bFromSweep :type Boolean) (SweepResult :type Hit%20Result%20Structure%20%28by%20ref%29))
  (Development|PrintString (Utilities|GetDisplayName OtherActor)))

(event OnComponentEndOverlap(Capsule)
  (params (OverlappedComponent :type Primitive%20Component%20Object%20Reference) (OtherActor :type Actor%20Object%20Reference) (OtherComp :type Primitive%20Component%20Object%20Reference) (OtherBodyIndex :type Integer))
  (Development|PrintString (Utilities|GetDisplayName OtherActor) true true "(R=1.000000,G=0.000000,B=0.112334,A=1.000000)"))

(event EventBeginPlay
  (bind _returnvalue (Transformation|GetActorLocation))
  (bind _cloud (Variables|Default|GetCloud))
  (bind (_outhit _returnvalue_2) (Collision|LineTraceForObjects _returnvalue (- _returnvalue "0.000000,0.000000,25000.000000") (Variables|Default|GetHitable) false 0 "None"))
  (if _returnvalue_2
    (Components|Capsule|SetCapsuleRadius (Variables|Default|GetCapsule) (Math|Float|Lerp 5e+01 5e+02 (Math|Float|Min(Float) (/ (Math|Vector|Distance(Vector) (.ImpactPoint (Collision|BreakHitResult _outhit)) _returnvalue) 2.5e+03) 1.0)) true)
    (Effects|Components|ParticleSystem|SetFloatParameter _cloud "FinalDist" (Math|Float|Lerp 5e+01 5e+02 (Math|Float|Min(Float) (/ (Math|Vector|Distance(Vector) (.ImpactPoint (Collision|BreakHitResult _outhit)) _returnvalue) 2.5e+03) 1.0)))
    (else
      (Effects|Components|ParticleSystem|SetFloatParameter _cloud "FinalDist" 5e+02)))
  (Components|Activation|Activate _cloud true))

(fn ConstructionScript)