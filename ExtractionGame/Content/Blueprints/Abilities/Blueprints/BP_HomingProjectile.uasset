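; Child projectile that homes toward the point where the first-person character who fired it is looking.
; SetActiveCustom toggles movement; on activation it launches forward, caches the instigator and makes the TargetLoc component the homing target.
; Each Tick teleports TargetLoc to the owner's GazeLocation, so the projectile's course follows the gaze.
; SetOwnerGaze is called on toggling but is empty, with disconnected logic for adjusting the character's IsHoming value.
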(event Custom|SetOwnerGaze
  (params (Val :type Integer)))

(event EventSetActiveCustom
  (params (isOn :type Boolean))
  (bind _projectilemovement (Variables|Default|GetProjectileMovement))
  (bind _output_get (Variables|/Script/Engine.ProjectileMovementComponent|SetbSimulationEnabled _projectilemovement isOn))
  (Components|Activation|SetActive _projectilemovement _output_get true)
  (if _output_get
    (Variables|/Script/Engine.MovementComponent|SetVelocity _projectilemovement (* (Transformation|GetActorForwardVector) (Variables|/Script/Engine.ProjectileMovementComponent|GetInitialSpeed _projectilemovement)))
    (bind _asbp_first_person_character (Utilities|Casting|CastToBP_FirstPersonCharacter (Game|GetInstigator)))
    (Variables|Default|SetOwningChar _asbp_first_person_character)
    (Variables|/Script/Engine.ProjectileMovementComponent|SetHomingTargetComponent (Variables|Default|GetProjectileMovement) (Variables|Default|GetTargetLoc))
    (CallFunction|SetOwnerGaze 1)
    (else
      (Utilities|IsValid (Components|GetOwner)
        (:Is%20Valid
          (CallFunction|SetOwnerGaze -1))))))

(event EventTick
  (params (DeltaSeconds :type Float%20%28single-precision%29))
  (bind _owningchar (Variables|Default|GetOwningChar))
  (Utilities|IsValid _owningchar
    (:Is%20Valid
      (Transformation|SetWorldLocation (Variables|Default|GetTargetLoc) (Variables|/Script/ExtractionGame.ExtractionGameCharacter|GetGazeLocation _owningchar) false true))))

(fn ConstructionScript
  (|CallParentFunction))

(fn OnPropertiesSet
  (|CallParentFunction))