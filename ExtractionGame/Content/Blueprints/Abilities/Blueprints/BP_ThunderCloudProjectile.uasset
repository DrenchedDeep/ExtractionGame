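; Thunder cloud ability projectile that spawns a lightning object at its position as it falls.
; Each tick accumulates lifetime and triggers Activate once vertical velocity is negative and a short minimum time has passed.
; Activate runs the parent logic, spawns BP_LightningObject with cooldown, radius and instigator settings, then resets the timer.
; An actor overlap sets the projectile's active state to false.
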(event Collision|EventActorBeginOverlap
  (params (OtherActor :type Actor%20Object%20Reference))
  (Class|PooledObject|SetActiveState false))

(event EventTick
  (params (DeltaSeconds :type Float%20%28single-precision%29))
  (|UpdateBaseFunction))

(fn ConstructionScript
  (|CallParentFunction))

(fn Activate
  (bind _returnvalue (Game|GetInstigator))
  (|CallParentFunction)
  (Game|SpawnActorfromClass "/Game/Blueprints/Abilities/Blueprints/BP_LightningObject.BP_LightningObject_C" (Transformation|GetActorTransform) "AlwaysSpawn" "MultiplyWithRoot" (Components|GetOwner) (Variables|Default|GetTraceCooldown) (Variables|Default|GetMinRadius) (Variables|Default|GetMaxRadius) _returnvalue _returnvalue)
  (Variables|Default|SetLife 0.0))