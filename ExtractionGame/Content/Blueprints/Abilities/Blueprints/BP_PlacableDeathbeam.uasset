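; Pooled, placeable death beam ability that deals massive damage to pawns along its up vector.
; SetActiveCustom resets effects and derives lifetime and startup delay from Power, so higher Power fires sooner and lasts longer.
; Activate spawns the Niagara beam, plays sounds and starts a looping timer that sphere-traces, scaled by actor size, until lifetime expires and the actor returns to the pool.
; The line-of-sight check is disconnected, and debug prints and trace drawing remain on.
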(event Custom|Handle%20Timers
  (bind _returnvalue (Utilities|Time|SetTimerbyEvent (delegate Custom|Timer) 0.1 true (Variables|Default|GetStartup)))
  (Variables|Default|SetHandle _returnvalue)
  (CallFunction|BoogerAids911 0.0))

(event Custom|Timer
  (bind _returnvalue (Transformation|GetActorLocation))
  (bind (_outhits _returnvalue_2) (Collision|MultiSphereTraceForObjects _returnvalue (+ _returnvalue (* (Transformation|GetActorUpVector) (Math|Conversions|ToVector(Float) (Math|Float|MakeLiteralFloat 1e+03)))) (* (.X (Math|Vector|BreakVector (Transformation|GetActorScale3D))) 25.0) (Utilities|Array|MakeArray "ObjectTypeQuery3") false 0 "ForOneFrame"))
  (if _returnvalue_2
    (for _array_element _outhits
      (Game|Damage|ApplyDamage (.HitActor (Collision|BreakHitResult _array_element)) 1e+04 (Game|GetInstigatorController) self "/Game/Blueprints/Abilities/Functors/DamageTypes/DT_Fireball.DT_Fireball_C")))
  (bind _output_get (Variables|Default|SetEndTime (- (Variables|Default|GetEndTime) 0.1)))
  (if (< _output_get 0.0)
    (Transformation|DetachFromActor "KeepWorld" "KeepWorld" "KeepWorld")
    (Class|PooledObject|ReturntoPool)
    (Utilities|Time|ClearandInvalidateTimerbyHandle (Variables|Default|GetHandle))))

(event Custom|BoogerAids911
  (params (ET :type Float%20%28double-precision%29))
  (bind _activation_noise (Variables|Default|GetActivation%20Noise))
  (bind _returnvalue (Niagara|SpawnSystemAttached "/Game/ParticleSystems/Ability/NS_Beam.NS_Beam" (Variables|Default|GetNiagara) "None" "0, 0, 0" "0, 0, 0" "KeepRelativeOffset" true false "AutoRelease"))
  (Utilities|IsValid _returnvalue
    (:Is%20Valid
      (Effects|Components|ParticleSystem|SetFloatParameter _returnvalue "Lifetime" (Variables|Default|GetEndTime))
      (Effects|Components|ParticleSystem|SetFloatParameter _returnvalue "Startup" (Variables|Default|GetStartup))
      (Components|Activation|Activate _returnvalue false)
      (Development|PrintString (Utilities|String|Append "Played" (Utilities|String|ToString(Float) (Variables|Default|GetStartup)) (Utilities|String|ToString(Float) (Variables|Default|GetEndTime))) true true "(R=1.000000,G=0.834509,B=0.000000,A=1.000000)" 5.0))
    (:Is%20Not%20Valid
      (Development|PrintString "Failed to play" true true "(R=1.000000,G=0.397846,B=0.000000,A=1.000000)" 5.0)))
  (Audio|Components|Audio|Play (Variables|Default|GetLoopingNoise) 0.0)
  (Utilities|IsValid _activation_noise
    (:Is%20Valid
      (Audio|SpawnSoundatLocation _activation_noise (Transformation|GetActorLocation) "0, 0, 0" 1.0 1.0 0.0 0 0))))

(event EventSetActiveCustom
  (params (isOn :type Boolean))
  (bind _power (Variables|Default|GetPower))
  (|CallParentFunction isOn)
  (Audio|Components|Audio|Stop (Variables|Default|GetLoopingNoise))
  (Components|Activation|SetActive (Variables|Default|GetNiagara) false true)
  (Utilities|Time|ClearandInvalidateTimerbyHandle (Variables|Default|GetHandle))
  (Variables|Default|SetEndTime (/ _power 4e+01))
  (Variables|Default|SetStartup (+ (/ (- 2e+02 _power) 1e+01) 0.5)))

(fn ConstructionScript
  (|CallParentFunction))

(fn Activate
  (CallFunction|HandleTimers))

(fn OnRepStartup)