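; BP_MagicPulse is an ability actor that releases an expanding shockwave, knocking characters away and applying a gameplay effect.
; Activate reads a DT_AttackInfo row, scales force, radius and lifetime by Power through curve tables, configures Niagara and launches the instigator upward.
; A looping timer runs CollisionDetection, growing a debug-drawn sphere overlap along an expo curve.
; Pawns inside, except the instigator, are affected every tick until the lifetime ends.
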(fn ConstructionScript)

(fn Activate
  (params (Power :type Float%20%28double-precision%29) (Row :type Name))
  (bind _niagara (Variables|Default|GetNiagara))
  (bind _returnvalue (Utilities|GetDataTableRow "/Game/DataAssets/DataTables/DT_AttackInfo.DT_AttackInfo" Row)
    (:then
      (bind _outxy (DataTable|EvaluateCurveTableRow (.CurveTable (Utilities|Struct|BreakCurveTableRowHandle (.KnockbackScaling (Utilities|Struct|BreakDStr_AttackInfo _returnvalue)))) (.RowName (Utilities|Struct|BreakCurveTableRowHandle (.KnockbackScaling (Utilities|Struct|BreakDStr_AttackInfo _returnvalue)))) Power)
        (:RowFound
          (bind _outxy_2 (DataTable|EvaluateCurveTableRow (.CurveTable (Utilities|Struct|BreakCurveTableRowHandle (.ScaleScaling (Utilities|Struct|BreakDStr_AttackInfo _returnvalue)))) (.RowName (Utilities|Struct|BreakCurveTableRowHandle (.ScaleScaling (Utilities|Struct|BreakDStr_AttackInfo _returnvalue)))) Power)
            (:RowFound
              (bind _outxy_3 (DataTable|EvaluateCurveTableRow (.CurveTable (Utilities|Struct|BreakCurveTableRowHandle (.LifetimeScaling (Utilities|Struct|BreakDStr_AttackInfo _returnvalue)))) (.RowName (Utilities|Struct|BreakCurveTableRowHandle (.LifetimeScaling (Utilities|Struct|BreakDStr_AttackInfo _returnvalue)))) Power)
                (:RowFound
                  (Variables|Default|SetLifetime (* _outxy_3 (.Lifetime (Utilities|Struct|BreakDStr_AttackInfo _returnvalue))))
                  (bind _output_get (Variables|Default|SetForce (* _outxy (.AdditionalKnockback (Utilities|Struct|BreakDStr_AttackInfo _returnvalue)))))
                  (Variables|Default|SetLevel (.EffectAbilityLevel (Utilities|Struct|BreakDStr_AttackInfo _returnvalue)))
                  (Variables|Default|SetGameplay%20Effect%20Class (.OnHitEffect (Utilities|Struct|BreakDStr_AttackInfo _returnvalue)))
                  (Variables|Default|SetMaxScale (* (* (.Scale (Utilities|Struct|BreakDStr_AttackInfo _returnvalue)) (.AoeMultiplier (Utilities|Struct|BreakDStr_AttackInfo _returnvalue))) _outxy_2))
                  (bind _returnvalue_2 (Utilities|Time|SetTimerbyFunctionName 0 "CollisionDetection" 0.1 true))
                  (Variables|Default|SetNewVar _returnvalue_2)
                  (Niagara|SetNiagaraVariable(LinearColor) _niagara "Linear Color" (.Color (Utilities|Struct|BreakDStr_AttackInfo _returnvalue)))
                  (Effects|Components|ParticleSystem|SetFloatParameter _niagara "Life" (Variables|Default|GetLifetime))
                  (Effects|Components|ParticleSystem|SetFloatParameter _niagara "Scale" (Variables|Default|GetMaxScale))
                  (bind _ascharacter (Utilities|Casting|CastToCharacter (Game|GetInstigator)))
                  (Character|LaunchCharacter _ascharacter (* (Math|Vector|VectorUp) _output_get) false true))))))))
    (:RowNotFound
      (Development|PrintString "Failed to find row"))))

(fn CollisionDetection
  (bind _returnvalue (Transformation|GetActorLocation))
  (bind _outxy (DataTable|EvaluateCurveTableRow "/Game/DataAssets/0-1ExpoCurve.0-1ExpoCurve" "Pulse" (/ (Variables|Default|GetCurrentTime) (Variables|Default|GetLifetime)))
    (:RowFound
      (bind _outactors (Collision|SphereOverlapActors _returnvalue (Math|Float|Lerp 0.0 (Variables|Default|GetMaxScale) _outxy) (Utilities|Array|MakeArray "ObjectTypeQuery3") "/Script/Engine.Pawn" (Utilities|Array|MakeArray (Game|GetInstigator))))
      (for _array_element _outactors
        (bind _ascharacter (Utilities|Casting|CastToCharacter _array_element)
          (:then
            (Character|LaunchCharacter _ascharacter (* (+ (Math|Vector|Normalize (- (Transformation|GetActorLocation _array_element) _returnvalue)) (Math|Vector|VectorUp)) (Variables|Default|GetForce)) true true))
          (:CastFailed
            _))
        (Utilities|IsValid (Ability|GetAbilitySystemComponent _ascharacter)
          (:Is%20Valid
            (GameplayEffects|ApplyGameplayEffectToSelf :self (Ability|GetAbilitySystemComponent _ascharacter) :GameplayEffectClass (Variables|Default|GetGameplay%20Effect%20Class) :Level (Variables|Default|GetLevel)))))
      (Rendering|Debug|DrawDebugSphere _returnvalue (Math|Float|Lerp 0.0 (Variables|Default|GetMaxScale) _outxy) 12 "(R=1.000000,G=1.000000,B=1.000000,A=1.000000)" 2.0)
      (bind _output_get (Variables|Default|SetCurrentTime (+ 0.1 (Variables|Default|GetCurrentTime))))
      (Development|PrintString (Utilities|String|Append "Repulsor Tick % " (Utilities|String|ToString(Float) (/ _output_get (Variables|Default|GetLifetime)))))
      (if (>= _output_get (Variables|Default|GetLifetime))
        (Utilities|Time|ClearandInvalidateTimerbyHandle (Variables|Default|GetNewVar))
        (Actor|SetLifeSpan 1.0)))))