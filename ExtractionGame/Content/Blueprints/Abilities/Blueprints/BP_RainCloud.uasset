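; Rain cloud ability actor that repeatedly applies a gameplay effect to actors with an Ability System Component overlapping its capsule.
; SetStats reads DT_AttackInfo, scales damage and radius by Power through curve tables, and starts a fast looping Effect timer.
; A downward trace stores the column's midpoint and half-height, with fallback values on a miss, then the actor destroys itself after its lifetime.
; Computed damage and dimensions are only stored in these graphs.
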(event EventSetStats
  (params (Stats :type Name :default "None") (Power :type Float%20%28double-precision%29))
  (bind _returnvalue (Math|Float|MakeLiteralFloat 5e+03))
  (bind _returnvalue_2 (Transformation|GetActorUpVector))
  (bind _returnvalue_3 (Transformation|GetActorLocation))
  (bind _returnvalue_4 (+ _returnvalue_3 "0.000000,0.000000,50.000000"))
  (bind _returnvalue_5 (Utilities|GetDataTableRow "/Game/DataAssets/DataTables/DT_AttackInfo.DT_AttackInfo" Stats)
    (:then
      (bind _returnvalue_6 (Utilities|Time|SetTimerbyFunctionName 0 "Effect" 0.18 true))
      (Variables|Default|SetTimer _returnvalue_6)
      (bind _outxy (DataTable|EvaluateCurveTableRow (.CurveTable (Utilities|Struct|BreakCurveTableRowHandle (.DamageScaling (Utilities|Struct|BreakDStr_AttackInfo _returnvalue_5)))) (.RowName (Utilities|Struct|BreakCurveTableRowHandle (.DamageScaling (Utilities|Struct|BreakDStr_AttackInfo _returnvalue_5)))) Power)
        (:RowFound
          (Variables|Default|SetDamage (* (.Damage (Utilities|Struct|BreakDStr_AttackInfo _returnvalue_5)) _outxy))
          (Variables|Default|SetDamage%20Type (.DamageType (Utilities|Struct|BreakDStr_AttackInfo _returnvalue_5)))
          (Variables|Default|SetOn%20Hit%20Effect (.OnHitEffect (Utilities|Struct|BreakDStr_AttackInfo _returnvalue_5)))
          (Variables|Default|SetEffect%20Ability%20Level (.EffectAbilityLevel (Utilities|Struct|BreakDStr_AttackInfo _returnvalue_5)))
          (bind _outxy_2 (DataTable|EvaluateCurveTableRow (.CurveTable (Utilities|Struct|BreakCurveTableRowHandle (.ScaleScaling (Utilities|Struct|BreakDStr_AttackInfo _returnvalue_5)))) (.RowName (Utilities|Struct|BreakCurveTableRowHandle (.ScaleScaling (Utilities|Struct|BreakDStr_AttackInfo _returnvalue_5)))) Power)
            (:RowFound
              (Variables|Default|SetRadius (* (* (.Scale (Utilities|Struct|BreakDStr_AttackInfo _returnvalue_5)) (* _outxy_2 (.AoeMultiplier (Utilities|Struct|BreakDStr_AttackInfo _returnvalue_5)))) 1e+01))
              (bind (_outhit _returnvalue_7) (Class|KismetSystemLibrary|LineTraceSinglebyProfile _returnvalue_4 (+ _returnvalue_3 (* (Math|Vector|NegateVector (Transformation|GetActorUpVector)) (Math|Conversions|ToVector(Float) 1e+04))) "WorldStatic" true 0 "ForDuration" true))
              (if _returnvalue_7
                (Development|PrintText (Utilities|Text|ToText(String) (Utilities|GetDisplayName (.HitActor (Collision|BreakHitResult _outhit)))))
                (Variables|Default|SetMidPoint (* (/ (Math|Vector|Distance(Vector) (.ImpactPoint (Collision|BreakHitResult _outhit)) _returnvalue_4) 2.0) _returnvalue_2))
                (Variables|Default|SetHeight (/ (Math|Vector|Distance(Vector) (.ImpactPoint (Collision|BreakHitResult _outhit)) _returnvalue_4) 2.0))
                (else
                  (Variables|Default|SetMidPoint (* _returnvalue _returnvalue_2))
                  (Variables|Default|SetHeight _returnvalue)))
              (Utilities|FlowControl|Delay (.Lifetime (Utilities|Struct|BreakDStr_AttackInfo _returnvalue_5)))
              (Actor|DestroyActor))))))))

(fn ConstructionScript)

(fn Effect
  (for _array_element (Collision|GetOverlappingActors (Variables|Default|GetCapsule) 0 :!class /Script/Engine.PrimitiveComponent)
    (Utilities|IsValid (Ability|GetAbilitySystemComponent _array_element)
      (:Is%20Valid
        (GameplayEffects|ApplyGameplayEffectToSelf :self (Ability|GetAbilitySystemComponent _array_element) :GameplayEffectClass (Variables|Default|GetOn%20Hit%20Effect) :Level (Variables|Default|GetEffect%20Ability%20Level))))))