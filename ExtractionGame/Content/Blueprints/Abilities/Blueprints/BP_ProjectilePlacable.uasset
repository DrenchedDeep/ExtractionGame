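; Placeable ability projectile that launches as a physics sphere and later turns into a colored volume object.
; SetActiveCustom toggles physics and launches it forward at the movement component's initial speed.
; OnHit stops it on surfaces whose normal roughly matches the sphere's up vector, aligns it to that normal and extends its lifespan.
; Activate spawns the volume and deactivates the projectile; Power and Color drive the mesh's material look.
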(event EventBeginPlay
  (|CallParentFunction)
  (Variables|Default|SetHitEffect 0))

(event EventSetActiveCustom
  (params (isOn :type Boolean))
  (bind _sphere (Variables|Default|GetSphere))
  (Physics|SetSimulatePhysics _sphere isOn)
  (if isOn
    (Physics|SetPhysicsLinearVelocity _sphere (* (Transformation|GetActorForwardVector) (Variables|/Script/Engine.ProjectileMovementComponent|GetInitialSpeed (Variables|Default|GetProjectileMovement))) false "None")))

(event EventTick
  (params (DeltaSeconds :type Float%20%28single-precision%29)))

(fn ConstructionScript
  (|CallParentFunction))

(fn OnHit
  (params (HitActor :type Actor%20Object%20Reference) (HitResult :type Hit%20Result%20Structure))
  (bind (_bblockinghit _binitialoverlap _time _distance _location _impactpoint _normal _impactnormal) (Collision|BreakHitResult HitResult))
  (bind _sphere (Variables|Default|GetSphere))
  (if (> (Math|Vector|DotProduct _impactnormal (Math|Vector|GetUpVector _sphere)) 0.7)
    (Physics|SetSimulatePhysics _sphere false)
    (Transformation|AttachComponentToComponent 0 "None" "KeepRelative" "KeepRelative" "KeepRelative" true)
    (Transformation|SetWorldLocationAndRotation _sphere _location (Math|Rotator|MakeRotfromZ _impactnormal) false true)
    (Actor|SetLifeSpan 1e+06)))

(fn Activate
  (|CallParentFunction)
  (bind _returnvalue (Game|SpawnActorfromClass "/Game/Blueprints/Abilities/Blueprints/VolumeObject.VolumeObject_C" (Transformation|GetActorTransform) "AlwaysSpawn" "MultiplyWithRoot" 0 0))
  (Default|SetColor _returnvalue (Variables|Default|GetColor))
  (Class|PooledObject|SetActiveState false)
  (Development|PrintString "BOOM"))

(fn OnPropertiesSet
  (bind _color (Variables|Default|GetColor))
  (bind _staticmesh (Variables|Default|GetStaticMesh))
  (bind (_r _g _b _a) (Math|Color|BreakColor _color))
  (|CallParentFunction)
  (Audio|Parameter|SetFloatParameter _staticmesh "EmissivePower" (* (Variables|Default|GetPower) 2e+01) :!class /Script/AudioExtensions.AudioParameterControllerInterface)
  (Class|PrimitiveComponent|SetVectorParameterforCustomPrimitiveData _staticmesh "Color" (Math|Vector4|MakeVector4 _r _g _b _a))
  (Development|PrintString "Properties Set"))