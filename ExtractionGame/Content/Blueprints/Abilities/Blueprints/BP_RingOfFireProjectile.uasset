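; BP_RingOfFireProjectile is a pooled ability projectile that places a ring of fire in the world.
; On sphere overlap it spawns BP_RingOfFireObject at its location, deactivates and returns to the pool.
; One second after an activation, a downward line trace also spawns an actor at any ground hit and recycles the projectile, though that spawn shows no class.
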(event OnComponentBeginOverlap(Sphere)
  (params (OverlappedComponent :type Primitive%20Component%20Object%20Reference) (OtherActor :type Actor%20Object%20Reference) (OtherComp :type Primitive%20Component%20Object%20Reference) (OtherBodyIndex :type Integer) (bFromSweep :type Boolean) (SweepResult :type Hit%20Result%20Structure%20%28by%20ref%29))
  (Game|SpawnActorfromClass "/Game/Blueprints/Abilities/Blueprints/BP_RingOfFireObject.BP_RingOfFireObject_C" (Math|Transform|MakeTransform (Transformation|GetActorLocation) "0, 0, 0" "1.000000,1.000000,1.000000") "AlwaysSpawn" "MultiplyWithRoot" 0 0)
  (Development|PrintText "is spawneing")
  (Class|PooledObject|SetActiveState false)
  (Class|PooledObject|ReturntoPool))

(event EventSetActiveCustom
  (params (isOn :type Boolean))
  (bind _returnvalue (Transformation|GetActorLocation))
  (|CallParentFunction isOn)
  (Utilities|FlowControl|Delay 1.0)
  (if isOn
    (bind (_outhit _returnvalue_2) (Collision|LineTraceByChannel _returnvalue (+ _returnvalue (* (Math|Vector|VectorDown) 1e+04)) "TraceTypeQuery1" false 0 "None"))
    (if _returnvalue_2
      (Game|SpawnActorfromClass "/Game/Blueprints/Abilities/Blueprints/BP_RingOfFireObject.BP_RingOfFireObject_C" (Math|Transform|MakeTransform (.ImpactPoint (Collision|BreakHitResult _outhit))) "AlwaysSpawn" "MultiplyWithRoot" 0 0)
      (Development|PrintText "is spawneing")
      (Class|PooledObject|SetActiveState false)
      (Class|PooledObject|ReturntoPool))))

(fn ConstructionScript
  (|CallParentFunction))