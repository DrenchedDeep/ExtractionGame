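; Pooled gravity-based projectile that deploys an actor once it starts to descend.
; When properties are set, a looping timer polls vertical velocity and calls Activate when it turns negative.
; Activate spawns the SpawnOnDeath class on the authority only, passes it group name and power, then returns the projectile to the pool.
; Hits return it to the pool without deploying, and SetActiveCustom clears the timer.
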(event EventSetActiveCustom
  (params (isOn :type Boolean))
  (|CallParentFunction isOn)
  (Utilities|Time|ClearandInvalidateTimerbyHandle (Variables|Default|GetTimerHandle)))

(fn ConstructionScript)

(fn Activate
  (Networking|SwitchHasAuthority
    (:Authority
      (bind _returnvalue (Game|SpawnActorfromClass (.SpawnOnDeath (Utilities|Struct|BreakDStr_AttackInfo (Variables|Default|GetProperties))) (Transformation|GetActorTransform) "AlwaysSpawn" "OverrideRootScale" (Components|GetOwner) (Game|GetInstigator)))
      (Class|IAttackInfoSettable|SetStats(Message) _returnvalue (Variables|Default|GetGroup%20Name) (Variables|Default|GetPower)) ; If needed, instead of using the same structure, it can use a new one
    )
    (:Remote
      _))
  (Class|PooledObject|ReturntoPool)
  (Development|PrintString "Succeesfully Deployed" true true "(R=0.000000,G=0.660000,B=1.000000,A=1.000000)" 1e+01))

(fn OnPropertiesSet
  (|CallParentFunction)
  (bind _returnvalue (Utilities|Time|SetTimerbyFunctionName 0 "CheckCanDeploy" 0.1 true 0.2 0.2))
  (Variables|Default|SetTimerHandle _returnvalue)
  (Development|PrintString "Bound timer successfully" true true "(R=1.000000,G=0.583201,B=0.000000,A=1.000000)" 15.0))

(fn CheckCanDeploy
  (Development|PrintString "Seen by" true true "(R=0.955806,G=1.000000,B=0.966854,A=1.000000)" 5.0)
  (if (< (.Z (Math|Vector|BreakVector (Variables|/Script/Engine.MovementComponent|GetVelocity (Variables|Default|GetProjectileMovement)))) 0.0)
    (CallFunction|Activate)))

(fn OnHit
  (params (HitActor :type Actor%20Object%20Reference) (HitResult :type Hit%20Result%20Structure))
  (Class|PooledObject|ReturntoPool))