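; Frost bomb projectile that spawns a follow-up actor once, either on overlap or in mid-air as it descends.
; Tick tracks lifetime and triggers Activate when vertical velocity turns negative after a short minimum flight time, printing a debug message.
; Activate spawns the class taken from the SpawnOnDeath property at its transform, passing on owner and instigator, then deactivates the bomb behind a Spawned guard.
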(event Collision|EventActorBeginOverlap
  (params (OtherActor :type Actor%20Object%20Reference))
  (Class|PooledObject|SetActiveState false)
  (CallFunction|Activate))

(event EventTick
  (params (DeltaSeconds :type Float%20%28single-precision%29))
  (if (not (Variables|Default|GetSpawned))
    (bind _output_get (Variables|Default|SetLife (+ (Variables|Default|GetLife) (Utilities|Time|GetWorldDeltaSeconds))))
    (if (and (< (.Z (Math|Vector|BreakVector (Variables|/Script/Engine.MovementComponent|GetVelocity (Variables|Default|GetProjectileMovement)))) 0.0) (> _output_get 0.8))
      (CallFunction|Activate)
      (Development|PrintText "spawno"))))

(fn ConstructionScript
  (|CallParentFunction))

(fn Activate
  (if (not (Variables|Default|GetSpawned))
    (Game|SpawnActorfromClass (Variables|Default|GetSpawnedActor) (Transformation|GetActorTransform) "AlwaysSpawn" "OverrideRootScale" (Components|GetOwner) (Game|GetInstigator))
    (Class|PooledObject|SetActiveState false)
    (Variables|Default|SetLife 0.0)
    (Variables|Default|SetSpawned true)))

(fn OnPropertiesSet
  (|CallParentFunction)
  (Variables|Default|SetSpawnedActor (.spawnondeath (Variables|Default|GetProperties))))