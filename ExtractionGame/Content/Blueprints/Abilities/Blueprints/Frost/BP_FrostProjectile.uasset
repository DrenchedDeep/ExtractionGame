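; Frost ability projectile that deactivates on hit, rather than destroying itself, and spawns a frost impact actor.
; On collision it hides its Niagara trail, and the authority sphere-traces forward to place a short-lived BP_FrostImpact aligned to the surface normal.
; Activate spawns the configured SpawnedActor only once, then deactivates the projectile.
; OnPropertiesSet shows the trail again and randomly scales the spin component's roll and pitch.
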(event OnComponentHit(Sphere)
  (params (HitComponent :type Primitive%20Component%20Object%20Reference) (OtherActor :type Actor%20Object%20Reference) (OtherComp :type Primitive%20Component%20Object%20Reference) (NormalImpulse :type Vector :default "0, 0, 0") (Hit :type Hit%20Result%20Structure%20%28by%20ref%29))
  (bind _arrow (Variables|Default|GetArrow))
  (bind _returnvalue (Transformation|GetWorldLocation _arrow))
  (Rendering|SetVisibility (Variables|Default|GetNS_ProjectileTrail1) false false)
  (Networking|SwitchHasAuthority
    (:Authority
      (Class|PooledObject|SetActiveState false)
      (Rendering|SetVisibility (Variables|Default|GetNS_ProjectileTrail1) false false)
      (bind (_outhit _returnvalue_2) (Collision|SphereTraceByChannel _returnvalue (+ _returnvalue (* (Transformation|GetActorForwardVector) 2e+02)) 5e+01 "TraceTypeQuery1" false 0 "None"))
      (if _returnvalue_2
        (bind _returnvalue_3 (Game|SpawnActorfromClass "/Game/BP_FrostImpact.BP_FrostImpact_C" (Math|Transform|MakeTransform (+ (.ImpactPoint (Collision|BreakHitResult _outhit)) (* (.ImpactNormal (Collision|BreakHitResult _outhit)) 2e+01)) (Math|Conversions|RotationFromXVector (.ImpactNormal (Collision|BreakHitResult _outhit))) "1.000000,1.000000,1.000000") "Undefined" "MultiplyWithRoot" 0 0))
        (Actor|SetLifeSpan _returnvalue_3 2e+01)))))

(fn ConstructionScript
  (|CallParentFunction))

(fn Activate
  (if (not (Variables|Default|GetSpawned))
    (Game|SpawnActorfromClass (Variables|Default|GetSpawnedActor) (Transformation|GetActorTransform) "AlwaysSpawn" "OverrideRootScale" (Components|GetOwner) (Game|GetInstigator))
    (Class|PooledObject|SetActiveState false)
    (Variables|Default|SetLife 0.0)
    (Variables|Default|SetSpawned true)))

(fn OnPropertiesSet
  (bind _spincomp (Variables|Default|GetSpinComp))
  (bind _returnvalue (Transformation|GetWorldRotation _spincomp))
  (Rendering|SetVisibility (Variables|Default|GetNS_ProjectileTrail1) true false)
  (Transformation|SetWorldRotation _spincomp (Math|Rotator|MakeRotator (* (Math|Random|RandomFloatinRange 0.0 45.0) (.roll _returnvalue)) (* (.pitch _returnvalue) (Math|Random|RandomFloatinRange 0.0 45.0)) (.yaw _returnvalue)) false false)
  (Rendering|SetVisibility (Variables|Default|GetNS_ProjectileTrail1) true false))