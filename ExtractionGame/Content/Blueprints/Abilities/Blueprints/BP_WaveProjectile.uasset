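; Wave ability projectile, a child Blueprint that overrides its parent's hit response to damage and knock back whatever it strikes.
; On the server, when hits are allowed, it applies point damage and the configured Gameplay Effect to targets with an Ability System Component.
; Characters are then launched along the projectile's forward vector by the calculated knockback, overriding their velocity.
; Construction and property setup defer to the parent, and a node aligning Niagara to velocity is left unconnected.
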(fn ConstructionScript
  (|CallParentFunction))

(fn OnHit
  (params (HitActor :type Actor%20Object%20Reference) (HitResult :type Hit%20Result%20Structure))
  (bind _returnvalue (Ability|GetAbilitySystemComponent HitActor))
  (bind _returnvalue_2 (Transformation|GetActorForwardVector))
  (bind _properties (Variables|Default|GetProperties))
  (bind (_modify_particlesystem _color _damage _damagescaling _damagetype _additionalknockback _knockbackscaling _onhiteffect _effectabilitylevel) (Utilities|Struct|BreakDStr_AttackInfo _properties))
  (if (and (Variables|Default|GetCanHit) (Ability|HasAuthority))
    (Game|Damage|ApplyPointDamage HitActor (Variables|Default|GetCalcDamage) _returnvalue_2 HitResult (Game|GetInstigatorController) self _damagetype)
    (Utilities|IsValid _returnvalue
      (:Is%20Valid
        (GameplayEffects|ApplyGameplayEffectToSelf :self _returnvalue :GameplayEffectClass _onhiteffect :Level _effectabilitylevel))
      (:Is%20Not%20Valid
        _))
    (bind _ascharacter (Utilities|Casting|CastToCharacter HitActor))
    (Character|LaunchCharacter _ascharacter (* _returnvalue_2 (Variables|Default|GetCalcKnockback)) true true)))

(fn OnPropertiesSet
  (|CallParentFunction))