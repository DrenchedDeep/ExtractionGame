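; Base pooled ability projectile that deals area fireball damage on impact, with gravity and color read from DT_AttackInfo and power set by the caller.
; Sphere hits and overlaps ignore the instigator, then gather nearby characters and damage those whose line trace returns a hit.
; Damage is server-only, damage numbers also spawn for the autonomous-proxy owner, and HitEffect particles spawn only on remotes.
; With a valid HitEffect, the projectile then returns to its pool.
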(event OnComponentBeginOverlap(Sphere)
  (params (OverlappedComponent :type Primitive%20Component%20Object%20Reference) (OtherActor :type Actor%20Object%20Reference) (OtherComp :type Primitive%20Component%20Object%20Reference) (OtherBodyIndex :type Integer) (bFromSweep :type Boolean) (SweepResult :type Hit%20Result%20Structure%20%28by%20ref%29))
  (CallFunction|ValidateHit OtherActor SweepResult))

(event OnComponentHit(Sphere)
  (params (HitComponent :type Primitive%20Component%20Object%20Reference) (OtherActor :type Actor%20Object%20Reference) (OtherComp :type Primitive%20Component%20Object%20Reference) (NormalImpulse :type Vector :default "0, 0, 0") (Hit :type Hit%20Result%20Structure%20%28by%20ref%29))
  (CallFunction|ValidateHit OtherActor Hit))

(event EventBeginPlay
  (Niagara|SetNiagaraVariable(Float) (Variables|Default|GetNiagara) "MySCale" (* (Class|SphereComponent|GetShapeScale (Variables|Default|GetSphere)) 85.0))
  (Game|Components|ProjectileMovement|Interpolation|SetInterpolatedComponent (Variables|Default|GetProjectileMovement) (Variables|Default|GetNiagara)))

(event EventSetAttributes
  (params (power :type Float%20%28single-precision%29) (groupName :type Name :default "None"))
  (Variables|Default|SetPower power)
  (bind _returnvalue (Utilities|GetDataTableRow "/Game/DataAssets/DataAssets/DT_AttackInfo.DT_AttackInfo" groupName)
    (:then
      (Variables|/Script/Engine.ProjectileMovementComponent|SetProjectileGravityScale (Variables|Default|GetProjectileMovement) (.Gravity (Utilities|Struct|BreakDStr_AttackInfo _returnvalue)))
      (Variables|Default|SetColor (.Color (Utilities|Struct|BreakDStr_AttackInfo _returnvalue)))
      (CallFunction|OnPropertiesSet))))

(event EventSetActiveCustom
  (params (isOn :type Boolean))
  (bind _projectilemovement (Variables|Default|GetProjectileMovement))
  (bind _output_get (Variables|/Script/Engine.ProjectileMovementComponent|SetbSimulationEnabled _projectilemovement isOn))
  (Components|Activation|SetActive _projectilemovement _output_get true)
  (Variables|/Script/Engine.MovementComponent|SetVelocity _projectilemovement (* (Transformation|GetActorForwardVector) (Variables|/Script/Engine.ProjectileMovementComponent|GetInitialSpeed _projectilemovement)))
  (Components|Activation|SetActive (Variables|Default|GetNiagara) _output_get true))

(event Custom|Spawn%20Particle
  (params (Color :type Linear%20Color%20Structure))
  (bind _returnvalue (Transformation|GetActorTransform))
  (bind (_location _rotation _scale) (Math|Transform|BreakTransform _returnvalue))
  (Networking|SwitchHasAuthority
    (:Remote
      (bind _returnvalue_2 (Niagara|SpawnSystematLocation (Variables|Default|GetHitEffect) _location _rotation _scale true true "AutoRelease"))
      (Niagara|SetNiagaraVariable(LinearColor) _returnvalue_2 "Linear Color" (Variables|Default|GetColor)))))

(fn ConstructionScript)

(fn SetSize
  (params (NewSize :type Float%20%28double-precision%29))
  (Niagara|SetNiagaraVariable(Float) (Variables|Default|GetNiagara) "Scale" (* NewSize 1e+01)))

(fn OnHit
  (params (HitActor :type Actor%20Object%20Reference) (HitResult :type Hit%20Result%20Structure))
  (bind _location (Collision|BreakHitResult HitResult))
  (if (Variables|Default|GetCanHit)
    (bind _outactors (Collision|SphereOverlapActors _location (* (Components|Sphere|GetScaledSphereRadius (Variables|Default|GetSphere)) 5.0) (LocalVariables|GetHitableActors) "/Script/Engine.Character"))
    (for _array_element _outactors
      (bind _returnvalue (Collision|LineTraceForObjects _location (Transformation|GetActorLocation _array_element) (LocalVariables|GetBlockingActors) false 0 "None"))
      (if _returnvalue
        (Networking|SwitchHasAuthority
          (:Authority
            (Game|Damage|ApplyDamage _array_element (Variables|Default|GetPower) (Game|GetInstigatorController) self "/Game/Blueprints/Abilities/Functors/DamageTypes/BP_FireballDamageType.BP_FireballDamageType_C"))
          (:Remote
            _))
        (if (or (Ability|HasAuthority) (Utilities|Enum|Equal(Enum) (Networking|GetLocalRole (Components|GetOwner)) "ROLE_AutonomousProxy"))
          (Game|SpawnActorfromClass "/Game/Blueprints/Widgets/Player/BP_DamageAmount.BP_DamageAmount_C" (Transformation|GetActorTransform _array_element) "Undefined" "MultiplyWithRoot" 0 (Variables|Default|GetPower) 0))))
    (Utilities|IsValid (Variables|Default|GetHitEffect)
      (:Is%20Valid
        (CallFunction|SpawnParticle)
        (Actor|Tick|SetActorTickEnabled false)
        (Class|PooledObject|ReturntoPool)))))

(fn Activate)

(fn ValidateHit
  (params (InActor :type Actor%20Object%20Reference) (Hit :type Hit%20Result%20Structure))
  (if (not (== InActor (Game|GetInstigator)))
    (CallFunction|OnHit InActor Hit)))

(fn OnPropertiesSet)