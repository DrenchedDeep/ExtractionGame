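; Lightning rain cloud ability that extends its parent's Effect with randomly placed, damaging lightning strikes.
; Effect traces downward from a random point above the actor and, on a hit, spawns a Niagara bolt fed with start, end and surface normal.
; CheckForPlayers then applies radial damage with falloff just above the impact point and prints the result.
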(fn ConstructionScript
  (|CallParentFunction))

(fn Effect
  (bind _returnvalue (Math|Random|RandomFloatinRange -1.0 1.0))
  (bind _returnvalue_2 (Math|Random|RandomFloatinRange -1.0 1.0))
  (bind _returnvalue_3 (Transformation|GetActorLocation))
  (bind _returnvalue_4 (Math|Vector|MakeVector _returnvalue_2 _returnvalue 1.0))
  (bind _returnvalue_5 (* _returnvalue_4 8e+02))
  (bind _returnvalue_6 (Math|Vector|MakeVector (.x _returnvalue_5) (.y _returnvalue_5) 8e+02))
  (bind _returnvalue_7 (+ _returnvalue_3 _returnvalue_6))
  (|CallParentFunction)
  (if (>= (- (Utilities|Time|GetTimeSeconds) 0.0) 0.0)
    (bind _outhit (Collision|LineTraceByChannel _returnvalue_7 (+ _returnvalue_7 (* (Math|Vector|VectorDown) 5e+03)) "TraceTypeQuery1" false 0 "None"))
    (if (.bBlockingHit (Collision|BreakHitResult _outhit))
      (bind _returnvalue_8 (Niagara|SpawnSystematLocation "/Game/ParticleSystems/Ability/NS_Lightning.NS_Lightning" "0, 0, 0"))
      (Utilities|IsValid _returnvalue_8
        (:Is%20Valid
          (Niagara|SetNiagaraVariable(Vector3) _returnvalue_8 "StartLocation" _returnvalue_7)
          (Niagara|SetNiagaraVariable(Vector3) _returnvalue_8 "EndLocation" (+ (.ImpactPoint (Collision|BreakHitResult _outhit)) (* (.ImpactNormal (Collision|BreakHitResult _outhit)) (LocalVariables|GetImpactOffset))))
          (Niagara|SetNiagaraVariable(Vector3) _returnvalue_8 "ImpactNormal" (.ImpactNormal (Collision|BreakHitResult _outhit)))
          (CallFunction|CheckforPlayers (+ (.ImpactPoint (Collision|BreakHitResult _outhit)) (* (.ImpactNormal (Collision|BreakHitResult _outhit)) (LocalVariables|GetImpactOffset)))))))))

(fn CheckforPlayers
  (params (Location :type Vector))
  (bind _returnvalue (Class|GameplayStatics|ApplyRadialDamagewithFalloff 45.0 1e+01 (+ Location "0.000000,0.000000,100.000000") 1e+02 2e+02 1.0 0 0 self (Game|GetInstigatorController) "ECC_Visibility"))
  (Development|PrintText (Utilities|Text|ToText(Boolean) _returnvalue)))