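; BP_BurstProjectile is a one-shot spawner actor that releases a burst of pooled objects when it begins play.
; It pulls Num objects of the configured Type from the pool handler subsystem, placing each above itself with a random direction inside a cone around its up vector.
; Each object inherits the burst's owner, instigator and group name, gets a fixed power and is activated, then the spawner destroys itself.
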(event EventBeginPlay
  (bind _returnvalue (Transformation|GetActorUpVector))
  (for _index (range 1 (Variables|Default|GetNum))
    (bind _returnvalue_2 (Class|PoolHandlerSubSystem|SpawnObject (Subsystems|GetPoolHandlerSubSystem) (Variables|Default|GetType)))
    (Transformation|SetActorTransform _returnvalue_2 (Math|Transform|MakeTransform (+ (* _returnvalue (Math|Conversions|ToVector(Float) 1.5e+02)) (Transformation|GetActorLocation)) (Math|Conversions|RotationFromXVector (Math|Random|RandomUnitVectorinConeinDegrees _returnvalue (Variables|Default|GetAngle)))) false true)
    (Actor|SetOwner _returnvalue_2 (Components|GetOwner))
    (Variables|/Script/Engine.Actor|SetInstigator _returnvalue_2 (Game|GetInstigator))
    (Class|PooledObject|SetAttributes _returnvalue_2 5e+01 (Variables|Default|GetGroupName))
    (Class|PooledObject|SetActiveState _returnvalue_2 true))
  (Actor|DestroyActor))

(fn ConstructionScript)