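; Pooled meteor ability actor that explodes on hit, dealing area damage.
; On hit, the authority applies radial explosive damage with falloff from a point raised above the impact, using the calculated damage and AoE.
; It also spawns an auto-released Niagara explosion scaled to the AoE, then calls Activate and returns itself to the pool.
; SetActiveCustom defers to the parent and prints the new state for debugging.
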(event EventSetActiveCustom
  (params (isOn :type Boolean))
  (|CallParentFunction isOn)
  (Development|PrintString (Utilities|String|Append "Setting Meteor State: " (Utilities|String|ToString(Boolean) isOn))))

(fn ConstructionScript)

(fn OnHit
  (params (HitActor :type Actor%20Object%20Reference) (HitResult :type Hit%20Result%20Structure))
  (bind _returnvalue (Transformation|GetActorLocation))
  (bind _calcaoe (Variables|Default|GetCalcAoe))
  (Utilities|FlowControl|Sequence
    (:then_0
      (Networking|SwitchHasAuthority
        (:Authority
          (Development|PrintString "Meteor Activate")
          (Class|GameplayStatics|ApplyRadialDamagewithFalloff (Variables|Default|GetCalcDamage) 25.0 (+ _returnvalue (* (Math|Vector|VectorUp) (* _calcaoe 0.25))) (/ _calcaoe 3.0) _calcaoe 2.0 "/Game/Blueprints/Abilities/Functors/DamageTypes/DT_Explosive.DT_Explosive_C" 0 self (Game|GetInstigatorController) "ECC_WorldStatic"))
        (:Remote
          _))
      (bind _returnvalue_2 (Niagara|SpawnSystematLocation "/Game/ParticleSystems/NS_Explosion.NS_Explosion" _returnvalue "0, 0, 0" "1.000000,1.000000,1.000000" true true "AutoRelease"))
      (Utilities|IsValid _returnvalue_2
        (:Is%20Valid
          (Effects|Components|ParticleSystem|SetFloatParameter _returnvalue_2 "Size" (/ _calcaoe 5e+02)))))
    (:then_1
      (CallFunction|Activate)
      (Class|PooledObject|ReturntoPool))))