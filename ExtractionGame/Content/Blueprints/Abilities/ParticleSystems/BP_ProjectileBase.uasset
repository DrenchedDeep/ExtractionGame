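; Base projectile Blueprint that damages whatever it hits, other than its instigator, then destroys itself.
; Sphere hit and overlap events feed ValidateHit into OnHit, which applies fixed fireball-type damage on the authority only, credited to the owning first-person character.
; Niagara scale follows the sphere's scale at BeginPlay, while SetSize writes a differently named parameter.
; SetProperties stores power and color, then calls an empty OnPropertiesSet; Activate is also empty.
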(event OnComponentBeginOverlap(Sphere)
  (params (OverlappedComponent :type Primitive%20Component%20Object%20Reference) (OtherActor :type Actor%20Object%20Reference) (OtherComp :type Primitive%20Component%20Object%20Reference) (OtherBodyIndex :type Integer) (bFromSweep :type Boolean) (SweepResult :type Hit%20Result%20Structure%20%28by%20ref%29))
  (CallFunction|ValidateHit OtherActor SweepResult))

(event OnComponentHit(Sphere)
  (params (HitComponent :type Primitive%20Component%20Object%20Reference) (OtherActor :type Actor%20Object%20Reference) (OtherComp :type Primitive%20Component%20Object%20Reference) (NormalImpulse :type Vector :default "0, 0, 0") (Hit :type Hit%20Result%20Structure%20%28by%20ref%29))
  (CallFunction|ValidateHit OtherActor Hit))

(event EventBeginPlay
  (bind _asbp_first_person_character (Utilities|Casting|CastToBP_FirstPersonCharacter (Game|GetInstigator)))
  (Variables|Default|SetOwningPlayer _asbp_first_person_character)
  (Niagara|SetNiagaraVariable(Float) (Variables|Default|GetNiagara) "MySCale" (* (Class|SphereComponent|GetShapeScale (Variables|Default|GetSphere)) 75.0)))

(fn ConstructionScript)

(fn SetSize
  (params (NewSize :type Float%20%28double-precision%29))
  (Niagara|SetNiagaraVariable(Float) (Variables|Default|GetNiagara) "Scale" (* NewSize 1e+01)))

(fn OnHit
  (params (HitActor :type Actor%20Object%20Reference) (HitResult :type Hit%20Result%20Structure))
  (if (Ability|HasAuthority)
    (Game|Damage|ApplyDamage HitActor 2e+01 0 (Variables|Default|GetOwningPlayer) "/Game/Blueprints/BP_FireballDamageType.BP_FireballDamageType_C")
    (Actor|DestroyActor)))

(fn Activate)

(fn ValidateHit
  (params (InActor :type Actor%20Object%20Reference) (Hit :type Hit%20Result%20Structure))
  (if (not (== InActor (Game|GetInstigator)))
    (CallFunction|OnHit InActor Hit)))

(fn SetProperties
  (params (NewPower :type Float%20%28double-precision%29) (Color :type Vector%204%20Structure))
  (Variables|Default|SetPower NewPower)
  (Variables|Default|SetColor Color)
  (CallFunction|OnPropertiesSet))

(fn OnPropertiesSet)