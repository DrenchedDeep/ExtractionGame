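; BP_HomingProjectile is an ability projectile that homes toward its owning player's gaze location.
; On BeginPlay it sets the TargetLoc component as the ProjectileMovement homing target, then moves that component to the owner's GazeLocation every Tick with sweep enabled.
; For a locally controlled owner, it increments the player's IsHoming counter on BeginPlay and decrements it on Destroyed, tracking live homing projectiles.
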(event EventBeginPlay
  (bind _owningplayer (Variables|Default|GetOwningPlayer))
  (|CallParentFunction)
  (Variables|/Script/Engine.ProjectileMovementComponent|SetHomingTargetComponent (Variables|Default|GetProjectileMovement) (Variables|Default|GetTargetLoc))
  (if (Pawn|IsLocallyControlled _owningplayer)
    (Variables|/Game/Blueprints/Gameplay/Pawns/BP_FirstPersonCharacter.BP_FirstPersonCharacter_C|SetIsHoming _owningplayer (+ (Variables|/Game/Blueprints/Gameplay/Pawns/BP_FirstPersonCharacter.BP_FirstPersonCharacter_C|GetIsHoming _owningplayer) 1))))

(event Collision|EventActorBeginOverlap
  (params (OtherActor :type Actor%20Object%20Reference))
  (|CallParentFunction OtherActor) ; This node is disabled and will not be called.\nDrag off pins to build functionality.
)

(event EventTick
  (params (DeltaSeconds :type Float%20%28single-precision%29))
  (Transformation|SetWorldLocation (Variables|Default|GetTargetLoc) (Variables|/Script/ExtractionGame.ExtractionGameCharacter|GetGazeLocation (Variables|Default|GetOwningPlayer)) true false))

(event EventDestroyed
  (bind _owningplayer (Variables|Default|GetOwningPlayer))
  (if (Pawn|IsLocallyControlled _owningplayer)
    (Variables|/Game/Blueprints/Gameplay/Pawns/BP_FirstPersonCharacter.BP_FirstPersonCharacter_C|SetIsHoming _owningplayer (- (Variables|/Game/Blueprints/Gameplay/Pawns/BP_FirstPersonCharacter.BP_FirstPersonCharacter_C|GetIsHoming _owningplayer) 1))))

(fn ConstructionScript
  (|CallParentFunction))