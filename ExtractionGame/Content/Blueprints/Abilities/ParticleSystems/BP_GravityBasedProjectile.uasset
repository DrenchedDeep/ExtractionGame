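; BP_GravityBasedProjectile is a projectile actor driven by a ProjectileMovement component that destroys itself on any actor overlap.
; Each Tick checks the Y component of its velocity, not Z, and calls Activate while that value is negative.
; Otherwise it prints the elapsed lifetime, computed from initial and remaining life span, as debug output.
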(event EventBeginPlay
  (|CallParentFunction) ; This node is disabled and will not be called.\nDrag off pins to build functionality.
)

(event Collision|EventActorBeginOverlap
  (params (OtherActor :type Actor%20Object%20Reference))
  (Actor|DestroyActor))

(event EventTick
  (params (DeltaSeconds :type Float%20%28single-precision%29))
  (if (< (.Y (Math|Vector|BreakVector (Variables|/Script/Engine.MovementComponent|GetVelocity (Variables|Default|GetProjectileMovement)))) 0.0)
    (CallFunction|Activate)
    (else
      (Development|PrintString (Utilities|String|ToString(Float) (- (Variables|Default|GetInitialLifeSpan) (Actor|GetLifeSpan)))))))

(fn ConstructionScript
  (|CallParentFunction))