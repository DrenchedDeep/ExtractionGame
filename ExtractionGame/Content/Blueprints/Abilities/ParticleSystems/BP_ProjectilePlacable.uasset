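; BP_ProjectilePlacable is a projectile that sticks to surfaces and can be activated to deploy a volume object.
; On a hit against a sufficiently upward-facing surface, it stops sphere physics, attaches, aligns to the impact normal and extends its lifespan.
; Activate spawns the VolumeObject in its place, passes on its Color and destroys the projectile.
; Power and Color drive the mesh's emissive and color parameters when properties are set.
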(event EventBeginPlay
  (|CallParentFunction) ; This node is disabled and will not be called.\nDrag off pins to build functionality.
)

(event EventTick
  (params (DeltaSeconds :type Float%20%28single-precision%29)))

(fn ConstructionScript
  (|CallParentFunction))

(fn OnHit
  (params (HitActor :type Actor%20Object%20Reference) (HitResult :type Hit%20Result%20Structure))
  (bind (_bblockinghit _binitialoverlap _time _distance _location _impactpoint _normal _impactnormal) (Collision|BreakHitResult HitResult))
  (bind _sphere (Variables|Default|GetSphere))
  (if (> (Math|Vector|DotProduct _impactnormal (Math|Vector|GetUpVector _sphere)) 0.7)
    (Physics|SetSimulatePhysics _sphere false)
    (Transformation|AttachComponentToComponent 0 "None" "KeepRelative" "KeepRelative" "KeepRelative" true)
    (Transformation|SetWorldLocationAndRotation _sphere _impactpoint (Math|Rotator|MakeRotfromZ _impactnormal) false true)
    (Actor|SetLifeSpan 1e+06)))

(fn Activate
  (|CallParentFunction)
  (bind _returnvalue (Game|SpawnActorfromClass "/Game/Blueprints/Abilities/ParticleSystems/VolumeObject.VolumeObject_C" (Transformation|GetActorTransform) "AlwaysSpawn" "MultiplyWithRoot" 0 0))
  (Default|SetColor _returnvalue (Variables|Default|GetColor))
  (Actor|DestroyActor)
  (Development|PrintString "BOOM"))

(fn OnPropertiesSet
  (bind _staticmesh (Variables|Default|GetStaticMesh))
  (|CallParentFunction)
  (Audio|Parameter|SetFloatParameter _staticmesh "EmissivePower" (* (Variables|Default|GetPower) 2e+01) :!class /Script/AudioExtensions.AudioParameterControllerInterface)
  (Class|PrimitiveComponent|SetVectorParameterforCustomPrimitiveData _staticmesh "Color" (Variables|Default|GetColor))
  (Development|PrintString "Properties Set"))