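; GA_S2 is a gameplay ability that launches a homing projectile.
; It commits and ends immediately, then, if the commit succeeded, pulls a BP_HomingProjectile from the pool subsystem rather than spawning a new actor.
; CustomSpawnActor supplies transform and owner; the projectile gets power from the ability level and the "S2" group name before activation.
; A debug print shows the owner's name on each successful cast.
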(event Ability|EventActivateAbility
  (bind _returnvalue (Ability|CommitAbility))
  (Ability|EndAbility)
  (if _returnvalue
    (bind (_owner _location _rotation) (CallFunction|CustomSpawnActor))
    (bind _returnvalue_2 (Class|PoolHandlerSubSystem|SpawnObject (Subsystems|GetPoolHandlerSubSystem) "BP_HomingProjectile_C"))
    (Development|PrintString (Utilities|GetDisplayName _owner) true true "(R=0.041096,G=1.000000,B=0.000000,A=1.000000)")
    (Transformation|SetActorTransform _returnvalue_2 (Math|Transform|MakeTransform _location _rotation) false true)
    (Actor|SetOwner _returnvalue_2 _owner)
    (Variables|/Script/Engine.Actor|SetInstigator _returnvalue_2 _owner)
    (Class|PooledObject|SetAttributes _returnvalue_2 (Math|Conversions|ToFloat(Integer) (Ability|GetAbilityLevel)) "S2")
    (Class|PooledObject|SetActiveState _returnvalue_2 true)))

(event Ability|EventOnEndAbility
  (params (bWasCancelled :type Boolean)))