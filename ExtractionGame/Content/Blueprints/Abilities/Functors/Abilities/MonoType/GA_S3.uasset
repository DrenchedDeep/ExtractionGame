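; GA_S3 is a gameplay ability that fires a lightning line trace forward from a custom spawn transform.
; On a hit, it spawns a BP_LightningObject_S3 targeting the hit actor, then sends that actor a distance-scaled pull toward the origin if the owner implements BPI_Pullable.
; On a miss, it draws an NS_Lightning Niagara beam out to full trace range.
; The pull interface check tests the owner, although the message goes to the hit actor.
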(event Ability|EventActivateAbility
  (Ability|CommitAbility)
  (bind (_owner _location _rotation) (CallFunction|CustomSpawnActor))
  (bind (_outhit _returnvalue) (Class|KismetSystemLibrary|LineTraceSinglebyProfile _location (+ _location (* (Math|Vector|GetForwardVector _rotation) 1.8e+03)) "None" false 0 "None" true))
  (if _returnvalue
    (Game|SpawnActorfromClass "/Game/Blueprints/BP_LightningObject_S3.BP_LightningObject_S3_C" (Math|Transform|MakeTransform "0, 0, 0") "Undefined" "MultiplyWithRoot" 0 0.18 3e+01 2e+03 _owner (.HitActor (Collision|BreakHitResult _outhit)) 0)
    (if (Utilities|DoesObjectImplementInterface _owner "/Game/Blueprints/PhysGun/BPI_Pullable.BPI_Pullable_C")
      (Class|BPIPullable|Pull(Message) (.HitActor (Collision|BreakHitResult _outhit)) (* (/ (Math|Vector|VectorLength (- _location (Transformation|GetActorLocation (.HitActor (Collision|BreakHitResult _outhit))))) 1e+03) 3.0) (- _location (Transformation|GetActorLocation (.HitActor (Collision|BreakHitResult _outhit)))))
      (Ability|EndAbility)
      (else
        (Ability|EndAbility)))
    (else
      (bind _returnvalue_2 (Niagara|SpawnSystematLocation "/Game/ParticleSystems/Ability/NS_Lightning.NS_Lightning" "0, 0, 0"))
      (Niagara|SetNiagaraVariable(Vector3) _returnvalue_2 "StartLocation" _location)
      (Niagara|SetNiagaraVariable(Vector3) _returnvalue_2 "EndLocation" (+ _location (* (Math|Vector|GetForwardVector _rotation) 1.8e+03)))
      (Ability|EndAbility))))