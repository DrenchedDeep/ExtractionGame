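; GA_F3 is a two-press gameplay ability that places a Shadow deathbeam, then triggers it on the next activation.
; The first press commits, ends the ability, multicasts sound and effect, and configures a pooled BP_PlacableDeathbeam with level-based power, storing it as MyBomb.
; While MyBomb is valid, activation skips the commit and just ends the ability, letting OnEndAbility activate the placed object and clear the reference.
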(event Ability|EventActivateAbility
  (Utilities|IsValid (Variables|Default|GetMyBomb)
    (:Is%20Valid
      (Ability|EndAbility)
      (Development|PrintString "BOOM" true true "(R=1.000000,G=0.816736,B=0.000000,A=1.000000)" 5.0))
    (:Is%20Not%20Valid
      (bind _returnvalue (Ability|CommitAbility))
      (Ability|EndAbility)
      (if _returnvalue
        (bind (_owner _location _rotation) (CallFunction|CustomSpawnActor))
        (CallFunction|MulticastPlayEffect 0 "/Game/Sound_Effects_SFX/Ability_Shadow.Ability_Shadow" "Shadow_Attack" _location _rotation true)
        (bind _returnvalue_2 (Class|PoolHandlerSubSystem|SpawnObject (Subsystems|GetPoolHandlerSubSystem) "BP_PlacableDeathbeam_C"))
        (Transformation|SetActorTransform _returnvalue_2 (Math|Transform|MakeTransform _location _rotation) false true)
        (Actor|SetOwner _returnvalue_2 _owner)
        (Variables|/Script/Engine.Actor|SetInstigator _returnvalue_2 _owner)
        (Class|PooledObject|SetAttributes _returnvalue_2 (Math|Conversions|ToFloat(Integer) (Ability|GetAbilityLevel)) "F3")
        (Class|PooledObject|SetActiveState _returnvalue_2 true)
        (bind _asbp_projectile_placable (Utilities|Casting|CastToBP_ProjectilePlacable _returnvalue_2))
        (Variables|Default|SetMyBomb _asbp_projectile_placable)
        (Development|PrintString "Thrown" true true "(R=1.000000,G=0.823312,B=0.000000,A=1.000000)" 5.0)))))

(event Ability|EventOnEndAbility
  (params (bWasCancelled :type Boolean))
  (Utilities|IsValid (Variables|Default|GetMyBomb)
    (:Is%20Valid
      (Default|Activate (Variables|Default|GetMyBomb))
      (Variables|Default|SetMyBomb 0)
      (Development|PrintString "F3 Explode" true true "(R=1.000000,G=0.815904,B=0.000000,A=1.000000)" 5.0))
    (:Is%20Not%20Valid
      (Development|PrintString "Hello" true true "(R=0.868699,G=1.000000,B=0.000000,A=1.000000)" 5.0))))