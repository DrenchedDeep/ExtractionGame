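; GA_W1 is a gameplay ability that fires a gravity-based projectile in the "W1" group.
; On activation it commits and ends immediately, then gets a spawn transform and owner from CustomSpawnActor and multicasts the fire sound and effect, ignoring the owner on authority.
; It takes the projectile from the pool subsystem rather than spawning one, then sets its transform, owner, instigator and attributes before activating it.
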(event Ability|EventActivateAbility
  (Ability|CommitAbility)
  (Ability|EndAbility)
  (bind (_owner _location _rotation) (CallFunction|CustomSpawnActor))
  (Ability|HasAuthority
    (:True
      (CallFunction|MulticastPlayEffect 0 "/Game/Sound_Effects_SFX/Ability_Fire.Ability_Fire" "Fire_Ult" _location _rotation true))
    (:False
      (CallFunction|MulticastPlayEffect 0 "/Game/Sound_Effects_SFX/Ability_Fire.Ability_Fire" "Fire_Ult" _location _rotation false)))
  (bind _returnvalue (Class|PoolHandlerSubSystem|SpawnObject (Subsystems|GetPoolHandlerSubSystem) "BP_GravityBasedProjectile_C"))
  (Transformation|SetActorTransform _returnvalue (Math|Transform|MakeTransform _location _rotation (Math|Conversions|ToVector(Float) 1.0)) false true)
  (Actor|SetOwner _returnvalue _owner)
  (Variables|/Script/Engine.Actor|SetInstigator _returnvalue _owner)
  (Class|PooledObject|SetAttributes _returnvalue 0.0 "W1")
  (Class|PooledObject|SetActiveState _returnvalue true))

(event Ability|EventOnEndAbility
  (params (bWasCancelled :type Boolean)))