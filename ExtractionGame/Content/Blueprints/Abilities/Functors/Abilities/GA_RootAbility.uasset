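; Root Gameplay Ability for arm-mounted abilities, using the sign of the ability level to choose left or right arm tags and effects.
; Activation requires enough arm resource and no active cooldown tag.
; CommitExecute applies cost and cooldown through SetByCaller effects, scaling cooldown by the command subsystem's attack multiplier.
; Helpers supply the arm spawn transform and multicast a sound or fallback particle, optionally skipping the local owner.
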(event Custom|Multicast_PlayEffect
  (params (Particle :type Niagara%20System%20Object%20Reference) (Sound :type Meta%20Sound%20Source%20Object%20Reference) (MetaTrigger :type Name) (Location :type Vector) (Rotation :type Rotator) (IgnoreOwner :type Boolean))
  (if IgnoreOwner
    (bind _asbp_first_person_character (Utilities|Casting|CastToBP_FirstPersonCharacter (Ability|GetOwningActorfromActorInfo)))
    (if (not (Pawn|IsLocallyControlled _asbp_first_person_character))
      (Utilities|IsValid Sound :!label _label
        (:Is%20Valid
          (bind _returnvalue (Audio|SpawnSoundatLocation Sound Location Rotation 1.0 1.0 0.0 "/Game/Sound_Effects_SFX/AbilityAtten.AbilityAtten" 0))
          (Utilities|IsValid _returnvalue
            (:Is%20Valid
              (Class|AudioParameterControllerInterface|SetTriggerParameter _returnvalue MetaTrigger))))
        (:Is%20Not%20Valid
          (Utilities|IsValid Particle
            (:Is%20Valid
              (Niagara|SpawnSystematLocation Particle Location Rotation "1.000000,1.000000,1.000000" true true "AutoRelease"))))))
    (else
      (goto _label))))

(event Ability|EventCommitExecute
  (CallFunction|ApplyCost)
  (CallFunction|ApplyCoolDown))

(fn CustomSpawnActor
  (bind _asbp_first_person_character (Utilities|Casting|CastToBP_FirstPersonCharacter (Ability|GetOwningActorfromActorInfo)))
  (bind (_location _rotation) (Default|GetArmPos _asbp_first_person_character (Ability|GetAbilityLevel)))
  (return _asbp_first_person_character _location _rotation))

(fn PlayHitEffects
  (params (Particle :type Niagara%20System%20Object%20Reference) (Sound :type Meta%20Sound%20Source%20Object%20Reference) (MetaTrigger :type Name) (Location :type Vector) (Rotation :type Rotator)))

(fn DefineAbility
  (if (< (Ability|GetAbilityLevel) 0)
    (Variables|Default|SetArm "(TagName=\"Cooldown.LeftArm\")")
    (Variables|Default|SetCooldownEffect "/Game/Blueprints/Abilities/Functors/Effects/GE_ArmCooldown_Left.GE_ArmCooldown_Left_C")
    (Variables|Default|SetCostEffect "/Game/Blueprints/Abilities/Functors/Effects/GE_ArmCost_Left.GE_ArmCost_Left_C")
    (Variables|Default|SetCostArm "(AttributeName=\"LeftManaPool\",Attribute=/Script/ExtractionGame.ExtractionAttributeSet:LeftManaPool,AttributeOwner=\"/Script/CoreUObject.Class'/Script/ExtractionGame.ExtractionAttributeSet'\")")
    (else
      (Variables|Default|SetArm "(TagName=\"Cooldown.RightArm\")")
      (Variables|Default|SetCooldownEffect "/Game/Blueprints/Abilities/Functors/Effects/GE_ArmCooldown_Right.GE_ArmCooldown_Right_C")
      (Variables|Default|SetCostEffect "/Game/Blueprints/Abilities/Functors/Effects/GE_ArmCost_Right.GE_ArmCost_Right_C")
      (Variables|Default|SetCostArm "(AttributeName=\"RightManaPool\",Attribute=/Script/ExtractionGame.ExtractionAttributeSet:RightManaPool,AttributeOwner=\"/Script/CoreUObject.Class'/Script/ExtractionGame.ExtractionAttributeSet'\")"))))

(fn OverridenSetActorInfo
  (if (not (Variables|Default|Getgenerated))
    (CallFunction|DefineAbility)
    (Variables|Default|Setgenerated true)))

(fn CanAfford
  (params (AbilitySys :type Ability%20System%20Component%20Object%20Reference) (Level :type Integer))
  (bind _costarm (Variables|Default|GetCostArm))
  (bind _cost (Variables|Default|GetCost))
  (bind _returnvalue (Math|Float|Absolute(Float) _cost))
  (bind (_bfound _returnvalue_2) (Class|AbilitySystemComponent|GetGameplayAttributeValue AbilitySys _costarm))
  (if _bfound
    (return (>= _returnvalue_2 _returnvalue))
    (elif (< Level 0)
      (return (>= (.ReturnValue (Class|AbilitySystemComponent|GetGameplayAttributeValue AbilitySys "(AttributeName=\"RightManaPool\",Attribute=/Script/ExtractionGame.ExtractionAttributeSet:RightManaPool,AttributeOwner=\"/Script/CoreUObject.Class'/Script/ExtractionGame.ExtractionAttributeSet'\")")) _returnvalue))
      (else
        (return (>= (.ReturnValue (Class|AbilitySystemComponent|GetGameplayAttributeValue AbilitySys "(AttributeName=\"LeftManaPool\",Attribute=/Script/ExtractionGame.ExtractionAttributeSet:LeftManaPool,AttributeOwner=\"/Script/CoreUObject.Class'/Script/ExtractionGame.ExtractionAttributeSet'\")")) _returnvalue))))))

(fn ApplyCoolDown
  (bind _arm (Variables|Default|GetArm))
  (bind _returnvalue (Ability|GameplayEffect|AddGrantedTag (Ability|MakeOutgoingGameplayEffectSpec (Variables|Default|GetCooldownEffect)) _arm))
  (bind _returnvalue_2 (Ability|GameplayEffect|AssignTagSetbyCallerMagnitude _returnvalue _arm (* (Variables|Default|GetCooldown) (Class|CommandHandlerSubsystem|GetAttackCooldownMultiplier (Subsystems|GetCommandHandlerSubsystem)))))
  (Ability|ApplyGameplayEffectSpecToOwner _returnvalue_2))

(fn ApplyCost
  (bind _returnvalue (Ability|GameplayEffect|AssignTagSetbyCallerMagnitude (Ability|MakeOutgoingGameplayEffectSpec (Variables|Default|GetCostEffect)) (Variables|Default|GetArm) (Variables|Default|GetCost)))
  (bind _returnvalue_2 (Ability|ApplyGameplayEffectSpecToOwner _returnvalue))
  (Variables|Default|SetActiveEffect _returnvalue_2))

(fn K2CanActivateAbility
  (params (ActorInfo :type Gameplay%20Ability%20Actor%20Info%20Structure) (Handle :type Gameplay%20Ability%20Spec%20Handle%20Structure))
  (bind _abilitysystemcomponent (Utilities|Struct|BreakGameplayAbilityActorInfo ActorInfo))
  (return "" (and (CallFunction|CanAfford _abilitysystemcomponent (Class|GameplayAbility|GetAbilityLevelBP Handle ActorInfo)) (not (GameplayTags|HasMatchingGameplayTag _abilitysystemcomponent (Variables|Default|GetArm))))))