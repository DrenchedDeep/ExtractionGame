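; GA_F1W2 is a duo-type gameplay ability that fires a pooled wave projectile with an explosion and fire-attack effect.
; It commits, ends immediately, then on success takes a transform and owner from CustomSpawnActor and multicasts particle and sound, ignoring the owner.
; It pulls BP_WaveProjectile from the pool subsystem, sets owner and instigator, passes ability level as power, then activates it.
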(event Ability|EventActivateAbility
  (bind _returnvalue (Ability|CommitAbility))
  (Ability|EndAbility)
  (if _returnvalue
    (bind (_owner _location _rotation) (CallFunction|CustomSpawnActor))
    (CallFunction|MulticastPlayEffect "/Niagara/DefaultAssets/Templates/Systems/SimpleExplosion.SimpleExplosion" "/Game/Sound_Effects_SFX/Ability_Fire.Ability_Fire" "Fire_Attack" _location _rotation true)
    (bind _returnvalue_2 (Class|PoolHandlerSubSystem|SpawnObject (Subsystems|GetPoolHandlerSubSystem) "BP_WaveProjectile_C"))
    (Transformation|SetActorTransform _returnvalue_2 (Math|Transform|MakeTransform _location _rotation) false true)
    (Actor|SetOwner _returnvalue_2 _owner)
    (Variables|/Script/Engine.Actor|SetInstigator _returnvalue_2 _owner)
    (Class|PooledObject|SetAttributes _returnvalue_2 (Math|Conversions|ToFloat(Integer) (Ability|GetAbilityLevel)) "F1W2")
    (Class|PooledObject|SetActiveState _returnvalue_2 true)))