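; Gameplay ability F2W2, a hold-to-aim meteor strike cast from the arm given by the ability level's sign.
; A short WaitDelay loop traces toward the gaze point and checks for clear space overhead, moving and tinting a locally spawned AOE marker.
; Releasing or timing out commits if the spot is valid, otherwise cancels.
; Success drops a pooled BP_Meteor from high above, powered by ability level, with a multicast effect.
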(event Ability|EventActivateAbility
  (bind _returnvalue (Ability|GetAbilityLevel))
  (bind _array (Utilities|Array|MakeArray "ObjectTypeQuery1"))
  (Development|PrintString "Start F2W2" false)
  (Variables|Default|SetTmiePassed 0.0)
  (Variables|Default|SetArmDir (/ _returnvalue (Math|Integer|Absolute(Integer) _returnvalue)))
  (bind _asbp_first_person_character (Utilities|Casting|CastToBP_FirstPersonCharacter (Ability|GetOwningActorfromActorInfo))
    (:then
      (Variables|Default|SetAs%20BP%20First%20Person%20Character _asbp_first_person_character)
      (if (Pawn|IsLocallyControlled _asbp_first_person_character)
        (bind _returnvalue_2 (Niagara|SpawnSystematLocation "/Game/ParticleSystems/Ability/NS_MeteorAOEInf.NS_MeteorAOEInf" "0, 0, 0" "0, 0, 0" "1.000000,1.000000,1.000000" true true "AutoRelease"))
        (Variables|Default|SetParticle _returnvalue_2))
      (Ability|Tasks|WaitDelay 0.05 :!label _label ; Prediction Key becomes invalid on OnFinish pin
        (:OnFinish
          (Development|PrintString "F2W2 Tick" true true "(R=0.000000,G=0.660000,B=1.000000,A=1.000000)" 0.1)
          (Variables|Default|SetTmiePassed (+ (Variables|Default|GetTmiePassed) 0.05))
          (bind (_outhit _returnvalue_3) (Collision|SphereTraceForObjects (Transformation|GetActorLocation (Variables|Default|GetAs%20BP%20First%20Person%20Character)) (Variables|/Script/ExtractionGame.ExtractionGameCharacter|GetGazeLocation (Variables|Default|GetAs%20BP%20First%20Person%20Character)) 5e+01 _array false 0 "ForOneFrame"))
          (bind _returnvalue_4 (Collision|LineTraceForObjects (+ (Variables|/Script/ExtractionGame.ExtractionGameCharacter|GetGazeLocation (Variables|Default|GetAs%20BP%20First%20Person%20Character)) "0.000000,0.000000,2000.000000") (+ (Variables|/Script/ExtractionGame.ExtractionGameCharacter|GetGazeLocation (Variables|Default|GetAs%20BP%20First%20Person%20Character)) "0.000000,0.000000,10000.000000") _array false 0 "ForOneFrame"))
          (bind _output_get (Variables|Default|SetColChecks (and _returnvalue_3 (not _returnvalue_4))))
          (Utilities|IsValid (Variables|Default|GetParticle)
            (:Is%20Valid
              (if _output_get
                (Niagara|SetNiagaraVariable(LinearColor) (Variables|Default|GetParticle) "LinearColor" (Math|Color|MakeColor 1.0 0.0 4.0))
                (else
                  (Niagara|SetNiagaraVariable(LinearColor) (Variables|Default|GetParticle) "LinearColor" (Math|Color|MakeColor 1.0 0.0 0.0))))
              (Transformation|SetWorldLocation (Variables|Default|GetParticle) (.Location (Collision|BreakHitResult _outhit)) false true))
            (:Is%20Not%20Valid
              _))
          (if (and (Class|ExtractionGameCharacter|WantstoFireAnyArm (Variables|Default|GetAs%20BP%20First%20Person%20Character) (Variables|Default|GetArmDir)) (< (Variables|Default|GetTmiePassed) 3e+01))
            (goto _label)
            (elif (and (> (Variables|Default|GetTmiePassed) 0.12) (Variables|Default|GetColChecks))
              (bind _returnvalue_5 (Ability|CommitAbility))
              (if _returnvalue_5
                (Ability|EndAbility)
                (else
                  (Ability|CancelAbility :!label _label_2)))
              (else
                (goto _label_2)))))))
    (:CastFailed
      (Development|PrintString "Failed to get player?"))))

(event Ability|EventOnEndAbility
  (params (bWasCancelled :type Boolean))
  (bind _as_bp_first_person_character (Variables|Default|GetAs%20BP%20First%20Person%20Character))
  (bind _particle (Variables|Default|GetParticle))
  (if bWasCancelled
    (Development|PrintString "F2W2 Fail" true true "(R=1.000000,G=0.168445,B=0.000000,A=1.000000)" 1e+01)
    (Utilities|IsValid _particle
      (:Is%20Valid
        (Components|Activation|Deactivate _particle)))
    (else
      (Development|PrintString "F2W2 Success" true true "(R=0.000000,G=0.660000,B=1.000000,A=1.000000)" 1e+01)
      (bind _returnvalue (Class|PoolHandlerSubSystem|SpawnObject (Subsystems|GetPoolHandlerSubSystem) "BP_Meteor_C"))
      (Transformation|SetActorTransform _returnvalue (Math|Transform|MakeTransform (+ (Variables|/Script/ExtractionGame.ExtractionGameCharacter|GetGazeLocation _as_bp_first_person_character) "0.000000,0.000000,150000.000000")) false true)
      (Actor|SetOwner _returnvalue _as_bp_first_person_character)
      (Variables|/Script/Engine.Actor|SetInstigator _returnvalue _as_bp_first_person_character)
      (Class|PooledObject|SetAttributes _returnvalue (Math|Conversions|ToFloat(Integer) (Ability|GetAbilityLevel)) "F2W2")
      (Class|PooledObject|SetActiveState _returnvalue true)
      (CallFunction|MulticastPlayEffect "/Game/ParticleSystems/Ability/NS_MeteorAOETimed1.NS_MeteorAOETimed1" 0 "None" (Variables|/Script/ExtractionGame.ExtractionGameCharacter|GetGazeLocation _as_bp_first_person_character) "0, 0, 0" false)
      (Utilities|IsValid _particle
        (:Is%20Valid
          (Components|Activation|Deactivate _particle))))))