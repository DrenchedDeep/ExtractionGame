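; Two-press shadow ability (S1W1) that places a pooled projectile bomb, then detonates it on the next activation.
; With no live bomb, it commits, ends, plays a multicast Shadow effect and configures a BP_ProjectilePlacable with owner and level-based power.
; EndAbility runs before the spawn, so OnEndAbility only triggers the stored bomb on a later activation, which skips CommitAbility.
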(event Ability|EventActivateAbility
  (Utilities|IsValid (Variables|Default|GetMyBomb)
    (:Is%20Valid
      (Ability|EndAbility))
    (:Is%20Not%20Valid
      (Ability|CommitAbility)
      (Ability|EndAbility)
      (bind (_owner _location _rotation) (CallFunction|CustomSpawnActor))
      (CallFunction|MulticastPlayEffect 0 "/Game/Sound_Effects_SFX/Ability_Shadow.Ability_Shadow" "Shadow_Attack" _location "0, 0, 0" false)
      (bind _returnvalue (Class|PoolHandlerSubSystem|SpawnObject (Subsystems|GetPoolHandlerSubSystem) "BP_ProjectilePlacable_C"))
      (Transformation|SetActorTransform _returnvalue (Math|Transform|MakeTransform _location _rotation) false true)
      (Actor|SetOwner _returnvalue _owner)
      (Variables|/Script/Engine.Actor|SetInstigator _returnvalue _owner)
      (Class|PooledObject|SetAttributes _returnvalue (Math|Conversions|ToFloat(Integer) (Ability|GetAbilityLevel)) "S1W1")
      (Class|PooledObject|SetActiveState _returnvalue true)
      (bind _asbp_projectile_placable (Utilities|Casting|CastToBP_ProjectilePlacable _returnvalue))
      (Variables|Default|SetMyBomb _asbp_projectile_placable))))

(event Ability|EventOnEndAbility
  (params (bWasCancelled :type Boolean))
  (Utilities|IsValid (Variables|Default|GetMyBomb)
    (:Is%20Valid
      (Default|Activate (Variables|Default|GetMyBomb))
      (Variables|Default|SetMyBomb 0)
      (Development|PrintString "Explode"))))