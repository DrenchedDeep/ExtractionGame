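; GA_F2S1 is a duo-type gameplay ability that fires a pooled projectile with fire ability effects.
; On activation it commits and immediately ends, then gets a spawn transform and owner from CustomSpawnActor and multicasts the sound and effect trigger to all but the owner.
; It takes a BP_ProjectileBase from the pool subsystem, places it, assigns owner and instigator, sets power from ability level under group F2S1, and activates it.
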(event Ability|EventActivateAbility
  (Ability|CommitAbility)
  (Ability|EndAbility)
  (bind (_owner _location _rotation) (CallFunction|CustomSpawnActor))
  (CallFunction|MulticastPlayEffect 0 "/Game/Sound_Effects_SFX/Ability_Fire.Ability_Fire" "Fire_Ult" _location _rotation true)
  (bind _returnvalue (Class|PoolHandlerSubSystem|SpawnObject (Subsystems|GetPoolHandlerSubSystem) "BP_ProjectileBase_C"))
  (Transformation|SetActorTransform _returnvalue (Math|Transform|MakeTransform _location _rotation) false true)
  (Actor|SetOwner _returnvalue _owner)
  (Variables|/Script/Engine.Actor|SetInstigator _returnvalue _owner)
  (Class|PooledObject|SetAttributes _returnvalue (Math|Conversions|ToFloat(Integer) (Ability|GetAbilityLevel)) "F2S1")
  (Class|PooledObject|SetActiveState _returnvalue true))