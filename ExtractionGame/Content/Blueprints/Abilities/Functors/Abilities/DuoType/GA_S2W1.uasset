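; GA_S2W1 is a duo-type gameplay ability that fires a magic pulse, labelled "Repuslor" in its debug print.
; On activation it commits and immediately ends the ability, continuing only if the commit succeeded.
; It multicasts explosion, sound and "Fire_Attack" effects at the custom spawn transform, ignoring the owner.
; It then spawns BP_MagicPulse there and activates it with the ability level as power and data row S2W1.
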(event Ability|EventActivateAbility
  (bind _returnvalue (Ability|CommitAbility))
  (Ability|EndAbility)
  (if _returnvalue
    (bind (_owner _location _rotation) (CallFunction|CustomSpawnActor))
    (CallFunction|MulticastPlayEffect "/Niagara/DefaultAssets/Templates/Systems/SimpleExplosion.SimpleExplosion" "/Game/Sound_Effects_SFX/Ability_Fire.Ability_Fire" "Fire_Attack" _location _rotation true)
    (bind _returnvalue_2 (Game|SpawnActorfromClass "/Game/Blueprints/Abilities/Blueprints/BP_MagicPulse.BP_MagicPulse_C" (Math|Transform|MakeTransform _location _rotation) "AlwaysSpawn" "OverrideRootScale" _owner _owner))
    (Default|Activate _returnvalue_2 (Math|Conversions|ToFloat(Integer) (Ability|GetAbilityLevel)) "S2W1")
    (Development|PrintString "Repuslor")))