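; Gameplay ability F1W1, a duo-type ability that launches a pooled gravity-based projectile.
; On activation it commits and ends immediately, then pulls the projectile from the pool subsystem rather than spawning a new actor.
; CustomSpawnActor supplies the transform and the owner, which also becomes the instigator.
; The projectile receives the ability level as power and the F1W1 group name before being activated.
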(event Ability|EventActivateAbility
  (Ability|CommitAbility)
  (Ability|EndAbility)
  (bind (_owner _location _rotation) (CallFunction|CustomSpawnActor))
  (bind _returnvalue (Class|PoolHandlerSubSystem|SpawnObject (Subsystems|GetPoolHandlerSubSystem) "BP_GravityBasedProjectile_C"))
  (Transformation|SetActorTransform _returnvalue (Math|Transform|MakeTransform _location _rotation "1.000000,1.000000,1.000000") false true)
  (Actor|SetOwner _returnvalue _owner)
  (Variables|/Script/Engine.Actor|SetInstigator _returnvalue _owner)
  (Class|PooledObject|SetAttributes _returnvalue (Math|Conversions|ToFloat(Integer) (Ability|GetAbilityLevel)) "F1W1")
  (Class|PooledObject|SetActiveState _returnvalue true))

(event Ability|EventOnEndAbility
  (params (bWasCancelled :type Boolean)))