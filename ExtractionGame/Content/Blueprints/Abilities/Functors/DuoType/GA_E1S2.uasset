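; GA_E1S2 is a DuoType gameplay ability that fires a placeable projectile from the first-person character.
; On activation it commits, prints its own name and calls EndAbility before doing the spawn work.
; It gets the arm transform from the character using the ability level, then spawns BP_ProjectilePlacable there with the character as Instigator.
; The projectile's gravity scale is set low after spawning.
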(event Ability|EventActivateAbility
  (Ability|CommitAbility)
  (Development|PrintString (Utilities|GetDisplayName self))
  (Ability|EndAbility)
  (bind _asbp_first_person_character (Utilities|Casting|CastToBP_FirstPersonCharacter (Ability|GetOwningActorfromActorInfo)))
  (bind (_location _rotation) (Default|GetArmPos _asbp_first_person_character (Ability|GetAbilityLevel)))
  (bind _returnvalue (Game|SpawnActorfromClass "/Game/Blueprints/Abilities/ParticleSystems/BP_ProjectilePlacable.BP_ProjectilePlacable_C" (Math|Transform|MakeTransform _location _rotation) "AdjustIfPossibleButAlwaysSpawn" "MultiplyWithRoot" 0 _asbp_first_person_character))
  (Variables|/Script/Engine.ProjectileMovementComponent|SetProjectileGravityScale (Variables|/Game/Blueprints/Abilities/ParticleSystems/BP_ProjectileBase.BP_ProjectileBase_C|GetProjectileMovement _returnvalue) 0.2))

(event Ability|EventOnEndAbility
  (params (bWasCancelled :type Boolean)))