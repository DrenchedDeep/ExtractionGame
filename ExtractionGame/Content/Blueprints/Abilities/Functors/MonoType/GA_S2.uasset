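; GA_S2 is a gameplay ability that fires a homing projectile.
; On activation it commits, prints its display name and calls EndAbility before doing the spawn work.
; It takes a BP_HomingProjectile from the pool handler subsystem instead of spawning a new one.
; The projectile gets its transform, owner and instigator from CustomSpawnActor, then receives power and the S2 group before being activated.
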(event Ability|EventActivateAbility
  (Ability|CommitAbility)
  (Development|PrintString (Utilities|GetDisplayName self))
  (Ability|EndAbility)
  (bind (_owner _location _rotation) (CallFunction|CustomSpawnActor))
  (bind _returnvalue (Class|PoolHandlerSubSystem|SpawnObject (Subsystems|GetPoolHandlerSubSystem) "BP_HomingProjectile_C"))
  (Transformation|SetActorTransform _returnvalue (Math|Transform|MakeTransform _location _rotation) false true)
  (Actor|SetOwner _returnvalue _owner)
  (Variables|/Script/Engine.Actor|SetInstigator _returnvalue _owner)
  (Class|PooledObject|SetAttributes _returnvalue 5e+01 "S2")
  (Class|PooledObject|SetActiveState _returnvalue true))

(event Ability|EventOnEndAbility
  (params (bWasCancelled :type Boolean)))