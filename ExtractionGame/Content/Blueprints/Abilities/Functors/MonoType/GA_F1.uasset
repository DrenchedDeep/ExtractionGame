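; GA_F1 is a Gameplay Ability in the MonoType functor set that fires a pooled fire-attack projectile.
; On activation it commits and immediately calls EndAbility, then gets a spawn point and owner from CustomSpawnActor and multicasts explosion, sound and meta-trigger effects there.
; It takes a BP_ProjectileBase from the pool subsystem, positions it, assigns owner and instigator, sets power and group "F1", and activates it.
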(event Ability|EventActivateAbility
  (Ability|CommitAbility)
  (Ability|EndAbility)
  (bind (_owner _location _rotation) (CallFunction|CustomSpawnActor))
  (CallFunction|MulticastPlayEffect "/Niagara/DefaultAssets/Templates/Systems/SimpleExplosion.SimpleExplosion" "/Game/Blueprints/SFXs/Ability_Fire.Ability_Fire" "Fire_Attack" _location _rotation)
  (bind _returnvalue (Class|PoolHandlerSubSystem|SpawnObject (Subsystems|GetPoolHandlerSubSystem) "BP_ProjectileBase_C"))
  (Transformation|SetActorTransform _returnvalue (Math|Transform|MakeTransform _location _rotation) false true)
  (Actor|SetOwner _returnvalue _owner)
  (Variables|/Script/Engine.Actor|SetInstigator _returnvalue _owner)
  (Class|PooledObject|SetAttributes _returnvalue 5e+01 "F1")
  (Class|PooledObject|SetActiveState _returnvalue true))