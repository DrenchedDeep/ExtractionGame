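; GA_S1 is a gameplay ability that launches a placeable projectile bomb on one activation and detonates it on the next.
; With no live bomb, it commits, ends, then spawns BP_ProjectilePlacable from CustomSpawnActor's transform, setting speed, gravity scale and power.
; With a live bomb, it only ends, and OnEndAbility activates the bomb and clears the reference.
; Ending before spawning keeps a new bomb from detonating immediately.
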(event Ability|EventActivateAbility
  (Utilities|IsValid (Variables|Default|GetMyBomb)
    (:Is%20Valid
      (Ability|EndAbility))
    (:Is%20Not%20Valid
      (Ability|CommitAbility)
      (Ability|EndAbility)
      (bind (_owner _location _rotation) (CallFunction|CustomSpawnActor))
      (bind _returnvalue (Game|SpawnActorfromClass "/Game/Blueprints/Abilities/Blueprints/BP_ProjectilePlacable.BP_ProjectilePlacable_C" (Math|Transform|MakeTransform _location _rotation) "AlwaysSpawn" "OverrideRootScale" _owner _owner))
      (bind _output_get (Variables|Default|SetMyBomb _returnvalue))
      (bind _output_get_2 (Variables|/Script/Engine.ProjectileMovementComponent|SetInitialSpeed (Variables|/Game/Blueprints/Abilities/Blueprints/BP_ProjectileBase.BP_ProjectileBase_C|GetProjectileMovement _output_get) 3e+03))
      (Variables|/Script/Engine.ProjectileMovementComponent|SetProjectileGravityScale (Variables|/Game/Blueprints/Abilities/Blueprints/BP_ProjectileBase.BP_ProjectileBase_C|GetProjectileMovement _output_get) _output_get_2)
      (Default|SetProperties _output_get 5e+01 "S1"))))

(event Ability|EventOnEndAbility
  (params (bWasCancelled :type Boolean))
  (Utilities|IsValid (Variables|Default|GetMyBomb)
    (:Is%20Valid
      (Default|Activate (Variables|Default|GetMyBomb))
      (Variables|Default|SetMyBomb 0)
      (Development|PrintString "Explode"))))