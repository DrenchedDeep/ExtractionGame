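; Base-style gameplay ability for arm-mounted abilities on BP_FirstPersonCharacter, using the sign of the ability level to pick left or right arm.
; Committing applies that arm's cooldown effect, with a set-by-caller duration scaled by the CommandHandlerSubsystem multiplier.
; CustomSpawnActor supplies the owner and arm transform for spawning.
; A multicast event plays a sound, or particles if none, optionally skipping the locally controlled owner.
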(event Custom|Multicast_PlayEffect
  (params (Particle :type Niagara%20System%20Object%20Reference) (Sound :type Meta%20Sound%20Source%20Object%20Reference) (MetaTrigger :type Name) (Location :type Vector) (Rotation :type Rotator) (IgnoreOwner :type Boolean))
  (if IgnoreOwner
    (bind _asbp_first_person_character (Utilities|Casting|CastToBP_FirstPersonCharacter (Ability|GetOwningActorfromActorInfo)))
    (if (not (Pawn|IsLocallyControlled _asbp_first_person_character))
      (Utilities|IsValid Sound :!label _label
        (:Is%20Valid
          (bind _returnvalue (Audio|SpawnSoundatLocation Sound Location Rotation 1.0 1.0 0.0 "/Game/Sound_Effects_SFX/AbilityAtten.AbilityAtten" 0))
          (Utilities|IsValid _returnvalue
            (:Is%20Valid
              (Class|AudioParameterControllerInterface|SetTriggerParameter _returnvalue MetaTrigger))))
        (:Is%20Not%20Valid
          (Utilities|IsValid Particle
            (:Is%20Valid
              (Niagara|SpawnSystematLocation Particle Location Rotation "1.000000,1.000000,1.000000" true true "AutoRelease"))))))
    (else
      (goto _label))))

(event Ability|EventCommitExecute
  (if (< (Ability|GetAbilityLevel) 0)
    (Variables|Default|SetArm "(TagName=\"Cooldown.LeftArm\")")
    (Variables|Default|SetCooldownEffect "/Game/Blueprints/Abilities/Functors/GE_ArmCooldown_Left.GE_ArmCooldown_Left_C")
    (else
      (Variables|Default|SetArm "(TagName=\"Cooldown.RightArm\")")
      (Variables|Default|SetCooldownEffect "/Game/Blueprints/Abilities/Functors/GE_ArmCooldown_Right.GE_ArmCooldown_Right_C")))
  (bind _returnvalue (Ability|GameplayEffect|AddGrantedTag (Ability|MakeOutgoingGameplayEffectSpec (Variables|Default|GetCooldownEffect)) (Variables|Default|GetArm)))
  (bind _returnvalue_2 (Ability|GameplayEffect|AssignTagSetbyCallerMagnitude _returnvalue (Variables|Default|GetArm) (* (Variables|Default|GetCooldown) (Class|CommandHandlerSubsystem|GetAttackCooldownMultiplier (Subsystems|GetCommandHandlerSubsystem)))))
  (Ability|ApplyGameplayEffectSpecToOwner _returnvalue_2))

(fn CustomSpawnActor
  (bind _asbp_first_person_character (Utilities|Casting|CastToBP_FirstPersonCharacter (Ability|GetOwningActorfromActorInfo)))
  (bind (_location _rotation) (Default|GetArmPos _asbp_first_person_character (Ability|GetAbilityLevel)))
  (return _asbp_first_person_character _location _rotation))

(fn K2CanActivateAbility
  (params (ActorInfo :type Gameplay%20Ability%20Actor%20Info%20Structure) (Handle :type Gameplay%20Ability%20Spec%20Handle%20Structure))
  (return "" (< "" (Math|DateTime|Now))))

(fn PlayHitEffects
  (params (Particle :type Niagara%20System%20Object%20Reference) (Sound :type Meta%20Sound%20Source%20Object%20Reference) (MetaTrigger :type Name) (Location :type Vector) (Rotation :type Rotator)))