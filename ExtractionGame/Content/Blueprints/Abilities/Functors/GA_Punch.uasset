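; GA_Punch is a Gameplay Ability that throws a punch from the first-person character's arm.
; On activation it commits and immediately ends, then gets the arm position using the ability level and sphere-traces from it for Pawns and Destructibles, ignoring the owner.
; A hit applies physical point damage and fires an impact trigger on the punch sound.
; The sound and Niagara effect play whether or not it hits.
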(event Ability|EventActivateAbility
  (bind _returnvalue (Ability|GetActorInfo))
  (bind _owneractor (Utilities|Struct|BreakGameplayAbilityActorInfo _returnvalue))
  (Ability|CommitAbility)
  (Ability|EndAbility)
  (bind _asbp_first_person_character (Utilities|Casting|CastToBP_FirstPersonCharacter (Ability|GetOwningActorfromActorInfo)))
  (bind (_location _rotation) (Default|GetArmPos _asbp_first_person_character (Ability|GetAbilityLevel)))
  (Development|PrintString (Utilities|String|ToString(Rotator) _rotation))
  (bind (_outhit _returnvalue_2) (Collision|SphereTraceForObjects _location (+ _location (* _rotation (Math|Conversions|ToVector(Float) 2.5e+02))) 5e+01 (Utilities|Array|MakeArray "ObjectTypeQuery6" "ObjectTypeQuery3") false (Utilities|Array|MakeArray _owneractor) "None" true "(R=1.000000,G=0.000000,B=0.000000,A=1.000000)" "(R=0.000000,G=1.000000,B=0.000000,A=1.000000)" 3.0))
  (bind _returnvalue_3 (Audio|SpawnSoundatLocation "/Game/Sound_Effects_SFX/Ability_Punch.Ability_Punch" _location _rotation 1.0 1.0 0.0 0 0))
  ;[1 1 1] Whether or not you hit something damagable
  (if _returnvalue_2
    (Game|Damage|ApplyPointDamage (.HitActor (Collision|BreakHitResult _outhit)) 15.0 (* _rotation (Math|Conversions|ToVector(Float) 2.5e+02)) _outhit (Pawn|GetController _asbp_first_person_character) _owneractor "/Game/Blueprints/Abilities/Functors/DamageTypes/BP_Physical.BP_Physical_C")
    (Class|AudioParameterControllerInterface|SetTriggerParameter _returnvalue_3 "Input_Impact"))
  (Niagara|SpawnSystematLocation "/Game/ParticleSystems/Ability/NS_Punch.NS_Punch" _location _rotation "1.000000,1.000000,1.000000" true true "AutoRelease"))

(event Ability|EventOnEndAbility
  (params (bWasCancelled :type Boolean)))