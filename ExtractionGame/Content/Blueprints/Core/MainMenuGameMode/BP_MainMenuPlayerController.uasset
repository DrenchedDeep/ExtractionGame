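; BP_MainMenuPlayerController is the main menu player controller, handling keyboard shortcuts for the exit menu and hosting intent.
; Escape and the 1 key share one path that casts the HUD to BP_MainMenuHUD and toggles its exit menu.
; P flips a local IsHosting flag and passes the new state to ExtractionGameInstance through SetWantsToHost.
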(event Input|KeyboardEvents|Escape
  (params (Key :type Key%20Structure :default "None"))
  (:Pressed
    (bind _asbp_main_menu_hud (Utilities|Casting|CastToBP_MainMenuHUD (HUD|GetHUD)))
    (Default|ToggleExitMenu _asbp_main_menu_hud)))

(event Input|KeyboardEvents|P
  (params (Key :type Key%20Structure :default "None"))
  (:Pressed
    (if (Variables|Default|GetIsHosting)
      (Variables|Default|SetIsHosting false)
      (bind _asextraction_game_instance (Utilities|Casting|CastToExtractionGameInstance (Game|GetGameInstance)))
      (Class|ExtractionGameInstance|SetWantstoHost _asextraction_game_instance false)
      (else
        (bind _asextraction_game_instance_2 (Utilities|Casting|CastToExtractionGameInstance (Game|GetGameInstance)))
        (Class|ExtractionGameInstance|SetWantstoHost _asextraction_game_instance_2 true)
        (Variables|Default|SetIsHosting true)))))

(event Input|KeyboardEvents|1
  (params (Key :type Key%20Structure :default "None"))
  (:Pressed
    (bind _asbp_main_menu_hud (Utilities|Casting|CastToBP_MainMenuHUD (HUD|GetHUD)))
    (Default|ToggleExitMenu _asbp_main_menu_hud)))

(fn ConstructionScript)