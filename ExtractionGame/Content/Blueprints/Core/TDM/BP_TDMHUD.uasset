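; BP_TDMHUD is the HUD for the Team Deathmatch mode, owning the on-screen match widget and kill notification popup.
; On BeginPlay it creates and adds both widgets to the viewport, keeping the kill notification hidden until a kill occurs.
; Its events forward kills, game over with the winning team, match timer updates and match state changes (as strings) to those widgets.
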(event EventUpdateMatchTimerText
  (params (MatchTimer :type Integer))
  (Default|UpdateMatchTimerText (Variables|Default|GetHUD) MatchTimer))

(event EventEndGame
  (params (WinningTeam :type String))
  (Default|GameOver (Variables|Default|GetHUD) WinningTeam))

(event EventOnKill
  (params (VictimName :type String))
  (bind _killnotif (Variables|Default|GetKillNotif))
  (Widget|SetVisibility _killnotif "Visible")
  (Default|OnKill _killnotif VictimName))

(event EventBeginPlay
  (|CallParentFunction)
  (bind _returnvalue (UserInterface|CreateWidget "/Game/Blueprints/Widgets/TDM/WB_TDMWidget.WB_TDMWidget_C"))
  (bind _output_get (Variables|Default|SetHUD _returnvalue))
  (UserInterface|Viewport|AddtoViewport _returnvalue 0)
  (bind _returnvalue_2 (UserInterface|CreateWidget "/Game/Blueprints/Widgets/WB_KillNotification.WB_KillNotification_C" (Game|Player|GetOwningPlayerController)))
  (bind _output_get_2 (Variables|Default|SetKillNotif _returnvalue_2))
  (Widget|SetVisibility _output_get_2 "Hidden")
  (UserInterface|Viewport|AddtoViewport _output_get_2 0))

(fn ConstructionScript)

(fn MatchStateChanged
  (params (MatchState :type Name))
  (bind _hud (Variables|Default|GetHUD))
  (Utilities|IsValid _hud
    (:Is%20Valid
      (Default|GameStateChanged _hud (Utilities|String|ToString(Name) MatchState)))))