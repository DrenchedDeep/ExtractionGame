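; Game state for TDM mode that registers abilities at startup and relays match state changes to the HUD.
; On BeginPlay it runs Mono, Duo and Trio loaders, each copying keyed Data entries into the AbilityHandler subsystem's map and printing a colored debug message.
; MatchStateChanged passes the new state to player 0's BP_TDMHUD when that cast succeeds.
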(event EventBeginPlay
  (CallFunction|LoadMonoType)
  (CallFunction|LoadDuoType)
  (CallFunction|LoadTrioType))

(event EventMatchStateChanged
  (params (NewState :type Name%20%28by%20ref%29 :default "None"))
  (bind _asbp_tdmhud (Utilities|Casting|CastToBP_TDMHUD (HUD|GetHUD (Game|GetPlayerController 0))))
  (Default|MatchStateChanged _asbp_tdmhud NewState))

(fn ConstructionScript)

(fn LoadMonoType
  (bind _data (LocalVariables|GetData))
  (bind _keys (Utilities|Map|Keys _data))
  (for _array_element _keys
    (Class|AbilityHandlerSubSystem|AddAbilitytoMap (Subsystems|GetAbilityHandlerSubSystem) _array_element (.Value (Utilities|Map|Find _data _array_element))))
  (Development|PrintString "Mono Abilities Loaded!" true true "(R=0.000000,G=1.000000,B=0.037928,A=1.000000)"))

(fn LoadDuoType
  (bind _data (LocalVariables|GetData))
  (bind _keys (Utilities|Map|Keys _data))
  (for _array_element _keys
    (Class|AbilityHandlerSubSystem|AddAbilitytoMap (Subsystems|GetAbilityHandlerSubSystem) _array_element (.Value (Utilities|Map|Find _data _array_element))))
  (Development|PrintString "Duo Abilities Loaded!" true true "(R=0.918360,G=1.000000,B=0.000000,A=1.000000)"))

(fn LoadTrioType
  (bind _data (LocalVariables|GetData))
  (bind _keys (Utilities|Map|Keys _data))
  (for _array_element _keys
    (Class|AbilityHandlerSubSystem|AddAbilitytoMap (Subsystems|GetAbilityHandlerSubSystem) _array_element (.Value (Utilities|Map|Find _data _array_element))))
  (Development|PrintString "Trio  Abilities Loaded!" true true "(R=1.000000,G=0.000000,B=0.099114,A=1.000000)"))