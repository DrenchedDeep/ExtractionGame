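; Main-menu manager for the player's stash, player inventory and gem loadout, binding the inventory components to the stash screen widgets.
; Starting items are built from DT_Items rows into the stash, and saving copies stash items into the game instance's SavedStash.
; Gem changes refresh the character gem UI, then record any new non-Punch arm ability in save data and show an unlock popup.
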(event EventBeginPlay
  (bind _playerinventory (Variables|Default|GetPlayerInventory))
  (bind _stashinventory (Variables|Default|GetStashInventory))
  (bind _asbp_main_menu_hud (Utilities|Casting|CastToBP_MainMenuHUD (HUD|GetHUD (Game|GetPlayerController 0))))
  (bind _aswb_main_menu (Utilities|Casting|CastToWB_MainMenu (Variables|/Script/ExtractionGame.MainMenuHUD|GetMainMenuWidget _asbp_main_menu_hud)))
  (Default|Init (Variables|/Game/Blueprints/Widgets/MainMenu/Inventory/WB_MainMenuStash.WB_MainMenuStash_C|GetWB_StashInventory (Variables|/Game/Blueprints/Widgets/MainMenu/WB_MainMenu.WB_MainMenu_C|GetWB_MainMenuStash _aswb_main_menu)) (Variables|/Script/ExtractionGame.InventoryComp|GetTileSize _stashinventory) _stashinventory)
  (Default|Init (Variables|/Game/Blueprints/Widgets/MainMenu/Inventory/WB_MainMenuStash.WB_MainMenuStash_C|GetPlayerInventoryWidget (Variables|/Game/Blueprints/Widgets/MainMenu/WB_MainMenu.WB_MainMenu_C|GetWB_MainMenuStash _aswb_main_menu)) (Variables|/Script/ExtractionGame.InventoryComp|GetTileSize _playerinventory) _playerinventory)
  (Class|InventoryComp|SetInventoryWidget (Variables|Default|GetPlayerInventory) (Variables|/Game/Blueprints/Widgets/MainMenu/Inventory/WB_MainMenuStash.WB_MainMenuStash_C|GetPlayerInventoryWidget (Variables|/Game/Blueprints/Widgets/MainMenu/WB_MainMenu.WB_MainMenu_C|GetWB_MainMenuStash _aswb_main_menu)))
  (Class|InventoryComp|SetInventoryWidget (Variables|Default|GetStashInventory) (Variables|/Game/Blueprints/Widgets/MainMenu/Inventory/WB_MainMenuStash.WB_MainMenuStash_C|GetWB_StashInventory (Variables|/Game/Blueprints/Widgets/MainMenu/WB_MainMenu.WB_MainMenu_C|GetWB_MainMenuStash _aswb_main_menu)))
  (Utilities|FlowControl|Delay 0.2)
  (Class|PlayerStashManager|SaveInventory))

(event EventInitGemUI
  (bind _asbp_main_menu_hud (Utilities|Casting|CastToBP_MainMenuHUD (HUD|GetHUD (Game|GetPlayerController 0))))
  (bind _aswb_main_menu (Utilities|Casting|CastToWB_MainMenu (Variables|/Script/ExtractionGame.MainMenuHUD|GetMainMenuWidget _asbp_main_menu_hud)))
  (Default|InitGemsMainMenu (Variables|/Game/Blueprints/Widgets/MainMenu/Inventory/WB_MainMenuStash.WB_MainMenuStash_C|GetWB_CharacterInventory (Variables|/Game/Blueprints/Widgets/MainMenu/WB_MainMenu.WB_MainMenu_C|GetWB_MainMenuStash _aswb_main_menu)) self))

(event EventOnSave
  (bind _asbp_game_instance (Utilities|Casting|CastToBP_GameInstance (Game|GetGameInstance)))
  (bind _returnvalue (Class|InventoryComp|GetItemsasAddItemInfo (Variables|Default|GetStashInventory)))
  (Utilities|Array|Clear (Variables|/Game/Blueprints/Core/BP_GameInstance.BP_GameInstance_C|GetSavedStash _asbp_game_instance))
  (for _array_element _returnvalue
    (Utilities|Array|Add (Variables|/Game/Blueprints/Core/BP_GameInstance.BP_GameInstance_C|GetSavedStash _asbp_game_instance) _array_element)))

(event EventOnGemInventoryChanged
  (Utilities|FlowControl|Sequence
    (:then_0
      (bind _asbp_main_menu_hud (Utilities|Casting|CastToBP_MainMenuHUD (HUD|GetHUD (Game|GetPlayerController 0))))
      (bind _aswb_main_menu (Utilities|Casting|CastToWB_MainMenu (Variables|/Script/ExtractionGame.MainMenuHUD|GetMainMenuWidget _asbp_main_menu_hud)))
      (bind _returnvalue (Class|PlayerStashManager|GetGemInventoryStruct))
      (Default|BetterUpdateGems (Variables|/Game/Blueprints/Widgets/MainMenu/Inventory/WB_MainMenuStash.WB_MainMenuStash_C|GetWB_CharacterInventory (Variables|/Game/Blueprints/Widgets/MainMenu/WB_MainMenu.WB_MainMenu_C|GetWB_MainMenuStash _aswb_main_menu)) _returnvalue))
    (:then_1
      (Utilities|FlowControl|Sequence
        (:then_0
          (bind _returnvalue_2 (Class|PlayerStashManager|GetLeftArmAbilityInfo))
          (if (not (Utilities|Enum|Equal(Enum) (.AbilityName (Utilities|Struct|BreakAbilityStruct _returnvalue_2)) "Punch"))
            (bind _asextraction_game_instance (Utilities|Casting|CastToExtractionGameInstance (Game|GetGameInstance)))
            (if (not (Utilities|Array|ContainsItem (Class|PlayerSaveData|GetSavedAbilities (Variables|/Script/ExtractionGame.ExtractionGameInstance|GetSaveData _asextraction_game_instance)) (.AbilityName (Utilities|Struct|BreakAbilityStruct _returnvalue_2))))
              (Class|PlayerSaveData|AddtoSavedAbility (Variables|/Script/ExtractionGame.ExtractionGameInstance|GetSaveData _asextraction_game_instance) (.AbilityName (Utilities|Struct|BreakAbilityStruct _returnvalue_2)))
              (bind _returnvalue_3 (UserInterface|CreateWidget "/Game/Blueprints/Widgets/WB_NewAbilityUnlocked.WB_NewAbilityUnlocked_C"))
              (UserInterface|Viewport|AddtoViewport _returnvalue_3 0)
              (Default|InitAbility _returnvalue_3 (.AbilityDescription (Utilities|Struct|BreakAbilityStruct _returnvalue_2)) (.AbilityName (Utilities|Struct|BreakAbilityStruct _returnvalue_2)) (.Image (Utilities|Struct|BreakAbilityStruct _returnvalue_2))))))
        (:then_1
          (bind _returnvalue_4 (Class|PlayerStashManager|GetRightArmAbilityInfo))
          (if (not (Utilities|Enum|Equal(Enum) (.AbilityName (Utilities|Struct|BreakAbilityStruct _returnvalue_4)) "Punch"))
            (bind _asextraction_game_instance_2 (Utilities|Casting|CastToExtractionGameInstance (Game|GetGameInstance)))
            (if (not (Utilities|Array|ContainsItem (Class|PlayerSaveData|GetSavedAbilities (Variables|/Script/ExtractionGame.ExtractionGameInstance|GetSaveData _asextraction_game_instance_2)) (.AbilityName (Utilities|Struct|BreakAbilityStruct _returnvalue_4))))
              (Class|PlayerSaveData|AddtoSavedAbility (Variables|/Script/ExtractionGame.ExtractionGameInstance|GetSaveData _asextraction_game_instance_2) (.AbilityName (Utilities|Struct|BreakAbilityStruct _returnvalue_4)))
              (bind _returnvalue_5 (UserInterface|CreateWidget "/Game/Blueprints/Widgets/WB_NewAbilityUnlocked.WB_NewAbilityUnlocked_C"))
              (UserInterface|Viewport|AddtoViewport _returnvalue_5 0)
              (Default|InitAbility _returnvalue_5 (.AbilityDescription (Utilities|Struct|BreakAbilityStruct _returnvalue_4)) (.AbilityName (Utilities|Struct|BreakAbilityStruct _returnvalue_4)) (.Image (Utilities|Struct|BreakAbilityStruct _returnvalue_4))))))))))

(event EventInitStartingItems
  (for _array_element (Variables|Default|GetStartingItems)
    (for _index (range 0 (- (.Count (Utilities|Struct|BreakAddItemStashManager _array_element)) 1))
      (bind _returnvalue (Utilities|GetDataTableRow "/Game/DataAssets/DataTables/DT_Items.DT_Items" (.Item (Utilities|Struct|BreakAddItemStashManager _array_element)))
        (:then
          (Class|InventoryComp|TryAddItembyAddItemInfo (Variables|Default|GetStashInventory) (Utilities|Struct|MakeAddItemInfo (Math|Vector2D|MakeVector2D (Math|Conversions|ToFloat(Integer) (.SizeX (Utilities|Struct|BreakItemDataStruct _returnvalue))) (Math|Conversions|ToFloat(Integer) (.SizeY (Utilities|Struct|BreakItemDataStruct _returnvalue)))) (Utilities|Array|Get(acopy) (.Icon (Utilities|Struct|BreakItemDataStruct _returnvalue))) (.IconRotated (Utilities|Struct|BreakItemDataStruct _returnvalue)) (.ItemCost (Utilities|Struct|BreakItemDataStruct _returnvalue)) (.ItemName (Utilities|Struct|BreakItemDataStruct _returnvalue)) (.ItemType (Utilities|Struct|BreakItemDataStruct _returnvalue)) (.Rarity (Utilities|Struct|BreakItemDataStruct _returnvalue)) (.Description (Utilities|Struct|BreakItemDataStruct _returnvalue)) (.GemType (Utilities|Struct|BreakItemDataStruct _returnvalue)) (.Polish (Utilities|Struct|BreakAddItemStashManager _array_element)) (.Item (Utilities|Struct|BreakAddItemStashManager _array_element))))
          (Class|PlayerStashManager|SaveInventory))))))

(fn ConstructionScript)