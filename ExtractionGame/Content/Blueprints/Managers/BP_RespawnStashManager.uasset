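; Respawn-screen stash manager that connects the stash and player inventory components to the extraction game HUD's respawn stash widgets on BeginPlay.
; OnSave replaces the game instance's SavedStash with the current stash items.
; Main-menu widget binding and the logic to restore saved or DataTable starting items are disconnected, so nothing here loads the stash.
; InitGemUI is an empty stub.
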(event EventBeginPlay
  (bind _stashinventory (Variables|Default|GetStashInventory))
  (bind _playerinventory (Variables|Default|GetPlayerInventory))
  (bind _asbp_extraction_game_hud (Utilities|Casting|CastToBP_ExtractionGameHUD (HUD|GetHUD (Game|GetPlayerController 0))))
  (Class|InventoryComp|SetInventoryWidget _stashinventory (Variables|/Game/Blueprints/Widgets/Respawn/WB_RespawnStash.WB_RespawnStash_C|GetWB_StashInventory (Variables|/Game/Blueprints/Widgets/Respawn/WB_Respawn.WB_Respawn_C|GetStashWidget (Variables|/Game/Blueprints/Gameplay/Core/BP_ExtractionGameHUD.BP_ExtractionGameHUD_C|GetRespawnWidget _asbp_extraction_game_hud))))
  (Default|Init (Variables|/Game/Blueprints/Widgets/Respawn/WB_RespawnStash.WB_RespawnStash_C|GetWB_StashInventory (Variables|/Game/Blueprints/Widgets/Respawn/WB_Respawn.WB_Respawn_C|GetStashWidget (Variables|/Game/Blueprints/Gameplay/Core/BP_ExtractionGameHUD.BP_ExtractionGameHUD_C|GetRespawnWidget _asbp_extraction_game_hud))) 8e+01 _stashinventory)
  (Default|Init (Variables|/Game/Blueprints/Widgets/Respawn/WB_RespawnStash.WB_RespawnStash_C|GetPlayerInventoryWidget (Variables|/Game/Blueprints/Widgets/Respawn/WB_Respawn.WB_Respawn_C|GetStashWidget (Variables|/Game/Blueprints/Gameplay/Core/BP_ExtractionGameHUD.BP_ExtractionGameHUD_C|GetRespawnWidget _asbp_extraction_game_hud))) 8e+01 _playerinventory)
  (Class|InventoryComp|SetInventoryWidget _playerinventory (Variables|/Game/Blueprints/Widgets/Respawn/WB_RespawnStash.WB_RespawnStash_C|GetPlayerInventoryWidget (Variables|/Game/Blueprints/Widgets/Respawn/WB_Respawn.WB_Respawn_C|GetStashWidget (Variables|/Game/Blueprints/Gameplay/Core/BP_ExtractionGameHUD.BP_ExtractionGameHUD_C|GetRespawnWidget _asbp_extraction_game_hud)))))

(event EventInitGemUI)

(event EventOnSave
  (bind _asbp_game_instance (Utilities|Casting|CastToBP_GameInstance (Game|GetGameInstance)))
  (bind _returnvalue (Class|InventoryComp|GetItemsasAddItemInfo (Variables|Default|GetStashInventory)))
  (Utilities|Array|Clear (Variables|/Game/Blueprints/Core/BP_GameInstance.BP_GameInstance_C|GetSavedStash _asbp_game_instance))
  (for _array_element _returnvalue
    (Utilities|Array|Add (Variables|/Game/Blueprints/Core/BP_GameInstance.BP_GameInstance_C|GetSavedStash _asbp_game_instance) _array_element)))

(fn ConstructionScript)