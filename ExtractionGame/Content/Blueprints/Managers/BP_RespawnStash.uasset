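; Respawn stash manager that connects stash and player inventory components to the respawn screen's UI in an extraction game.
; One second after BeginPlay, it gets the respawn stash widget from the HUD and cross-links both inventories with their grid widgets.
; It also initializes the character inventory's gem display from the player inventory and itself.
; UpdateGemUI prints debug text and re-runs only the respawn gem setup, reusing the BeginPlay HUD cast.
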(event EventBeginPlay
  (bind _stashinventory (Variables|Default|GetStashInventory))
  (bind _playerinventory (Variables|Default|GetPlayerInventory))
  (Utilities|FlowControl|Delay 1.0)
  (bind _asbp_extraction_game_hud (Utilities|Casting|CastToBP_ExtractionGameHUD (HUD|GetHUD (Game|GetPlayerController 0))))
  (Class|InventoryComp|SetInventoryWidget _stashinventory (Variables|/Game/Blueprints/Widgets/Respawn/WB_RespawnStash.WB_RespawnStash_C|GetWB_StashInventory (Variables|/Game/Blueprints/Widgets/Respawn/WB_Respawn.WB_Respawn_C|GetWB_RespawnStash (Variables|/Game/Blueprints/Gameplay/Core/BP_ExtractionGameHUD.BP_ExtractionGameHUD_C|GetRespawnWidget _asbp_extraction_game_hud))))
  (Default|Init (Variables|/Game/Blueprints/Widgets/Respawn/WB_RespawnStash.WB_RespawnStash_C|GetWB_StashInventory (Variables|/Game/Blueprints/Widgets/Respawn/WB_Respawn.WB_Respawn_C|GetWB_RespawnStash (Variables|/Game/Blueprints/Gameplay/Core/BP_ExtractionGameHUD.BP_ExtractionGameHUD_C|GetRespawnWidget _asbp_extraction_game_hud))) 8e+01 _stashinventory)
  (Default|Init (Variables|/Game/Blueprints/Widgets/Respawn/WB_RespawnStash.WB_RespawnStash_C|GetPlayerInventoryWidget (Variables|/Game/Blueprints/Widgets/Respawn/WB_Respawn.WB_Respawn_C|GetWB_RespawnStash (Variables|/Game/Blueprints/Gameplay/Core/BP_ExtractionGameHUD.BP_ExtractionGameHUD_C|GetRespawnWidget _asbp_extraction_game_hud))) 8e+01 _playerinventory)
  (Class|InventoryComp|SetInventoryWidget _playerinventory (Variables|/Game/Blueprints/Widgets/Respawn/WB_RespawnStash.WB_RespawnStash_C|GetPlayerInventoryWidget (Variables|/Game/Blueprints/Widgets/Respawn/WB_Respawn.WB_Respawn_C|GetWB_RespawnStash (Variables|/Game/Blueprints/Gameplay/Core/BP_ExtractionGameHUD.BP_ExtractionGameHUD_C|GetRespawnWidget _asbp_extraction_game_hud))))
  (Default|InitGems (Variables|/Game/Blueprints/Widgets/Respawn/WB_RespawnStash.WB_RespawnStash_C|GetWB_CharacterInventory (Variables|/Game/Blueprints/Widgets/Respawn/WB_Respawn.WB_Respawn_C|GetWB_RespawnStash (Variables|/Game/Blueprints/Gameplay/Core/BP_ExtractionGameHUD.BP_ExtractionGameHUD_C|GetRespawnWidget _asbp_extraction_game_hud))) (Variables|Default|GetPlayerInventory))
  (Default|InitGemsRespawn (Variables|/Game/Blueprints/Widgets/Respawn/WB_RespawnStash.WB_RespawnStash_C|GetWB_CharacterInventory (Variables|/Game/Blueprints/Widgets/Respawn/WB_Respawn.WB_Respawn_C|GetWB_RespawnStash (Variables|/Game/Blueprints/Gameplay/Core/BP_ExtractionGameHUD.BP_ExtractionGameHUD_C|GetRespawnWidget _asbp_extraction_game_hud))) self))

(event EventUpdateGemUI
  (Development|PrintText "good101" true true "(R=0.000000,G=0.660000,B=1.000000,A=1.000000)" 9e+01)
  (Default|InitGemsRespawn (Variables|/Game/Blueprints/Widgets/Respawn/WB_RespawnStash.WB_RespawnStash_C|GetWB_CharacterInventory (Variables|/Game/Blueprints/Widgets/Respawn/WB_Respawn.WB_Respawn_C|GetWB_RespawnStash (Variables|/Game/Blueprints/Gameplay/Core/BP_ExtractionGameHUD.BP_ExtractionGameHUD_C|GetRespawnWidget (stale EventBeginPlay _asbp_extraction_game_hud)))) self))

(fn ConstructionScript)