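; BP_PartyManager is a party manager that links session joining and party player updates to the game instance and main menu camera.
; On BeginPlay it binds to ExtractionGameInstance's join-session completion, then connects to the saved session when that fires, without checking the success flag.
; UpdatePlayers prints a debug message and passes the PartyPlayers count to BP_MainMenuCam through OnPartyUpdated.
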(event Custom|OnJoinSessionComplete
  (params (bWasSuccess :type Boolean))
  (Class|ExtractionGameInstance|ConnecttoCurrentlySavedSession (stale EventBeginPlay _asextraction_game_instance)))

(event EventUpdatePlayers
  (Development|PrintText "updating players")
  (bind _returnvalue (Actor|GetActorOfClass "/Game/Blueprints/Cameras/BP_MainMenuCam.BP_MainMenuCam_C"))
  (Default|OnPartyUpdated _returnvalue (Utilities|Array|Length (Variables|Default|GetPartyPlayers))))

(event EventBeginPlay
  (bind _asextraction_game_instance (Utilities|Casting|CastToExtractionGameInstance (Game|GetGameInstance)))
  (EventDispatchers|AssignOnJoinSessionComplete _asextraction_game_instance (delegate Custom|OnJoinSessionComplete)))

(fn ConstructionScript)