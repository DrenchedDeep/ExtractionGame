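; BP_WizardGuy is a wizard with a gem-equipping UI, apparently a test of gem slots on body parts.
; BeginPlay creates the gem equip master widget, registers arm and head sockets, then hides the UI.
; ToggleUI switches the widget and, optionally, the world gem buttons.
; AddSocket and SpawnAbility are empty; the data-table-driven spawning of gem buttons at mesh sockets is disconnected, so GemButtons is never filled here.
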(event EventBeginPlay
  (bind _returnvalue (UserInterface|CreateWidget "/Game/Blueprints/NewGemEquippingTest/WB_WizardGemEquipMaster.WB_WizardGemEquipMaster_C"))
  (Variables|Default|SetGemEquipMaster _returnvalue)
  (UserInterface|Viewport|AddtoViewport _returnvalue -100000)
  (CallFunction|AddSocket "LeftArmGemSlot1" "LeftArm0")
  (CallFunction|AddSocket "LeftArmGemSlot2" "LeftArm1")
  (CallFunction|AddSocket "RightArmGemSlot1" "RightArm0")
  (CallFunction|AddSocket "RightArmGemSlot2" "RightArm1")
  (CallFunction|AddSocket "HeadGemSlotSocket" "Head")
  (CallFunction|ToggleUI false false))

(fn ConstructionScript)

(fn AddSocket
  (params (SocketName :type Name) (BodyPart :type EBodyPart%20Enum :default "None")))

(fn SpawnAbility)

(fn ToggleUI
  (params (Visible :type Boolean) (DontDoGemButtons :type Boolean))
  (if DontDoGemButtons
    _
    (else
      (for _array_element (Variables|Default|GetGemButtons)
        (Rendering|SetActorHiddenInGame _array_element (not Visible)))))
  (if Visible
    (Widget|SetVisibility (Variables|Default|GetGemEquipMaster) "Visible")
    (else
      (Widget|SetVisibility (Variables|Default|GetGemEquipMaster) "Hidden"))))