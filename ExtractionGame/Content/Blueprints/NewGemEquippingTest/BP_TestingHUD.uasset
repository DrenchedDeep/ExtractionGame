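; BP_TestingHUD is the HUD for the gem equipping test, managing the stash inventory UI and its reminder widget.
; On BeginPlay it displays the stash widget, links it to BP_PlayerStashManager's inventory component, and creates the open-stash reminder without showing it.
; ToggleStash uses the widget's returned state to either hide BP_WizardGuy's gem bars and remove the reminder, or show both.
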(event Custom|ToggleStash
  (bind _isshowing (Default|ToggleStash (Variables|Default|GetStashInventory)))
  (bind _returnvalue (Actor|GetActorOfClass "/Game/Blueprints/NewGemEquippingTest/BP_WizardGuy.BP_WizardGuy_C"))
  (if _isshowing
    (Default|ToggleGemBars (Variables|/Game/Blueprints/NewGemEquippingTest/BP_WizardGuy.BP_WizardGuy_C|GetGemEquipMaster _returnvalue) "Hidden")
    (Widget|RemovefromParent (Variables|Default|GetStashReminder))
    (else
      (Default|ToggleGemBars (Variables|/Game/Blueprints/NewGemEquippingTest/BP_WizardGuy.BP_WizardGuy_C|GetGemEquipMaster _returnvalue) "Visible")
      (UserInterface|Viewport|AddtoViewport (Variables|Default|GetStashReminder) 0))))

(event EventBeginPlay
  (bind _returnvalue (UserInterface|CreateWidget "/Game/Blueprints/NewGemEquippingTest/WB_NewStashInventory.WB_NewStashInventory_C"))
  (Variables|Default|SetStashInventory _returnvalue)
  (UserInterface|Viewport|AddtoViewport _returnvalue 0)
  (bind _returnvalue_2 (Actor|GetActorOfClass "/Game/Blueprints/Managers/BP_PlayerStashManager.BP_PlayerStashManager_C"))
  (Default|Init (Variables|/Game/Blueprints/NewGemEquippingTest/WB_NewStashInventory.WB_NewStashInventory_C|GetWB_StashInventory _returnvalue) 75.0 (Variables|/Script/ExtractionGame.PlayerStashManager|GetStashInventory _returnvalue_2))
  (Class|InventoryComp|SetInventoryWidget (Variables|/Script/ExtractionGame.PlayerStashManager|GetStashInventory _returnvalue_2) (Variables|/Game/Blueprints/NewGemEquippingTest/WB_NewStashInventory.WB_NewStashInventory_C|GetWB_StashInventory _returnvalue))
  (bind _returnvalue_3 (UserInterface|CreateWidget "/Game/Blueprints/NewGemEquippingTest/WB_OpenStashReminder.WB_OpenStashReminder_C"))
  (Variables|Default|SetStashReminder _returnvalue_3))

(fn ConstructionScript)