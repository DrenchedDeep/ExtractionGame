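; Geyser spawn point actor that switches between smoking, active and deactivated states and rains essence pickups while active.
; Status updates toggle the geyser VFX and recolor or hide its widget icon, with a shockwave burst on activation; the smoke toggle is an empty stub.
; While active, the authority's Tick spawns BP_EssenceObject on a timed interval, high above the geyser at a random horizontal offset.
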(event EventOnGeyserStatusUpdated
  (bind _returnvalue (Class|GeyserSpawnpoint|GetGeyserState))
  (Development|PrintText (Utilities|Text|ToText(String) (Utilities|String|EnumtoString _returnvalue)))
  (switch Utilities|FlowControl|Switch|SwitchonEGeyserStates _returnvalue
    (:Smoking
      (CallFunction|ToggleGeiserSmoke true)
      (CallFunction|ToggleGeiserVFX false)
      (CallFunction|ToggleIcon true (Variables|Default|GetSmokingColor))
      (Variables|Default|SetSpawnItems false))
    (:Active
      (CallFunction|ToggleGeiserSmoke false)
      (CallFunction|ToggleGeiserVFX true)
      (Niagara|SpawnSystematLocation "/Game/ParticleSystems/ExtractionBeacon/NS_ExtractionBeaconShockwave.NS_ExtractionBeaconShockwave" (Transformation|GetActorLocation) (Transformation|GetActorRotation))
      (CallFunction|ToggleIcon true (Variables|Default|GetActiveColor))
      (Networking|SwitchHasAuthority
        (:Authority
          (Variables|Default|SetSpawnItems true))))
    (:Deactive
      (CallFunction|ToggleGeiserSmoke false)
      (CallFunction|ToggleGeiserVFX false)
      (CallFunction|ToggleIcon false (Variables|Default|GetDefaultColor))
      (Variables|Default|SetSpawnItems false))))

(event EventTick
  (params (DeltaSeconds :type Float%20%28single-precision%29))
  (bind _returnvalue (Math|Random|RandomUnitVector))
  (Networking|SwitchHasAuthority
    (:Authority
      (if (Variables|Default|GetSpawnItems)
        (if (>= (- (Utilities|Time|GetTimeSeconds) (Variables|Default|GetLastItemDrop)) (Variables|Default|GetItemDropTime))
          (Variables|Default|SetLastItemDrop (Utilities|Time|GetTimeSeconds))
          (Game|SpawnActorfromClass "/Game/Blueprints/BP_EssenceObject.BP_EssenceObject_C" (Math|Transform|MakeTransform (+ (Transformation|GetActorLocation) (Math|Vector|MakeVector (* (.x _returnvalue) 5e+02) (* (.y _returnvalue) 5e+02) 3e+03)) "0, 0, 0" "1.000000,1.000000,1.000000") "Undefined" "MultiplyWithRoot" 0 0))))))

(event EventBeginPlay
  (bind _aswb_geiser_icon (Utilities|Casting|CastToWB_GeiserIcon (UserInterface|GetWidget (Variables|Default|GetGeiserIcon))))
  (Variables|/Game/Blueprints/Widgets/WB_GeiserIcon.WB_GeiserIcon_C|SetGeiserActor _aswb_geiser_icon self))

(fn ConstructionScript)

(fn ToggleGeiserSmoke
  (params (Visible :type Boolean)))

(fn ToggleGeiserVFX
  (params (Visible :type Boolean))
  (Rendering|SetVisibility (Variables|Default|GetNS_Gieser) Visible false))

(fn ToggleIcon
  (params (Visible :type Boolean) (Color :type Color%20Structure))
  (Rendering|SetVisibility (Variables|Default|GetGeiserIcon) Visible false)
  (bind _aswb_geiser_icon (Utilities|Casting|CastToWB_GeiserIcon (UserInterface|GetWidget (Variables|Default|GetGeiserIcon))))
  (Default|SetColor _aswb_geiser_icon Color))