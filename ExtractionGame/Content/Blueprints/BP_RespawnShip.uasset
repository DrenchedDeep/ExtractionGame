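; Respawn ship pawn that crash-lands and ejects the player as a ragdoll before handing control to a first-person character.
; On BeginPlay it passes itself to BP_ShipSpawnPoint to be positioned.
; CrashLand snaps it to the impact, launches a spawned physics door and the ragdoll, and stops the trail effects.
; The ragdoll collider arms after a short delay; its overlap spawns and possesses the character on authority if controlled.
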(event OnComponentBeginOverlap(RagdollCollider)
  (params (OverlappedComponent :type Primitive%20Component%20Object%20Reference) (OtherActor :type Actor%20Object%20Reference) (OtherComp :type Primitive%20Component%20Object%20Reference) (OtherBodyIndex :type Integer) (bFromSweep :type Boolean) (SweepResult :type Hit%20Result%20Structure%20%28by%20ref%29))
  (CallFunction|SpawnPlayer))

(event Custom|CustomEvent
  (Collision|SetCollisionEnabled (Variables|Default|GetRagdollCollider) "QueryOnly"))

(event EventBeginPlay
  (bind _returnvalue (Actor|GetActorOfClass "/Game/Blueprints/BP_ShipSpawnPoint.BP_ShipSpawnPoint_C"))
  (Class|ShipSpawnPoint|MovetoPosition _returnvalue self)
  (Collision|SetCollisionEnabled (Variables|Default|GetRagdollCollider) "NoCollision")
  (Variables|Default|SetPrimary (Variables|Default|GetMain))
  (Variables|Default|SetBackLeft (Variables|Default|GetBackLeft0))
  (Variables|Default|SetBackMid (Variables|Default|GetBackMid0))
  (Variables|Default|SetBackRight (Variables|Default|GetBackRight0))
  (Variables|Default|SetFrontLeft (Variables|Default|GetFrontLeft0))
  (Variables|Default|SetFrontMid (Variables|Default|GetFrontMid0))
  (Variables|Default|SetFrontRight (Variables|Default|GetFrontRight0)))

(event Collision|EventActorBeginOverlap
  (params (OtherActor :type Actor%20Object%20Reference)))

(event EventTick
  (params (DeltaSeconds :type Float%20%28single-precision%29)))

(event EventCrashLand
  (params (HitResult :type Hit%20Result%20Structure))
  (bind (_bblockinghit _binitialoverlap _time _distance _location _impactpoint _normal) (Collision|BreakHitResult HitResult))
  (bind _returnvalue (Transformation|GetActorForwardVector))
  (bind _returnvalue_2 (Transformation|GetActorRightVector))
  (bind _impact (Variables|Default|GetImpact))
  (bind _spacebowlunreal_spaceshipdoor (Variables|Default|GetSpaceBowlUnreal_SpaceShipDoor))
  (bind _spawnoffset (Variables|Default|GetSpawnOffset))
  (bind _buffer (Variables|Default|GetBuffer))
  (bind _skeletalmesh (Variables|Default|GetSkeletalMesh))
  (bind _returnvalue_3 (Math|Vector|RotateVectorAroundAxis _returnvalue 2e+02 _returnvalue_2))
  (bind _returnvalue_4 (* _normal _buffer))
  (bind _returnvalue_5 (+ _returnvalue_4 _impactpoint))
  (bind _returnvalue_6 (* _returnvalue_3 _spawnoffset))
  (bind _returnvalue_7 (+ _returnvalue_5 _returnvalue_6))
  (Utilities|Time|SetTimerbyEvent (delegate Custom|CustomEvent) 0.2)
  (Transformation|SetActorLocation _returnvalue_5 false true)
  (Rendering|SetVisibility _spacebowlunreal_spaceshipdoor false false)
  (bind _returnvalue_8 (Game|SpawnActorfromClass "/Script/Engine.StaticMeshActor" (Math|Transform|MakeTransform _returnvalue_7 (Transformation|GetWorldRotation _spacebowlunreal_spaceshipdoor)) "AlwaysSpawn" "OverrideRootScale" (Pawn|GetController) 0))
  (Transformation|SetWorldLocation _skeletalmesh _returnvalue_7 false true)
  (Physics|SetSimulatePhysics _skeletalmesh true)
  (Class|PrimitiveComponent|SetAllPhysicsLinearVelocity _skeletalmesh "0, 0, 0" false)
  (Physics|SetPhysicsLinearVelocity _skeletalmesh (* _returnvalue_3 (Variables|Default|GetPlayer%20Force)) false "None")
  (Transformation|SetMobility _returnvalue_8 "Movable")
  (Components|StaticMesh|SetStaticMesh (Variables|/Script/Engine.StaticMeshActor|GetStaticMeshComponent _returnvalue_8) "/Game/Models/Props/PlayerSpawnBS/SpaceBowlUnreal_SpaceShipDoor.SpaceBowlUnreal_SpaceShipDoor")
  (Physics|SetSimulatePhysics (Variables|/Script/Engine.StaticMeshActor|GetStaticMeshComponent _returnvalue_8) true)
  (Physics|SetPhysicsLinearVelocity (Variables|/Script/Engine.StaticMeshActor|GetStaticMeshComponent _returnvalue_8) (* _returnvalue_3 (Variables|Default|GetForce)) false "None")
  (Class|PrimitiveComponent|AddTorqueinRadians (Variables|/Script/Engine.StaticMeshActor|GetStaticMeshComponent _returnvalue_8) (* (Math|Random|RandomUnitVector) (Variables|Default|GetTorque)) "None" true)
  (Rendering|SetVisibility _impact false false)
  (Components|Activation|Deactivate _impact)
  (Components|Activation|Deactivate (Variables|Default|GetTrail)))

(fn ConstructionScript)

(fn SpawnPlayer
  (bind _returnvalue (Pawn|GetController))
  (if (and (Class|Pawn|IsControlled) (Ability|HasAuthority))
    (Development|PrintString "GOOD")
    (bind _returnvalue_2 (Game|SpawnActorfromClass "/Game/Blueprints/Gameplay/Pawns/BP_FirstPersonCharacter.BP_FirstPersonCharacter_C" (Math|Transform|MakeTransform (Transformation|GetWorldLocation (Variables|Default|GetSkeletalMesh))) "AdjustIfPossibleButAlwaysSpawn" "OverrideRootScale" _returnvalue (Game|GetInstigator)))
    (Pawn|Possess _returnvalue _returnvalue_2)
    (Rendering|SetVisibility (Variables|Default|GetSkeletalMesh) false false)))