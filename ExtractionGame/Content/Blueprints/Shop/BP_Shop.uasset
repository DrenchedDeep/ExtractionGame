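; BP_Shop is the main-menu shop actor that backs the shop screen's inventories and stocks it with starting items.
; On BeginPlay it binds shop, buy and sell inventory components, plus the player controller's stash, to grid widgets in the main menu HUD, sharing the shop's tile size.
; It then fills the shop from DT_Items rows, pricing each by rarity, base cost and polish, with optional per-item polish overrides.
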(event EventBeginPlay
  (bind _returnvalue (Game|GetPlayerController 0))
  (bind _sellinventory (Variables|Default|GetSellInventory))
  (bind _buyinventory (Variables|Default|GetBuyInventory))
  (bind _shopinventory (Variables|Default|GetShopInventory))
  (bind _tilesize (Variables|/Script/ExtractionGame.InventoryComp|GetTileSize _shopinventory))
  (bind _asbp_main_menu_hud (Utilities|Casting|CastToBP_MainMenuHUD (HUD|GetHUD _returnvalue)))
  (bind _aswb_main_menu (Utilities|Casting|CastToWB_MainMenu (Variables|/Script/ExtractionGame.MainMenuHUD|GetMainMenuWidget _asbp_main_menu_hud)))
  (Default|Init (Variables|/Game/Blueprints/Widgets/MainMenu/Shop/WB_Shop.WB_Shop_C|GetShopInventoryWidget (Variables|/Game/Blueprints/Widgets/MainMenu/WB_MainMenu.WB_MainMenu_C|GetWB_Shop _aswb_main_menu)) _tilesize _shopinventory)
  (Class|InventoryComp|SetInventoryWidget (Variables|Default|GetShopInventory) (Variables|/Game/Blueprints/Widgets/MainMenu/Shop/WB_Shop.WB_Shop_C|GetShopInventoryWidget (Variables|/Game/Blueprints/Widgets/MainMenu/WB_MainMenu.WB_MainMenu_C|GetWB_Shop _aswb_main_menu)))
  (Default|Init (Variables|/Game/Blueprints/Widgets/MainMenu/Shop/WB_Shop.WB_Shop_C|GetBuyInventoryWidget (Variables|/Game/Blueprints/Widgets/MainMenu/WB_MainMenu.WB_MainMenu_C|GetWB_Shop _aswb_main_menu)) _tilesize _buyinventory)
  (Class|InventoryComp|SetInventoryWidget _buyinventory (Variables|/Game/Blueprints/Widgets/MainMenu/Shop/WB_Shop.WB_Shop_C|GetBuyInventoryWidget (Variables|/Game/Blueprints/Widgets/MainMenu/WB_MainMenu.WB_MainMenu_C|GetWB_Shop _aswb_main_menu)))
  (Default|Init (Variables|/Game/Blueprints/Widgets/MainMenu/Shop/WB_Shop.WB_Shop_C|GetSellInventoryWidget (Variables|/Game/Blueprints/Widgets/MainMenu/WB_MainMenu.WB_MainMenu_C|GetWB_Shop _aswb_main_menu)) _tilesize _sellinventory)
  (Class|InventoryComp|SetInventoryWidget _sellinventory (Variables|/Game/Blueprints/Widgets/MainMenu/Shop/WB_Shop.WB_Shop_C|GetSellInventoryWidget (Variables|/Game/Blueprints/Widgets/MainMenu/WB_MainMenu.WB_MainMenu_C|GetWB_Shop _aswb_main_menu)))
  (bind _asbp_main_menu_player_controller (Utilities|Casting|CastToBP_MainMenuPlayerController _returnvalue))
  (Default|Init (Variables|/Game/Blueprints/Widgets/MainMenu/Shop/WB_Shop.WB_Shop_C|GetPlayerStashWidget (Variables|/Game/Blueprints/Widgets/MainMenu/WB_MainMenu.WB_MainMenu_C|GetWB_Shop _aswb_main_menu)) _tilesize (Variables|/Script/ExtractionGame.PlayerStashManager|GetStashInventory (Variables|/Script/ExtractionGame.MainMenuPlayerController|GetPlayerStashManager _asbp_main_menu_player_controller)))
  (Class|InventoryComp|SetInventoryWidget (Variables|/Script/ExtractionGame.PlayerStashManager|GetStashInventory (Variables|/Script/ExtractionGame.MainMenuPlayerController|GetPlayerStashManager _asbp_main_menu_player_controller)) (Variables|/Game/Blueprints/Widgets/MainMenu/Shop/WB_Shop.WB_Shop_C|GetPlayerStashWidget (Variables|/Game/Blueprints/Widgets/MainMenu/WB_MainMenu.WB_MainMenu_C|GetWB_Shop _aswb_main_menu)))
  (CallFunction|AddStartingItemstoShop))

(fn ConstructionScript)

(fn AddStartingItemstoShop
  (for _array_element (Variables|Default|GetStartingItems)
    (bind _returnvalue (Utilities|GetDataTableRow "/Game/DataAssets/DataTables/DT_Items.DT_Items" (.ItemName (Utilities|Struct|BreakShopItem _array_element)))
      (:then
        (Class|InventoryComp|TryAddItembyAddItemInfo (Variables|Default|GetShopInventory) (Utilities|Struct|MakeAddItemInfo (Math|Vector2D|MakeVector2D (Math|Conversions|ToFloat(Integer) (.SizeX (Utilities|Struct|BreakItemDataStruct _returnvalue))) (Math|Conversions|ToFloat(Integer) (.SizeY (Utilities|Struct|BreakItemDataStruct _returnvalue)))) (Utilities|Array|Get(acopy) (.Icon (Utilities|Struct|BreakItemDataStruct _returnvalue))) (.IconRotated (Utilities|Struct|BreakItemDataStruct _returnvalue)) (Class|ExtractionGameBPLibrary|GetAdjustedPrice (.Rarity (Utilities|Struct|BreakItemDataStruct _returnvalue)) (.ItemCost (Utilities|Struct|BreakItemDataStruct _returnvalue)) (select (.bOverridePolish (Utilities|Struct|BreakShopItem _array_element)) (.PolishAmount (Utilities|Struct|BreakShopItem _array_element)) (.DefaultPolish (Utilities|Struct|BreakItemDataStruct _returnvalue)))) (.ItemName (Utilities|Struct|BreakItemDataStruct _returnvalue)) (.ItemType (Utilities|Struct|BreakItemDataStruct _returnvalue)) (.Rarity (Utilities|Struct|BreakItemDataStruct _returnvalue)) (.Description (Utilities|Struct|BreakItemDataStruct _returnvalue)) (.GemType (Utilities|Struct|BreakItemDataStruct _returnvalue)) (select (.bOverridePolish (Utilities|Struct|BreakShopItem _array_element)) (.PolishAmount (Utilities|Struct|BreakShopItem _array_element)) (.DefaultPolish (Utilities|Struct|BreakItemDataStruct _returnvalue))) (.ItemName (Utilities|Struct|BreakShopItem _array_element))))))))