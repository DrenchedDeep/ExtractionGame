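; HUD for the extraction game mode that creates and manages the player's UI widgets.
; BeginPlay builds the notification grid, score, crosshair, extraction timer and, after a short delay, pause menu.
; Events refresh score and timer and spawn kill and extraction notifications; functions handle inventory visibility, spaceship HUD and swapping pause menu with player bar.
; The end-of-extraction camera fade is disconnected, and ExtractionStarted still contains debug prints.
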(event EventBeginPlay
  (bind _returnvalue (Game|GetPlayerController 0))
  (bind _returnvalue_2 (UserInterface|CreateWidget "/Game/Blueprints/Widgets/Notifcation/WB_NotifcationGrid.WB_NotifcationGrid_C"))
  (bind _output_get (Variables|Default|SetNotificationGrid _returnvalue_2))
  (UserInterface|Viewport|AddtoViewport _output_get 0)
  (bind _returnvalue_3 (UserInterface|CreateWidget "/Game/Blueprints/Widgets/Extraction/WB_Extraction.WB_Extraction_C"))
  (Variables|Default|SetExtractionWidget _returnvalue_3)
  (bind _returnvalue_4 (UserInterface|CreateWidget "/Game/Blueprints/Widgets/WB_Score.WB_Score_C"))
  (Variables|Default|SetScoreWidget _returnvalue_4)
  (UserInterface|Viewport|AddtoViewport _returnvalue_4 -100)
  (bind _returnvalue_5 (UserInterface|CreateWidget "/Game/Blueprints/Widgets/Player/WB_CrossHair.WB_CrossHair_C" _returnvalue))
  (UserInterface|Viewport|AddtoViewport _returnvalue_5 0)
  (Utilities|FlowControl|Delay 0.2)
  (bind _returnvalue_6 (UserInterface|CreateWidget "/Game/Blueprints/Widgets/WB_PauseMenu.WB_PauseMenu_C" _returnvalue))
  (Variables|Default|SetPauseMenu _returnvalue_6))

(event EventUpdateScore
  (params (Kills :type Integer) (Deaths :type Integer))
  (Default|Refresh (Variables|Default|GetScoreWidget) Kills Deaths))

(event EventUpdateExtractionTimerWidget
  (params (ExtractionTimer :type Float%20%28single-precision%29))
  (bind _extractionwidget (Variables|Default|GetExtractionWidget))
  (if (UserInterface|Viewport|IsinViewport _extractionwidget)
    _
    (else
      (UserInterface|Viewport|AddtoViewport _extractionwidget 0)))
  (Utilities|IsValid _extractionwidget
    (:Is%20Valid
      (bind _aswb_extraction (Utilities|Casting|CastToWB_Extraction _extractionwidget))
      (Default|SetTimer _aswb_extraction ExtractionTimer)
      (if (and (<= ExtractionTimer 5.0) (!= (Variables|Default|GetSetCamFade) true))
        _))))

(event EventOnKill
  (params (VictimName :type String))
  (Utilities|IsValid (Variables|Default|GetCurrentKillNotif)
    (:Is%20Valid
      (Widget|RemovefromParent (Variables|Default|GetCurrentKillNotif)))
    (:Is%20Not%20Valid
      _))
  (bind _returnvalue (UserInterface|CreateWidget "/Game/Blueprints/Widgets/WB_KillNotification.WB_KillNotification_C"))
  (UserInterface|Viewport|AddtoViewport _returnvalue 0)
  (Default|OnKill _returnvalue VictimName)
  (Variables|Default|SetCurrentKillNotif _returnvalue))

(fn ConstructionScript)

(fn ToggleInventoryUI
  (params (Visible :type ESlateVisibility%20Enum :default "Visible"))
  (Widget|SetVisibility (Variables|Default|GetInventoryWidget) Visible))

(fn CreateSpaceShipHUD
  (bind _returnvalue (UserInterface|CreateWidget "/Game/Blueprints/Widgets/Spaceship/WB_SpaceShipHUD.WB_SpaceShipHUD_C"))
  (bind _output_get (Variables|Default|SetSpaceShipHUD _returnvalue))
  (return _output_get))

(fn RemoveSpaceShipHUD
  (bind _spaceshiphud (Variables|Default|GetSpaceShipHUD))
  (Utilities|IsValid _spaceshiphud
    (:Is%20Valid
      (Widget|RemovefromParent _spaceshiphud))))

(fn TogglePauseMenu
  (params (Enable :type Boolean))
  (if Enable
    (UserInterface|Viewport|AddtoViewport (Variables|Default|GetPauseMenu) 0)
    (Widget|RemovefromParent (Class|ExtractionGameHUD|GetPlayerBarWidget))
    (else
      (UserInterface|Viewport|AddtoViewport (Class|ExtractionGameHUD|GetPlayerBarWidget) 0)
      (Widget|RemovefromParent (Variables|Default|GetPauseMenu)))))

(fn ExtractionStarted
  (params (Location :type Vector) (Extractor :type BP%20Extractor%20Object%20Reference))
  (Development|PrintText "wtf" true true "(R=0.000000,G=0.660000,B=1.000000,A=1.000000)" 9e+01)
  (bind _returnvalue (UserInterface|CreateWidget "/Game/Blueprints/Widgets/Extraction/WB_ExtractionNotification.WB_ExtractionNotification_C"))
  (Development|PrintText "wtf?2" true true "(R=0.000000,G=0.660000,B=1.000000,A=1.000000)" 9e+01)
  (UserInterface|Viewport|AddtoViewport _returnvalue 0)
  (Development|PrintText "wtyf3?o" true true "(R=0.000000,G=0.660000,B=1.000000,A=1.000000)" 9e+01)
  (Default|Init _returnvalue Extractor Extractor)
  (Development|PrintText "test?" true true "(R=0.000000,G=0.660000,B=1.000000,A=1.000000)" 9e+01))