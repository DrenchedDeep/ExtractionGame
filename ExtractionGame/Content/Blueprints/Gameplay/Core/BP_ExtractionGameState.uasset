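; Game state for the extraction mode, handling ability registration, match-state reactions and item drops.
; On BeginPlay it copies mono, duo and trio abilities plus head effects from data maps into the AbilityHandlerSubSystem.
; State and top-three updates drive the local HUD, and Ending Game saves the player's inventory to stash.
; It also plays low-time VO with final music, and spawns physics-simulated items from DT_Items.
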(event Custom|CringeTest
  (bind _asbp_game_instance (Utilities|Casting|CastToBP_GameInstance (Game|GetGameInstance)))
  (Default|PlayVO _asbp_game_instance (Utilities|Array|Get(acopy) (Utilities|Array|MakeArray "/Game/Sound_Effects_SFX/CreatorInGame/creator_LowTimeLeft0.creator_LowTimeLeft0" "/Game/Sound_Effects_SFX/CreatorInGame/Creator_LowTimeLeft1.Creator_LowTimeLeft1" "/Game/Sound_Effects_SFX/CreatorInGame/Creator_LowTimeLeft2.Creator_LowTimeLeft2") (Math|Random|RandomIntegerinRange 0 2)))
  (Default|PlayGlobalMusic _asbp_game_instance "/Game/Sound_Effects_SFX/BGM/Bossbattle.Bossbattle" 5.0 1.0 5e+01 false)
  (Development|PrintString "Playing Final Music"))

(event EventBeginPlay
  (Utilities|FlowControl|Sequence
    (:then_0
      (CallFunction|LoadMonoType)
      (CallFunction|LoadDuoType)
      (CallFunction|LoadTrioType)
      (CallFunction|LoadHeadEffects))))

(event EventOnExtractionGameStateUpdated
  (bind _returnvalue (Class|ExtractionGameState|GetExtractionGameState))
  (bind _asbp_extraction_game_hud (Utilities|Casting|CastToBP_ExtractionGameHUD (HUD|GetHUD (Game|GetPlayerController 0))))
  (Default|GameStateChanged _asbp_extraction_game_hud _returnvalue)
  (switch Utilities|FlowControl|Switch|SwitchonEGameModeState _returnvalue
    (:EndingGame
      (bind _asbp_first_person_character (Utilities|Casting|CastToBP_FirstPersonCharacter (Pawn|GetControlledPawn (Game|GetPlayerController 0))))
      (Class|PlayerInventoryComponent|AddInventorytoSavedStash (Variables|/Script/ExtractionGame.ExtractionGameCharacter|GetInventoryComponent _asbp_first_person_character)))))

(event EventOnTopThreePlayersUpdated
  (bind _asbp_extraction_game_hud (Utilities|Casting|CastToBP_ExtractionGameHUD (HUD|GetHUD (Game|GetPlayerController 0))))
  (Default|EndMatch _asbp_extraction_game_hud))

(event EventGameNearlyOverBoys
  (CallFunction|CringeTest)
  (Development|PrintString "Client should be capable of playing final music on their own" true true "(R=1.000000,G=0.560248,B=0.000000,A=1.000000)" 2e+01))

(fn ConstructionScript)

(fn LoadMonoType
  (bind _data (LocalVariables|GetData))
  (bind _keys (Utilities|Map|Keys _data))
  (for _array_element _keys
    (Class|AbilityHandlerSubSystem|AddAbilitytoMap (Subsystems|GetAbilityHandlerSubSystem) _array_element (.Value (Utilities|Map|Find _data _array_element))))
  (Development|PrintString "Mono Abilities Loaded!" true true "(R=0.000000,G=1.000000,B=0.037928,A=1.000000)"))

(fn LoadDuoType
  (bind _data (LocalVariables|GetData))
  (bind _keys (Utilities|Map|Keys _data))
  (for _array_element _keys
    (Class|AbilityHandlerSubSystem|AddAbilitytoMap (Subsystems|GetAbilityHandlerSubSystem) _array_element (.Value (Utilities|Map|Find _data _array_element))))
  (Development|PrintString "Duo Abilities Loaded!" true true "(R=0.918360,G=1.000000,B=0.000000,A=1.000000)"))

(fn LoadTrioType
  (bind _data (LocalVariables|GetData))
  (bind _keys (Utilities|Map|Keys _data))
  (for _array_element _keys
    (Class|AbilityHandlerSubSystem|AddAbilitytoMap (Subsystems|GetAbilityHandlerSubSystem) _array_element (.Value (Utilities|Map|Find _data _array_element))))
  (Development|PrintString "Trio  Abilities Loaded!" true true "(R=1.000000,G=0.000000,B=0.099114,A=1.000000)"))

(fn DropItematLocation
  (params (ItemName :type Name) (SpawnLocation :type Vector) (SpawnDirection :type Vector) (Polish :type Float%20%28double-precision%29) (Rarity :type ERarityType%20Enum :default "Common"))
  (bind _returnvalue (Utilities|GetDataTableRow "/Game/DataAssets/DataTables/DT_Items.DT_Items" ItemName)
    (:then
      (Development|PrintText "found")
      (bind _returnvalue_2 (Game|SpawnActorfromClass (.ItemActor (Utilities|Struct|BreakItemDataStruct _returnvalue)) (Math|Transform|MakeTransform (+ SpawnLocation (/ (* SpawnDirection 500) 2)) "0, 0, 0" "1.000000,1.000000,1.000000") "Undefined" "MultiplyWithRoot" 0 true Polish 0))
      (bind _asbp_item (Utilities|Casting|CastToBP_Item _returnvalue_2))
      (Physics|SetSimulatePhysics (Variables|/Game/Inventory/Items/BP_Item.BP_Item_C|GetItemMesh _asbp_item) true))
    (:RowNotFound
      (Development|PrintText "not found"))))

(fn LoadHeadEffects
  (bind _data (LocalVariables|GetData))
  (bind _keys (Utilities|Map|Keys _data))
  (for (_array_element _array_index) _keys
    (Class|AbilityHandlerSubSystem|AddEffecttoMap (Subsystems|GetAbilityHandlerSubSystem) _array_index (.Value (Utilities|Map|Find _data _array_element))))
  (Development|PrintString "Head Abilities Loaded" true true "(R=0.787358,G=0.000000,B=1.000000,A=1.000000)"))