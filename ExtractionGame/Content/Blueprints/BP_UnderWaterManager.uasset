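; BP_UnderWaterManager is a manager that damages first-person player characters whose camera is underwater, treated as world Z at or below zero.
; On BeginPlay, only the authority starts a looping timer that fires every few seconds and prints a debug tick.
; Each tick walks the GameState PlayerArray, checks each character's camera height and applies fixed damage through its health component, crediting player controller 0 as instigator.
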(event Custom|CheckUnderWater
  (Development|PrintText "tick")
  (for _array_element (Variables|/Script/Engine.GameStateBase|GetPlayerArray (Game|GetGameState))
    (bind _asbp_first_person_character (Utilities|Casting|CastToBP_FirstPersonCharacter (PlayerState|GetPawn _array_element)))
    (if (<= (.z (Transformation|GetWorldLocation (Variables|/Game/Blueprints/Gameplay/Pawns/BP_FirstPersonCharacter.BP_FirstPersonCharacter_C|GetCamera _asbp_first_person_character))) 0.0)
      (Class|PlayerHealthComponent|ApplyDamage (Variables|/Script/ExtractionGame.ExtractionGameCharacter|GetPlayerHealthComponent _asbp_first_person_character) 6e+01 (Game|GetPlayerController 0)))))

(event EventBeginPlay
  (Networking|SwitchHasAuthority
    (:Authority
      (Utilities|Time|SetTimerbyEvent (delegate Custom|CheckUnderWater) 3.0 true))))

(fn ConstructionScript)