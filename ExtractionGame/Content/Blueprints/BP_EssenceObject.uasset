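; BP_EssenceObject is an essence pickup that grants essence to the first-person character who overlaps its sphere.
; A looping 30 Hz timer feeds the target's location to the Niagara PlayerLoc variable, using the pickup itself as the target until overlap.
; After overlap, the timer counts 1.5 seconds, then awards the essence and destroys the actor, which never moves itself.
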(event OnComponentBeginOverlap(Sphere)
  (params (OverlappedComponent :type Primitive%20Component%20Object%20Reference) (OtherActor :type Actor%20Object%20Reference) (OtherComp :type Primitive%20Component%20Object%20Reference) (OtherBodyIndex :type Integer) (bFromSweep :type Boolean) (SweepResult :type Hit%20Result%20Structure%20%28by%20ref%29))
  (bind _asbp_first_person_character (Utilities|Casting|CastToBP_FirstPersonCharacter OtherActor))
  (Variables|Default|SetTargetActor _asbp_first_person_character)
  (Variables|Default|SetMovingToPlayer true))

(event EventBeginPlay
  (Utilities|Time|SetTimerbyFunctionName 0 "MoveEssence" (/ 1.0 3e+01) true)
  (Variables|Default|SetTargetActor self))

(fn ConstructionScript)

(fn MoveEssence
  (bind _targetactor (Variables|Default|GetTargetActor))
  (Utilities|IsValid _targetactor
    (:Is%20Valid
      (Class|NiagaraComponent|SetVariablePosition (Variables|Default|GetNS_Essence) "PlayerLoc" (Transformation|GetActorLocation _targetactor))
      (if (Variables|Default|GetMovingToPlayer)
        (bind _output_get (Variables|Default|SetTimePassed (+ (Variables|Default|GetTimePassed) (/ 1.0 3e+01))))
        (if (>= _output_get 1.5)
          (Utilities|Time|ClearTimerbyFunctionName 0 "MoveEssence")
          (bind _asbp_first_person_character (Utilities|Casting|CastToBP_FirstPersonCharacter (Variables|Default|GetTargetActor)))
          (Class|ExtractionGameCharacter|AddEssence _asbp_first_person_character 1e+01)
          (Actor|DestroyActor))))))