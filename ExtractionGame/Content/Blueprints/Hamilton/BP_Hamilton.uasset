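; BP_Hamilton is an actor that fires lightning at zappable actors within its sphere.
; On Tick, throttled by TraceCooldown, it checks the Sphere's overlapping actors for BPI_Zappable and asks each whether it can be zapped.
; For each willing actor it spawns an NS_HamiltonLightning Niagara effect ending at that actor and sends ZapMessage.
; An older random-direction line trace that spawned attached bolts at impact points remains disconnected.
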(event EventTick
  (params (DeltaSeconds :type Float%20%28single-precision%29))
  (CallFunction|UpdateLightning))

(fn ConstructionScript)

(fn UpdateLightning
  (if (>= (- (Utilities|Time|GetTimeSeconds) (Variables|Default|GetLastTrace)) (Variables|Default|GetTraceCooldown))
    (Variables|Default|SetLastTrace (Utilities|Time|GetTimeSeconds))
    (for _array_element (Collision|GetOverlappingActors (Variables|Default|GetSphere) 0 :!class /Script/Engine.PrimitiveComponent)
      (if (Utilities|DoesObjectImplementInterface _array_element "/Game/Blueprints/Hamilton/BPI_Zappable.BPI_Zappable_C")
        (bind _canzap (Class|BPIZappable|CanZap(Message) _array_element))
        (if _canzap
          (bind _returnvalue (Niagara|SpawnSystematLocation "/Game/ParticleSystems/Ability/NS_HamiltonLightning.NS_HamiltonLightning" (Transformation|GetActorLocation)))
          (Utilities|IsValid _returnvalue
            (:Is%20Valid
              (Niagara|SetNiagaraVariable(Vector3) _returnvalue "StartLocation" "0.000000,0.000000,200.000000")
              (Niagara|SetNiagaraVariable(Vector3) _returnvalue "EndLocation" (Transformation|GetActorLocation _array_element))
              (Class|BPIZappable|Zap(Message) _array_element))))))))