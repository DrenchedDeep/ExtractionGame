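; Gem is an interactable pickup item that players can collect into their inventory.
; Focus events toggle custom depth on its static mesh, likely for an outline highlight.
; On interact it prints its gem type and polish stats, then, for a BP_FirstPersonCharacter invoker, calls ServerManageGem and adds the gem item to InventoryComponent with client simulation enabled.
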(event Collision|EventActorBeginOverlap
  (params (OtherActor :type Actor%20Object%20Reference)))

(event EventTick
  (params (DeltaSeconds :type Float%20%28single-precision%29)))

(event EventOnStartFocus
  (Rendering|SetRenderCustomDepth (Variables|Default|GetStaticMesh) true))

(event EventOnInteract
  (params (Invoker :type Actor%20Object%20Reference))
  (Development|PrintString (Utilities|String|Append (Utilities|String|EnumtoString (Class|Gem|GetGemType)) (Utilities|String|Append " with stats" (Utilities|String|ToString(Float) (Class|Gem|GetPolish)))))
  (bind _asbp_first_person_character (Utilities|Casting|CastToBP_FirstPersonCharacter Invoker))
  (Default|ServerManageGem _asbp_first_person_character self)
  (Class|InventoryComponent|AddItem (Variables|/Script/ExtractionGame.ExtractionGameCharacter|GetInventoryComponent _asbp_first_person_character) (Variables|Default|GetGemItem) 1 true -1))

(event EventOnCancelFocus
  (Rendering|SetRenderCustomDepth (Variables|Default|GetStaticMesh) false))

(fn ConstructionScript)