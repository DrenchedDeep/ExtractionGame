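; RespawnShip is an actor Blueprint that stores references for a ship's main part and six positions around it.
; On BeginPlay it copies Main into Primary and assigns the front and back left, middle and right variables from their "0"-suffixed counterparts.
; It holds no respawn logic itself: overlap, Tick and the construction script are empty.
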(event EventBeginPlay
  (Variables|Default|SetPrimary (Variables|Default|GetMain))
  (Variables|Default|SetBackLeft (Variables|Default|GetBackLeft0))
  (Variables|Default|SetBackMid (Variables|Default|GetBackMid0))
  (Variables|Default|SetBackRight (Variables|Default|GetBackRight0))
  (Variables|Default|SetFrontLeft (Variables|Default|GetFrontLeft0))
  (Variables|Default|SetFrontMid (Variables|Default|GetFrontMid0))
  (Variables|Default|SetFrontRight (Variables|Default|GetFrontRight0)))

(event Collision|EventActorBeginOverlap
  (params (OtherActor :type Actor%20Object%20Reference)))

(event EventTick
  (params (DeltaSeconds :type Float%20%28single-precision%29)))

(fn ConstructionScript)