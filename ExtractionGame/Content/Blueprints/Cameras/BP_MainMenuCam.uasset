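; Main menu camera that repositions itself to suit the current party size.
; On BeginPlay it becomes player 0's view target and stores its starting location.
; OnPartyUpdated prints the count and targets the two- or three-player location, or the start location for any other count.
; Tick eases toward that target by lerping from the current location with DeltaSeconds as alpha.
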(event EventBeginPlay
  (Game|Player|SetViewTargetwithBlend (Game|GetPlayerController 0) self 0.0 "VTBlend_Linear" 0.0 false)
  (bind _output_get (Variables|Default|SetStartLocation (Transformation|GetActorLocation)))
  (Variables|Default|SetTargetLocation _output_get))

(event EventTick
  (params (DeltaSeconds :type Float%20%28single-precision%29))
  (Transformation|SetActorLocation (Math|Vector|Lerp(Vector) (Transformation|GetActorLocation) (Variables|Default|GetTargetLocation) DeltaSeconds) false false))

(fn ConstructionScript)

(fn OnPartyUpdated
  (params (PartyCount :type Integer))
  (Development|PrintText (Utilities|Text|ToText(Integer) PartyCount) true true "(R=0.000000,G=0.660000,B=1.000000,A=1.000000)" 9e+01)
  (if (== PartyCount 1)
    (Variables|Default|SetTargetLocation (Variables|Default|GetStartLocation) :!label _label)
    (elif (== PartyCount 2)
      (Variables|Default|SetTargetLocation (Variables|Default|GetTwoPlayersLocation))
      (elif (== PartyCount 3)
        (Variables|Default|SetTargetLocation (Variables|Default|GetThreePlayersLocation))
        (else
          (goto _label))))))