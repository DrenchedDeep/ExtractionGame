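; BP_Area is a placeable discovery zone that shows an area-name notification the first time the player enters it.
; A box trigger, sized in the construction script from the SphereSize variable, detects an overlapping BP_FirstPersonCharacter.
; Only for a locally controlled character, it creates a WB_AreaDiscovered widget with AreaName, adds it to the viewport and sets HasBeenHere so it does not repeat.
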(event OnComponentBeginOverlap(Box)
  (params (OverlappedComponent :type Primitive%20Component%20Object%20Reference) (OtherActor :type Actor%20Object%20Reference) (OtherComp :type Primitive%20Component%20Object%20Reference) (OtherBodyIndex :type Integer) (bFromSweep :type Boolean) (SweepResult :type Hit%20Result%20Structure%20%28by%20ref%29))
  (bind _asbp_first_person_character (Utilities|Casting|CastToBP_FirstPersonCharacter OtherActor))
  (Utilities|IsValid _asbp_first_person_character
    (:Is%20Valid
      (if (Pawn|IsLocallyControlled _asbp_first_person_character)
        (if (not (Variables|Default|GetHasBeenHere))
          (bind _returnvalue (UserInterface|CreateWidget "/Game/Blueprints/Widgets/WB_AreaDiscovered.WB_AreaDiscovered_C" 0 (Variables|Default|GetAreaName)))
          (UserInterface|Viewport|AddtoViewport _returnvalue 0)
          (Variables|Default|SetHasBeenHere true))))))

(fn ConstructionScript
  (Components|Box|SetBoxExtent (Variables|Default|GetBox) (Variables|Default|GetSphereSize) true))