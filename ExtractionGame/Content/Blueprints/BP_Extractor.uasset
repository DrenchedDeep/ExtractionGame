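; Extraction beacon actor that players activate with Essence to begin extraction.
; Its child interact actor is initialized with a self reference; Interact either starts extraction through a player controller server call and removes Essence, or shows an item-needed notification.
; Collision overlaps report players entering and leaving.
; Extraction state changes toggle beam, cylinder and audio, with a sound and notification widget only on first activation.
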(event OnComponentBeginOverlap(PlayerCollision)
  (params (OverlappedComponent :type Primitive%20Component%20Object%20Reference) (OtherActor :type Actor%20Object%20Reference) (OtherComp :type Primitive%20Component%20Object%20Reference) (OtherBodyIndex :type Integer) (bFromSweep :type Boolean) (SweepResult :type Hit%20Result%20Structure%20%28by%20ref%29))
  (bind _asextraction_game_character (Utilities|Casting|CastToExtractionGameCharacter OtherActor))
  (Class|ExtractionBeacon|PlayerEnter _asextraction_game_character))

(event OnComponentEndOverlap(PlayerCollision)
  (params (OverlappedComponent :type Primitive%20Component%20Object%20Reference) (OtherActor :type Actor%20Object%20Reference) (OtherComp :type Primitive%20Component%20Object%20Reference) (OtherBodyIndex :type Integer))
  (bind _asextraction_game_character (Utilities|Casting|CastToExtractionGameCharacter OtherActor))
  (Class|ExtractionBeacon|PlayerExit _asextraction_game_character))

(event EventBeginPlay
  (bind _asbp_extraction_beacon_interact (Utilities|Casting|CastToBP_ExtractionBeaconInteract (Variables|/Script/Engine.ChildActorComponent|GetChildActor (Variables|Default|GetBP_ExtractionBeaconInteract))))
  (Default|Init _asbp_extraction_beacon_interact self)
  (Audio|Components|Audio|Stop (Variables|Default|GetAudio)))

(event EventTick
  (params (DeltaSeconds :type Float%20%28single-precision%29))
  (Development|PrintText (Utilities|Text|ToText(Float) (Variables|Default|GetExtractionTimer) "HalfToEven") false false))

(event EventOnExtractionStateChangedEverybody
  (params (bExtracting :type Boolean))
  (Development|PrintText "extracti")
  (if bExtracting
    (|EnableVFX)
    (if (not (Variables|Default|GetbhasRun))
      (Variables|Default|SetbhasRun true)
      (Audio|PlaySound2D "/Game/Sound_Effects_SFX/BGM/Bossbattle.Bossbattle" 1.0 1.0 0.0 0 0 false)
      (bind _returnvalue (UserInterface|CreateWidget "/Game/Blueprints/Widgets/Extraction/WB_ExtractionNotification.WB_ExtractionNotification_C"))
      (UserInterface|Viewport|AddtoViewport _returnvalue 1))
    (else
      (|DisableVFX))))

(fn ConstructionScript)

(fn Interact
  (params (Success :type Boolean) (Player :type BP%20First%20Person%20Character%20Object%20Reference))
  (if Success
    (Default|PlayCamShake Player "/Game/Blueprints/Gameplay/Camera/Attack/BP_AttackCamShake1.BP_AttackCamShake1_C")
    (bind _asextraction_game_player_controller (Utilities|Casting|CastToExtractionGamePlayerController (Pawn|GetController Player)))
    (Class|ExtractionGamePlayerController|ServerStartExtraction _asextraction_game_player_controller self)
    (Class|InventoryComp|RemoveItembyName (Variables|/Script/ExtractionGame.ExtractionGameCharacter|GetInventoryComponent Player) (Utilities|Name|MakeLiteralName "Essence"))
    (else
      (bind _asplayer_controller (Utilities|Casting|CastToPlayerController (Pawn|GetController Player)))
      (bind _asbp_extraction_game_hud (Utilities|Casting|CastToBP_ExtractionGameHUD (HUD|GetHUD _asplayer_controller)))
      (Default|NotifyPlayer (Variables|/Game/Blueprints/Gameplay/Core/BP_ExtractionGameHUD.BP_ExtractionGameHUD_C|GetNotificationGrid _asbp_extraction_game_hud) (Utilities|Struct|MakeS_Notification "ITEM NEEDED!" "10 ESSENCE NEEDED TO START EXTRACTION BEACON" "/Game/UI/82986150-money-icon-on-isolated-background-coins-vector-illustration-in-flat-style-icons-for-design-website-removebg-preview.82986150-money-icon-on-isolated-background-coins-vector-illustration-in-flat-style-icons-for-design-website-removebg-preview")))))