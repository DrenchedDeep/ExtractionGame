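; Networked Goober AI creature with randomized body paint that players can zap, knock back, kill, cook and collect as meat.
; Sight, hits, geyser targets and gem searches feed its AI controller's blackboard.
; Picked-up gems fade in replicated eye effects, with fire and shadow gems setting angry fireball or explode states.
; Death ragdolls it using the last knockback force, counts the kill, spawns essence and drops any gem.
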(event OnSeePawn(PawnSensing)
  (params (Pawn :type Pawn%20Object%20Reference))
  (if (not (Variables|Default|GetbIsDead))
    (bind _ascharacter_pawn_base (Utilities|Casting|CastToCharacterPawnBase Pawn))
    (switch Utilities|FlowControl|Switch|SwitchonEPawnType (Class|CharacterPawnBase|GetPawnType _ascharacter_pawn_base)
      (:Player
        (bind _asbp_aicontroller (Utilities|Casting|CastToBP_AIController (Pawn|GetController)))
        (Utilities|FlowControl|Sequence
          (:then_0
            (AI|Components|Blackboard|SetValueasBool (AI|GetBlackboard _asbp_aicontroller) (Utilities|Name|MakeLiteralName "HasSeenPlayer") true)
            (AI|Components|Blackboard|SetValueasObject (AI|GetBlackboard _asbp_aicontroller) (Utilities|Name|MakeLiteralName "PlayerPawn") Pawn)
            (Variables|Default|SetLookTarget Pawn))
          (:then_1
            (Utilities|FlowControl|RetriggerableDelay 1.0)
            (AI|Components|Blackboard|SetValueasBool (AI|GetBlackboard _asbp_aicontroller) (Utilities|Name|MakeLiteralName "HasSeenPlayer") false)
            (AI|Components|Blackboard|SetValueasObject (AI|GetBlackboard _asbp_aicontroller) (Utilities|Name|MakeLiteralName "PlayerPawn") 0)))))))

(event Custom|Goober%20UnPossess
  (bind _output_get (Variables|Default|SetAlphaShift (- (Variables|Default|GetAlphaShift) 0.05)))
  (if (< _output_get 0.0)
    (Utilities|Time|ClearandInvalidateTimerbyHandle (Variables|Default|GetGooberGemUnpossesHandle))))

(event Custom|PickupGem
  (params (Gem :type BP%20Item%20Object%20Reference))
  (bind _returnvalue (Animation|Montage|MontagePlay (Components|SkeletalMesh|GetAnimInstance (Variables|Character|GetMesh)) "/Game/Models/Characters/GooberPickup_Montage.GooberPickup_Montage" 1.0 "MontageLength" 0.0 true))
  (Utilities|FlowControl|Delay (/ _returnvalue 2.5))
  (Transformation|AttachComponentToComponent Gem (Variables|Character|GetMesh) "Item" "SnapToTarget" "SnapToTarget" "SnapToTarget" true)
  (Physics|SetSimulatePhysics (Variables|/Game/Inventory/Items/BP_Item.BP_Item_C|GetItemMesh Gem) false)
  (Networking|SwitchHasAuthority
    (:Authority
      (Networking|SetReplicates Gem true)
      (Utilities|FlowControl|Sequence
        (:then_0
          (switch Utilities|FlowControl|Switch|SwitchonEGemType (.GemType (Utilities|Struct|BreakItemDataStruct (Default|GetItemData Gem)))
            (:Fire
              (Class|Goober|SetGooberState "EG_AngryFireball")
              (Variables|Default|SetGooberEyeTint "(R=10.000000,G=4.647597,B=1.273593,A=1.000000)"))
            (:Shadow
              (Class|Goober|SetGooberState "EG_AngryExplode")
              (Variables|Default|SetGooberEyeTint "(R=6.633221,G=1.071998,B=10.000000,A=1.000000)"))
            (:Water
              _))
          (bind _returnvalue_2 (Utilities|Time|SetTimerbyEvent (delegate Custom|GooberPosses) 0.1 true))
          (Variables|Default|SetGooberGemPossesHandle _returnvalue_2))
        (:then_1
          (bind _asbp_aicontroller (Utilities|Casting|CastToBP_AIController (Pawn|GetController)))
          (AI|Components|Blackboard|SetValueasEnum (AI|GetBlackboard _asbp_aicontroller) (Utilities|Name|MakeLiteralName "GooberState") (Class|Goober|GetGooberState))
          (Variables|Default|SetGemActor Gem))))))

(event Custom|GooberPosses
  (bind _output_get (Variables|Default|SetAlphaShift (+ (Variables|Default|GetAlphaShift) 0.05)))
  (if (> _output_get 1.0)
    (Utilities|Time|ClearandInvalidateTimerbyHandle (Variables|Default|GetGooberGemPossesHandle))))

(event EventBeginPlay
  (Networking|SwitchHasAuthority
    (:Authority
      (bind _output_get (Variables|Default|SetGoobTex (Math|Random|RandomFloatinRange 0.0 12.0)))
      (Rendering|Material|SetScalarParameterValue (Variables|Default|GetCookedMat) "ID" _output_get :!class /Script/Engine.MaterialInstanceDynamic)
      (bind _output_get_2 (Variables|Default|SetGooberTexMask (Math|Random|RandomFloatinRange 0.0 3.0)))
      (Rendering|Material|SetScalarParameterValue (Variables|Default|GetCookedMat) "Channel" _output_get_2 :!class /Script/Engine.MaterialInstanceDynamic)
      (bind _output_get_3 (Variables|Default|SetPaintColor (* (Utilities|Struct|MakeLinearColor (Math|Random|RandomFloat) (Math|Random|RandomFloat) (Math|Random|RandomFloat) 0.0) "(R=3.000000,G=3.000000,B=3.000000,A=1.000000)")))
      (Rendering|Material|SetVectorParameterValue (Variables|Default|GetCookedMat) "BodyPaintColor" _output_get_3 :!class /Script/Engine.MaterialInstanceDynamic)
      (Variables|Default|SetGooberSeesPlayerEvent (Utilities|Enum|ByteToEnumE_GooberSeesPlayerEvent (Math|Conversions|ToByte(Integer) (Math|Random|RandomIntegerinRange 0 1))))
      (bind _asbp_aicontroller (Utilities|Casting|CastToBP_AIController (Pawn|GetController)))
      (Default|InitGooberProperties _asbp_aicontroller (Variables|Default|GetGooberSeesPlayerEvent) (Variables|Default|GetGooberSeesSpaceShipEvent))
      (Collision|SetCollisionEnabled (Variables|Character|GetMesh) "NoCollision"))
    (:Remote
      (Rendering|Material|SetScalarParameterValue (Variables|Default|GetCookedMat) "ID" (Variables|Default|GetGoobTex) :!class /Script/Engine.MaterialInstanceDynamic)
      (Rendering|Material|SetScalarParameterValue (Variables|Default|GetCookedMat) "Channel" (Variables|Default|GetGooberTexMask) :!class /Script/Engine.MaterialInstanceDynamic)
      (Rendering|Material|SetVectorParameterValue (Variables|Default|GetCookedMat) "BodyPaintColor" (Variables|Default|GetPaintColor) :!class /Script/Engine.MaterialInstanceDynamic))))

(event Game|Damage|EventAnyDamage
  (params (Damage :type Float%20%28single-precision%29) (DamageType :type Damage%20Type%20Object%20Reference) (InstigatedBy :type Controller%20Object%20Reference) (DamageCauser :type Actor%20Object%20Reference))
  ;[1 1 1] Dmg
  (Class|Goober|ApplyDamage Damage)
  (bind _asbp_aicontroller (Utilities|Casting|CastToBP_AIController (Pawn|GetController)))
  (bind _asbp_first_person_character (Utilities|Casting|CastToBP_FirstPersonCharacter (Pawn|GetControlledPawn InstigatedBy)))
  (Utilities|FlowControl|Sequence
    (:then_0
      (AI|Components|Blackboard|SetValueasBool (AI|GetBlackboard _asbp_aicontroller) (Utilities|Name|MakeLiteralName "WasHit") true)
      (Default|ShowDamageNum _asbp_first_person_character Damage (Transformation|GetActorLocation) InstigatedBy (Variables|Default|GetbIsDead) true)
      (if (== (Utilities|GetClass DamageType) "/Game/Blueprints/Abilities/Functors/DamageTypes/DT_Fireball.DT_Fireball_C")
        (Class|Goober|AddCook (* Damage 0.05))))
    (:then_1
      (Utilities|FlowControl|RetriggerableDelay 2.0)
      (AI|Components|Blackboard|SetValueasBool (AI|GetBlackboard _asbp_aicontroller) (Utilities|Name|MakeLiteralName "WasHit") false))))

(event EventZap
  (Class|Goober|ApplyDamage 5e+01))

(event EventPull
  (params (Amt :type Float%20%28double-precision%29) (Dir :type Vector :default "0, 0, 0"))
  (CallFunction|ApplyKnockback Dir Amt))

(event EventMovetoGeyser
  (params (Geyser :type Actor%20Object%20Reference))
  (Variables|Default|SetCurrentGeyser Geyser)
  (bind _asbp_aicontroller (Utilities|Casting|CastToBP_AIController (Pawn|GetController)))
  (AI|Components|Blackboard|SetValueasBool (AI|GetBlackboard _asbp_aicontroller) (Utilities|Name|MakeLiteralName "MovingToGeyser") true))

(event Game|Damage|EventPointDamage
  (params (Damage :type Float%20%28single-precision%29) (DamageType :type Damage%20Type%20Object%20Reference) (HitLocation :type Vector :default "0, 0, 0") (HitNormal :type Vector :default "0, 0, 0") (HitComponent :type Primitive%20Component%20Object%20Reference) (BoneName :type Name :default "None") (ShotFromDirection :type Vector :default "0, 0, 0") (InstigatedBy :type Controller%20Object%20Reference) (DamageCauser :type Actor%20Object%20Reference) (HitInfo :type Hit%20Result%20Structure%20%28by%20ref%29))
  ;[1 1 1] Dmg
  (CallFunction|ApplyKnockback ShotFromDirection (* Damage (Variables|/Script/Engine.DamageType|GetDamageImpulse DamageType))))

(event Game|Damage|EventRadialDamage
  (params (DamageReceived :type Float%20%28single-precision%29) (DamageType :type Damage%20Type%20Object%20Reference) (Origin :type Vector :default "0, 0, 0") (HitInfo :type Hit%20Result%20Structure%20%28by%20ref%29) (InstigatedBy :type Controller%20Object%20Reference) (DamageCauser :type Actor%20Object%20Reference))
  ;[1 1 1] Dmg
  (CallFunction|ApplyKnockback (- (Transformation|GetActorLocation) Origin) (* DamageReceived (Variables|/Script/Engine.DamageType|GetDamageImpulse DamageType))))

(event EventOnGooberDeadAll
  (bind _mesh (Variables|Character|GetMesh))
  (Collision|SetCollisionResponsetoChannel (Variables|Default|GetCapsuleComponent) "ECC_Pawn" "ECR_Ignore")
  (Components|DestroyComponent (Variables|Default|GetPawnSensing))
  (Collision|SetCollisionEnabled (Variables|Character|GetMesh) "QueryAndPhysics")
  (Physics|SetSimulatePhysics _mesh true)
  (Class|SkeletalMeshComponent|AddImpulsetoAllBodiesBelow _mesh (* (Variables|Default|GetprvForce) (Math|Conversions|ToVector(Float) 1.0)) "None" true true)
  (CallFunction|PlaySound "Death")
  (Actor|Tick|SetActorTickEnabled false))

(event EventOnStartFocus
  (Rendering|SetVisibility (Variables|Default|GetWidget) (or (not (Variables|Default|GetbIsDead)) (Variables|Default|GetbIsCooked)) false))

(event EventOnStartCook
  (Class|Goober|StartCook))

(event EventOnCancelFocus
  (Rendering|SetVisibility (Variables|Default|GetWidget) false false))

(event EventOnGooberDeadServer
  (bind _mesh (Variables|Character|GetMesh))
  (Utilities|Time|ClearandInvalidateTimerbyHandle (Variables|Default|GetGooberGemPossesHandle))
  (if (not (Variables|Default|GetDidDeadStuff))
    (Collision|SetCollisionResponsetoChannel (Variables|Default|GetCapsuleComponent) "ECC_Pawn" "ECR_Ignore")
    (Components|DestroyComponent (Variables|Default|GetPawnSensing))
    (Collision|SetCollisionEnabled (Variables|Character|GetMesh) "QueryAndPhysics")
    (Physics|SetSimulatePhysics _mesh true)
    (Class|SkeletalMeshComponent|AddImpulsetoAllBodiesBelow _mesh (* (Variables|Default|GetprvForce) (Math|Conversions|ToVector(Float) 1.0)) "None" true true)
    (Actor|Tick|SetActorTickEnabled false)
    (Variables|Default|SetDidDeadStuff true)
    (bind _asextraction_game_state (Utilities|Casting|CastToExtractionGameState (Game|GetGameState)))
    (Class|ExtractionGameState|AddGoobersKilled _asextraction_game_state 1)
    (Utilities|FlowControl|Sequence
      (:then_0
        (Game|SpawnActorfromClass "/Game/Blueprints/BP_EssenceObject.BP_EssenceObject_C" (Math|Transform|MakeTransform (Transformation|GetActorLocation)) "Undefined" "MultiplyWithRoot" 0 0)
        (Utilities|IsValid (Variables|Default|GetGemActor)
          (:Is%20Valid
            (CallFunction|DiscardGem)
            (bind _returnvalue (Utilities|Time|SetTimerbyEvent (delegate Custom|Goober%20UnPossess) 0.1 true))
            (Variables|Default|SetGooberGemUnpossesHandle _returnvalue))))
      (:then_1
        (Utilities|FlowControl|Delay 3e+01)
        (Actor|DestroyActor))
      (:then_2
        (for _array_element (Actor|GetAttachedActors false true)
          (Actor|DestroyActor _array_element)))
      (:then_3
        (bind _asaicontroller (Utilities|Casting|CastToAIController (Pawn|GetController)))
        (AI|Logic|StopLogic (Variables|/Script/AIModule.AIController|GetBrainComponent _asaicontroller) "")))))

(event EventOnStopCook
  (Class|Goober|StopCook))

(event EventOnCookTick
  (params (currentPercent :type Float%20%28single-precision%29))
  (Rendering|Material|SetScalarParameterValue (Variables|Default|GetCookedMat) "Cooked" currentPercent :!class /Script/Engine.MaterialInstanceDynamic))

(event EventOnInteract
  (params (Invoker :type Actor%20Object%20Reference))
  (if (Variables|Default|GetbIsCooked)
    (bind _asbp_first_person_character (Utilities|Casting|CastToBP_FirstPersonCharacter Invoker))
    (bind _returnvalue (Utilities|GetDataTableRow "/Game/DataAssets/DataTables/DT_Items.DT_Items" "GooberMeat")
      (:then
        (Class|InventoryComp|TryAddItembyAddItemInfo (Variables|/Script/ExtractionGame.ExtractionGameCharacter|GetInventoryComponent _asbp_first_person_character) (Utilities|Struct|MakeAddItemInfo (Math|Vector2D|MakeVector2D (Math|Conversions|ToFloat(Integer) (.sizex _returnvalue)) (Math|Conversions|ToFloat(Integer) (.sizey _returnvalue))) (Utilities|Array|Get(acopy) (.icon _returnvalue)) (.iconrotated _returnvalue) 0 (.itemname _returnvalue) (.itemtype _returnvalue) (.rarity _returnvalue) (.description _returnvalue) "Earth" 0.0 "GooberMeat"))
        (Actor|DestroyActor)))
    (else
      (bind _caninteract (CallFunction|CanInteract))
      (if _caninteract
        (bind _asbp_first_person_character_2 (Utilities|Casting|CastToBP_FirstPersonCharacter Invoker))
        (bind _asbp_first_person_player_controller (Utilities|Casting|CastToBP_FirstPersonPlayerController (Pawn|GetController _asbp_first_person_character_2)))
        (Default|ServerInteractwithGoober _asbp_first_person_player_controller self)))))

(fn ConstructionScript
  (bind _returnvalue (Rendering|Material|CreateDynamicMaterialInstance "/Game/Models/Characters/m_goobcooked_Inst.m_goobcooked_Inst" "None" "Transient" :!class /Script/Engine.KismetMaterialLibrary))
  (bind _output_get (Variables|Default|SetCookedMat _returnvalue))
  (Rendering|Material|SetMaterial (Variables|Character|GetMesh) 0 _output_get)
  (Rendering|Material|SetScalarParameterValue (Variables|Default|GetCookedMat) "ID" (Math|Random|RandomFloatinRange 0.0 12.0) :!class /Script/Engine.MaterialInstanceDynamic)
  (Rendering|Material|SetScalarParameterValue (Variables|Default|GetCookedMat) "Channel" (Math|Random|RandomFloatinRange 0.0 3.0) :!class /Script/Engine.MaterialInstanceDynamic)
  (Rendering|Material|SetVectorParameterValue (Variables|Default|GetCookedMat) "BodyPaintColor" (* (Utilities|Struct|MakeLinearColor (Math|Random|RandomFloat) (Math|Random|RandomFloat) (Math|Random|RandomFloat) 0.0) "(R=3.000000,G=3.000000,B=3.000000,A=1.000000)") :!class /Script/Engine.MaterialInstanceDynamic)
  (Rendering|Material|SetScalarParameterValue (Variables|Default|GetCookedMat) "Cooked" 0.0 :!class /Script/Engine.MaterialInstanceDynamic))

(fn ApplyKnockback
  (params (InDirection :type Vector) (Force :type Float%20%28double-precision%29))
  (bind _output_get (Variables|Default|SetprvForce (* (+ (Math|Vector|Normalize InDirection) "") (* (* (Class|CommandHandlerSubsystem|GetDamageMultiplier (Subsystems|GetCommandHandlerSubsystem)) Force) (Class|CommandHandlerSubsystem|GetKnockBack (Subsystems|GetCommandHandlerSubsystem))))))
  (Character|LaunchCharacter _output_get false true))

(fn PlaySound
  (params (ID :type String))
  (bind _asbp_extraction_game_state (Utilities|Casting|CastToBP_ExtractionGameState (Game|GetGameState)))
  (Class|GooberSoundsManager|PlaySFX (Variables|/Script/ExtractionGame.ExtractionGameState|GetGooberSounds _asbp_extraction_game_state) ID (Transformation|GetActorLocation)))

(fn CanInteract
  (bind _returnvalue (Utilities|Time|GetTimeSeconds))
  (if (and (> (- _returnvalue (Variables|Default|GetLastInteractTime)) 2.0) (not (Variables|Default|GetbIsDead)))
    (Variables|Default|SetLastInteractTime _returnvalue)
    (return true)
    (else
      (return false))))

(fn CheckforGems
  (if (Variables|Default|GetHasGem)
    (return false 0)
    (else
      (bind _outhits (Class|KismetSystemLibrary|SphereTraceMultibyProfile (Transformation|GetActorLocation) (+ (Transformation|GetActorLocation) (* (Transformation|GetActorForwardVector) 5e+02)) 1e+03 "None" false 0 "None" true))
      (bind _array_element (Utilities|Array|ForEachLoopwithBreak _outhits)
        (:LoopBody
          (if (Utilities|DoesObjectImplementInterface (.HitActor (Collision|BreakHitResult _array_element)) "/Game/Blueprints/AI/BPI_GooberPickupable.BPI_GooberPickupable_C")
            (Variables|Default|SetGemActor (.HitActor (Collision|BreakHitResult _array_element)))
            (bind _asbp_aicontroller (Utilities|Casting|CastToBP_AIController (Pawn|GetController)))
            (AI|Components|Blackboard|SetValueasBool (AI|GetBlackboard _asbp_aicontroller) (Utilities|Name|MakeLiteralName "SeesGem") true)
            (AI|Components|Blackboard|SetValueasVector (AI|GetBlackboard _asbp_aicontroller) (Utilities|Name|MakeLiteralName "GemLocation") (Transformation|GetActorLocation (Variables|Default|GetGemActor)))
            (return true (Variables|Default|GetGemActor))
            (else
              (return false 0))))))))

(fn PlayGemPickup
  (CallFunction|PickupGem))

(fn DiscardGem
  (bind _gemactor (Variables|Default|GetGemActor))
  (Transformation|DetachFromActor _gemactor "KeepWorld" "KeepWorld" "KeepWorld")
  (Transformation|SetActorScale3D _gemactor "0.500000,0.500000,0.500000")
  (bind _asbp_item (Utilities|Casting|CastToBP_Item _gemactor))
  (Physics|SetSimulatePhysics (Variables|/Game/Inventory/Items/BP_Item.BP_Item_C|GetItemMesh _asbp_item) true)
  (Variables|/Game/Inventory/Items/BP_Item.BP_Item_C|SetIsBeingHeld _asbp_item false)
  (bind _returnvalue (Actor|GetActorOfClass "/Game/Blueprints/AI/Spawning/BP_GooberManager.BP_GooberManager_C"))
  (Class|GooberManager|MulticastResetGem _returnvalue (Variables|Default|GetGemActor)))

(fn OnRepAlphaShift
  (Rendering|Material|SetScalarParameterValue (Variables|Default|GetCookedMat) "EyeLensAlpha" (Variables|Default|GetAlphaShift) :!class /Script/Engine.MaterialInstanceDynamic))

(fn OnRepGooberEyeTint
  (bind _mesh (Variables|Character|GetMesh))
  (Utilities|IsValid (Variables|Default|GetCookedMat)
    (:Is%20Valid
      (Rendering|Material|SetVectorParameterValue (Variables|Default|GetCookedMat) "EyeTint" (Variables|Default|GetGooberEyeTint) :!class /Script/Engine.MaterialInstanceDynamic))
    (:Is%20Not%20Valid
      (bind _returnvalue (Rendering|Material|CreateDynamicMaterialInstance _mesh 0 (Rendering|Material|GetMaterial _mesh 0) "None" :!class /Script/Engine.PrimitiveComponent))
      (bind _output_get (Variables|Default|SetCookedMat _returnvalue))
      (Rendering|Material|SetMaterial _mesh 0 _output_get))))

(fn CanZap
  (return (not (Variables|Default|GetbIsDead))))