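; BP_GooberManager handles visual and pickup events for Goober AI characters and their gems.
; Its events spawn a pooled explosion effect at a location, forward gem pickups to BP_Goober, and reset a gem's actor scale.
; The attack event plays a shoot montage on the Goober's mesh only on the Remote side of an authority switch.
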(event EventPlayPickupGem
  (params (GemActor :type Actor%20Object%20Reference) (Goober :type Goober%20Object%20Reference))
  (bind _asbp_goober (Utilities|Casting|CastToBP_Goober Goober))
  (bind _asbp_item (Utilities|Casting|CastToBP_Item GemActor))
  (Default|PickupGem _asbp_goober _asbp_item))

(event EventPlayAttackAnim
  (params (Goober :type Goober%20Object%20Reference))
  (Networking|SwitchHasAuthority
    (:Remote
      (bind _asbp_goober (Utilities|Casting|CastToBP_Goober Goober))
      (Animation|Montage|PlayMontage (Variables|/Script/Engine.Character|GetMesh _asbp_goober) "/Game/Models/Characters/goob_Anim_shoot_r_Montage.goob_Anim_shoot_r_Montage"))))

(event EventResetGemSize
  (params (Gem :type Actor%20Object%20Reference))
  (Transformation|SetActorScale3D Gem "0.700000,0.700000,0.700000"))

(event EventPlayExplosionEffect
  (params (Location :type Vector :default "0, 0, 0"))
  (Niagara|SpawnSystematLocation "/Niagara/DefaultAssets/Templates/Systems/SimpleExplosion.SimpleExplosion" Location "0, 0, 0" "1.000000,1.000000,1.000000" true true "AutoRelease"))

(fn ConstructionScript)