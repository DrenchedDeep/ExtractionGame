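; Construction-script tool Blueprint that repeats a chosen static mesh along a spline as deforming spline mesh segments.
; Segment count and spacing come from the mesh's X bounding-box length measured against the spline length.
; Each segment takes local-space positions and tangents from the spline, with tangents clamped to segment length, and has collision and overlap events enabled.
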(fn ConstructionScript
  (bind _mesh (Variables|Default|GetMesh))
  (bind _spline (Variables|Default|GetSpline))
  (bind _spline_2 (Variables|Default|GetSpline))
  (bind _returnvalue (StaticMesh|GetBoundingBox _mesh))
  (bind _output_get (Variables|Default|SetX_Length (.x (+ (Math|Vector|VectorGetAbs (.min _returnvalue)) (Math|Vector|VectorGetAbs (.max _returnvalue))))))
  (for _index (range 0 (Math|Float|Truncate (/ (Spline|GetSplineLength (Variables|Default|GetSpline)) _output_get)))
    (bind _returnvalue_2 (AddComponent|AddSplineMeshComponent false))
    (Variables|/Script/Engine.PrimitiveComponent|SetbGenerateOverlapEvents _returnvalue_2 true)
    (Collision|SetCollisionEnabled _returnvalue_2 "QueryAndPhysics")
    (Components|StaticMesh|SetStaticMesh _returnvalue_2 (Variables|Default|GetMesh))
    (SplineMesh|SetStartandEnd _returnvalue_2 (Spline|GetLocationatDistanceAlongSpline _spline_2 (* _index (Variables|Default|GetX_Length)) "Local") (Math|Vector|ClampVectorSize (Spline|GetTangentatDistanceAlongSpline _spline_2 (* _index (Variables|Default|GetX_Length)) "Local") 0.0 (Variables|Default|GetX_Length)) (Spline|GetLocationatDistanceAlongSpline _spline (* (+ _index 1) (Variables|Default|GetX_Length)) "Local") (Math|Vector|ClampVectorSize (Spline|GetTangentatDistanceAlongSpline _spline (* (+ _index 1) (Variables|Default|GetX_Length)) "Local") 0.0 (Variables|Default|GetX_Length)) true :!class /Script/Engine.SplineMeshComponent)))